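; BP_GameManager bootstraps a terminal-and-network game on BeginPlay and signals when setup completes.
; It creates the HUD, sets up the camera pawn and Enhanced Input, spawns the network builder, and binds a spawned interpreter to the HUD terminal.
; Music starts paused, with playback position sampling non-real-time (NRT) loudness and Constant-Q analysis into stored values.
; GenerateAlert rebroadcasts an amount and shell; its root-connection check is unused.
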(event EventBeginPlay
  (CallFunction|AddHUD)
  (CallFunction|SetupInputs)
  (CallFunction|SetupManagers)
  (CallFunction|SetupMusic)
  (Default|CallOnSetupComplete))

(fn ConstructionScript)

(fn AddHUD
  (bind _returnvalue (UserInterface|CreateWidget "/Game/UI/WBP_HUD.WBP_HUD_C"))
  (Variables|Default|SetHUD _returnvalue)
  (bind _asbp_camera (Utilities|Casting|CastToBP_Camera (Game|Player|GetPlayerPawn 0)))
  (bind _output_get (Variables|Default|SetCameraPawn _asbp_camera))
  (Default|Setup _output_get)
  (CallFunction|SetupInterpreter)
  (UserInterface|Viewport|AddtoViewport (Variables|Default|GetHUD) 0)
  (Widget|SetVisibility (Variables|/Game/UI/WBP_HUD.WBP_HUD_C|GetInstructionDialog (Variables|Default|GetHUD)) "Hidden"))

(fn SetupInputs
  (Input|AddMappingContext (PlayerController|LocalPlayerSubsystems|GetEnhancedInputLocalPlayerSubsystem (Game|GetPlayerController 0)) "/Game/GameMode/Inputs/IM_Inputs.IM_Inputs" 0 "(bIgnoreAllPressedKeysUntilRelease=True,bForceImmediately=False,bNotifyUserSettings=False)"))

(fn SetupManagers
  (bind _returnvalue (Game|SpawnActorfromClass "/Game/GameMode/NetworkBuilder/BP_NetworkBuilder.BP_NetworkBuilder_C" (Math|Transform|MakeTransform "0, 0, 0") "Undefined" "MultiplyWithRoot" 0 0))
  (Variables|Default|SetNetworkBuilder _returnvalue))

(fn SetupMusic
  (EventDispatchers|BindEventtoOnAudioPlaybackPercent (Variables|Default|GetMusicPlayer) (EventDispatchers|CreateEvent :!event UpdateMusic))
  (CallFunction|SetPlayMusic false))

(fn UpdateMusic
  (params (PlayingSoundWave :type Sound%20Wave%20Object%20Reference) (PlaybackPercent :type Float%20%28single-precision%29))
  (bind _returnvalue (Math|Float|%(Float) PlaybackPercent 1.0))
  (bind _duration (Variables|/Script/Engine.SoundBase|GetDuration PlayingSoundWave))
  (bind _returnvalue_2 (* _duration _returnvalue))
  (Variables|Default|SetMusicLoudness (Class|LoudnessNRT|GetNormalizedLoudnessatTime (Variables|Default|GetMusicLoudnessNRT) _returnvalue_2))
  (Variables|Default|SetMusicConstants (Class|ConstantQNRT|GetNormalizedChannelConstantQatTime (Variables|Default|GetMusicConstantNRT) _returnvalue_2)))

(fn SetPlayMusic
  (params (PlayMusic :type Boolean))
  (Class|AudioComponent|SetPaused (Variables|Default|GetMusicPlayer) (not PlayMusic)))

(fn GenerateAlert
  (params (Amount :type Float%20%28double-precision%29) (Shell :type BP%20Shell%20Object%20Reference))
  (Default|CallOnGenerateAlert Amount Shell))

(fn SetupInterpreter
  (bind _returnvalue (Game|SpawnActorfromClass "/Game/Blueprints/BP_Interpreter.BP_Interpreter_C" (Math|Transform|MakeTransform "0, 0, 0") "Undefined" "MultiplyWithRoot" 0 0))
  (bind _output_get (Variables|Default|SetInterpreter _returnvalue))
  (Default|BindTerminal _output_get (Variables|/Game/UI/WBP_HUD.WBP_HUD_C|GetTerminal (Variables|Default|GetHUD))))