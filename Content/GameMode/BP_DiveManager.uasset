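; Dive manager that runs a timed network level, registering itself with BP_GameManager and spawning the player root once setup completes.
; LoadNetwork builds a random network from NetworkTable and resets the countdown, which starts only when a positive alert is generated.
; Network root shutdown triggers a win and clears the network; timeout or player root deletion shows the lose screen with the reason.
; It drives the HUD timer and status texts directly.
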(event EventBeginPlay
  (bind _asbp_game_manager (Utilities|Casting|CastToBP_GameManager (Game|GetGameMode)))
  (bind _output_get (Variables|Default|SetGameManager _asbp_game_manager))
  (EventDispatchers|BindEventtoOnSetupComplete _output_get (EventDispatchers|CreateEvent :!event OnSetupComplete))
  (EventDispatchers|BindEventtoOnGenerateAlert _output_get (EventDispatchers|CreateEvent :!event AlertGenerated)))

(event EventTick
  (params (DeltaSeconds :type Float%20%28single-precision%29))
  (CallFunction|UpdateTimer DeltaSeconds))

(fn ConstructionScript)

(fn OnSetupComplete
  (bind _gamemanager (Variables|Default|GetGameManager))
  (Variables|/Game/GameMode/BP_GameManager.BP_GameManager_C|SetDiveManager _gamemanager self)
  (Variables|Default|SetNetworkBuilder (Variables|/Game/GameMode/BP_GameManager.BP_GameManager_C|GetNetworkBuilder _gamemanager))
  (Variables|Default|SetHUD (Variables|/Game/GameMode/BP_GameManager.BP_GameManager_C|GetHUD _gamemanager))
  (CallFunction|ResetHUD)
  (bind _asbp_interpreter (Utilities|Casting|CastToBP_Interpreter (Game|Player|GetPlayerPawn 0)))
  (EventDispatchers|BindEventtoOnRootDeleted _asbp_interpreter (EventDispatchers|CreateEvent :!event OnRootDeleted))
  (Default|SpawnPlayerRoot (Variables|Default|GetNetworkBuilder)))

(fn LoadNetwork
  (bind _hud (Variables|Default|GetHUD))
  (bind _hud_2 (Variables|Default|GetHUD))
  (bind _alerthud (Variables|/Game/UI/WBP_HUD.WBP_HUD_C|GetAlertHUD _hud))
  (bind _alerthud_2 (Variables|/Game/UI/WBP_HUD.WBP_HUD_C|GetAlertHUD _hud_2))
  (bind _timertext (Variables|/Game/UI/WBP_Alert.WBP_Alert_C|GetTimerText _alerthud))
  (Utilities|FlowControl|Sequence
    (:then_0
      (Variables|Default|SetTimeLeft (Variables|Default|GetBaseLevelTime))
      (Variables|Default|SetRunTimer false)
      (Variables|Default|SetHasLost false)
      (Variables|Default|SetHasWon false))
    (:then_1
      (bind _outrownames (DataTable|GetDataTableRowNames (Variables|Default|GetNetworkTable)))
      (Default|BuildNetwork (Variables|Default|GetNetworkBuilder) (Variables|Default|GetNetworkTable) (Utilities|Array|Get(acopy) _outrownames (Math|Random|RandomIntegerinRange 0 (Utilities|Array|LastIndex _outrownames))))
      (EventDispatchers|BindEventtoOnShutdownStarted (Variables|/Game/GameMode/NetworkBuilder/BP_NetworkBuilder.BP_NetworkBuilder_C|GetNetworkRoot (Variables|Default|GetNetworkBuilder)) (EventDispatchers|CreateEvent :!event OnNetworkShutdown)))
    (:then_2
      (bind _time (CallFunction|FloattoTime (Variables|Default|GetTimeLeft)))
      (Rendering|Components|TextRender|SetText _timertext _time)
      (Widget|SetVisibility _timertext "Visible")
      (Widget|SetVisibility (Variables|/Game/UI/WBP_Alert.WBP_Alert_C|GetDeepscanText _alerthud_2) "Hidden")
      (Widget|SetVisibility (Variables|/Game/UI/WBP_Alert.WBP_Alert_C|GetWinText _alerthud_2) "Hidden"))))

(fn TriggerWin
  (bind _hud (Variables|Default|GetHUD))
  (bind _alerthud (Variables|/Game/UI/WBP_HUD.WBP_HUD_C|GetAlertHUD _hud))
  (Variables|Default|SetHasWon true)
  (Widget|SetVisibility (Variables|/Game/UI/WBP_Alert.WBP_Alert_C|GetWinText _alerthud) "Visible")
  (Widget|SetVisibility (Variables|/Game/UI/WBP_Alert.WBP_Alert_C|GetTimerText _alerthud) "Hidden")
  (Widget|SetVisibility (Variables|/Game/UI/WBP_Alert.WBP_Alert_C|GetDeepscanText _alerthud) "Visible")
  (Default|ClearNetwork (Variables|Default|GetNetworkBuilder) true))

(fn UpdateTimer
  (params (DeltaTime :type Float%20%28double-precision%29))
  (if (Math|Boolean|ANDBoolean (not (Variables|Default|GetHasWon)) (not (Variables|Default|GetHasLost)) (Variables|Default|GetRunTimer))
    (bind _output_get (Variables|Default|SetTimeLeft (Math|Float|Max(Float) (- (Variables|Default|GetTimeLeft) DeltaTime) 0.0)))
    (bind _time (CallFunction|FloattoTime _output_get))
    (Rendering|Components|TextRender|SetText (Variables|/Game/UI/WBP_Alert.WBP_Alert_C|GetTimerText (Variables|/Game/UI/WBP_HUD.WBP_HUD_C|GetAlertHUD (Variables|Default|GetHUD))) _time)
    (if (<= (Variables|Default|GetTimeLeft) 0.0)
      (CallFunction|TriggerLose true))))

(fn TriggerLose
  (params (LoseByTime :type Boolean))
  (bind _hud (Variables|Default|GetHUD))
  (bind _losescreen (Variables|/Game/UI/WBP_HUD.WBP_HUD_C|GetLoseScreen _hud))
  (Widget|SetVisibility _losescreen "Visible")
  (Rendering|Components|TextRender|SetText (Variables|/Game/UI/WBP_Lose.WBP_Lose_C|GetReasonText _losescreen) (Utilities|String|SelectText "Connection timedout" "Root disconnected" LoseByTime))
  (Variables|/Game/UI/WBP_Terminal.WBP_Terminal_C|SetkeepFocus (Variables|/Game/UI/WBP_HUD.WBP_HUD_C|GetTerminal (Variables|Default|GetHUD)) false))

(fn OnRootDeleted
  (CallFunction|TriggerLose false))

(fn AlertGenerated
  (params (Amount :type Float%20%28double-precision%29) (Shell :type BP%20Shell%20Object%20Reference))
  (if (> Amount 0.0)
    (Variables|Default|SetRunTimer true)))

(fn OnNetworkShutdown
  (CallFunction|TriggerWin))

(fn ResetHUD
  (bind _hud (Variables|Default|GetHUD))
  (bind _alerthud (Variables|/Game/UI/WBP_HUD.WBP_HUD_C|GetAlertHUD _hud))
  (Widget|SetVisibility (Variables|/Game/UI/WBP_Alert.WBP_Alert_C|GetWinText _alerthud) "Hidden")
  (Widget|SetVisibility (Variables|/Game/UI/WBP_Alert.WBP_Alert_C|GetTimerText _alerthud) "Hidden")
  (Widget|SetVisibility (Variables|/Game/UI/WBP_HUD.WBP_HUD_C|GetLoseScreen (Variables|Default|GetHUD)) "Hidden"))