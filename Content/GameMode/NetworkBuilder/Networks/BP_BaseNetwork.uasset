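; Base network actor for the network builder, generating a network of shells, programs and links from randomly chosen modules.
; PrepNetwork spawns a random count of modules per NetworkData entry, picking each class from a data table and assigning its depth.
; Separate passes tell modules to build, spawn data objects, create internal then external links, and clean up.
; Helpers register spawned shells, create entry address files and find modules by depth range or neighbouring depth.
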(fn ConstructionScript)

(fn AddEntryAddressFiles
  (params (EntryAddresses :type Array%20of%20BP%20Shell%20Object%20References))
  (for _array_element EntryAddresses
    (Game|SpawnActorfromClass "/Game/Blueprints/FileTypes/File_Address.File_Address_C" (Math|Transform|MakeTransform "0, 0, 0") "Undefined" "MultiplyWithRoot" 0 _array_element 4 (Utilities|GetAddressFileName _array_element) 0 (Variables|/Game/GameMode/NetworkBuilder/BP_NetworkBuilder.BP_NetworkBuilder_C|GetAccessShell (Variables|Default|GetNetworkBuilder)) true false 0)))

(fn SelectModule
  (params (ModuleData :type Struct%20Random%20Module%20Data%20Structure%20%28by%20ref%29))
  (bind (_possiblemodules _modulestable) (Utilities|Struct|BreakStruct_RandomModuleData ModuleData))
  (LocalVariables|SetModulesTables _modulestable)
  (bind _output_get (LocalVariables|SetSelectedModuleName (Utilities|Array|Get(acopy) _possiblemodules (Math|Random|RandomIntegerinRange 0 (Utilities|Array|LastIndex _possiblemodules)))))
  (bind _returnvalue (Utilities|GetDataTableRow (LocalVariables|GetModulesTables) (Utilities|String|StringToName _output_get))
    (:then
      (return true _returnvalue))
    (:RowNotFound
      (return false ""))))

(fn SpawnShell
  (params (Struct_ShellData :type Struct%20Shell%20Data%20Structure%20%28by%20ref%29) (Level :type Float%20%28double-precision%29))
  (bind _spawnedshell (Default|SpawnShell (Variables|Default|GetDomain) Struct_ShellData Level))
  (bind _output_get (LocalVariables|SetShell _spawnedshell))
  (Utilities|Map|Add (Variables|Default|GetNetworkShells) (Variables|/Game/Blueprints/GameObjects/BP_Shell.BP_Shell_C|GetName _output_get) (LocalVariables|GetShell))
  (return (LocalVariables|GetShell)))

(fn SpawnRandomShell
  (params (ReadAccess :type Boolean) (Level :type Float%20%28double-precision%29))
  (bind _spawnedshell (Default|SpawnRandomShell (Variables|Default|GetNetworkBuilder) ReadAccess Level))
  (Utilities|Map|Add (Variables|Default|GetNetworkShells) (Variables|/Game/Blueprints/GameObjects/BP_Shell.BP_Shell_C|GetName _spawnedshell) _spawnedshell)
  (return _spawnedshell))

(fn PrepNetwork
  (params (DiveData :type Struct%20Dive%20Option%20Structure))
  (for _array_element (Utilities|Struct|BreakStruct_NetworkData (Variables|Default|GetNetworkData))
    (bind _output_get (LocalVariables|SetModuleData _array_element))
    (for _index (range 1 (Math|Random|RandomIntegerinRange (.Min (Utilities|Struct|BreakStruct_RandomModuleData _output_get)) (.Max (Utilities|Struct|BreakStruct_RandomModuleData _output_get))))
      (bind (_modulefound _module) (CallFunction|SelectModule (LocalVariables|GetModuleData)))
      (if _modulefound
        (bind _returnvalue (Game|SpawnActorfromClass (.ModuleClass (Utilities|Struct|BreakStruct_ModuleData _module)) (Transformation|GetActorTransform) "Undefined" "MultiplyWithRoot" 0 _module self (Variables|Default|GetNetworkBuilder) DiveData (Utilities|Struct|BreakStruct_RandomModuleData (LocalVariables|GetModuleData)) 0))
        (Utilities|Array|Add (Variables|Default|GetModules) _returnvalue)))))

(fn GenerateShells
  (params (DiveData :type Struct%20Dive%20Option%20Structure))
  (for _array_element (Variables|Default|GetModules)
    (Default|BuildModule _array_element)))

(fn GeneratePrograms
  (params (DiveData :type Struct%20Dive%20Option%20Structure))
  (for _array_element (Variables|Default|GetModules)
    (Default|SpawnDataObjects _array_element)))

(fn GenerateLinks
  (for _array_element (Variables|Default|GetModules)
    (Default|CreateLinks _array_element))
  (for _array_element_2 (Variables|Default|GetModules)
    (Default|CreateExternalLinks _array_element_2)))

(fn Cleanup
  (for _array_element (Variables|Default|GetModules)
    (Default|Cleanup _array_element)))

(fn GetModulesOfDepth
  (params (MinDepth :type Float%20%28double-precision%29) (MaxDepth :type Float%20%28double-precision%29) (InclusiveMin :type Boolean) (InclusiveMax :type Boolean))
  (for _array_element (Variables|Default|GetModules)
    (if (Math|Float|InRange(Float) (Variables|/Game/GameMode/NetworkBuilder/Modules/BP_BaseModule.BP_BaseModule_C|GetDepth _array_element) MinDepth MaxDepth InclusiveMin InclusiveMax)
      (Utilities|Array|Add (LocalVariables|GetFoundModules) _array_element)))
  (return (LocalVariables|GetFoundModules)))

(fn GetNextExteriorModules
  (params (Module :type BP%20Base%20Module%20Object%20Reference) (AllowLateral :type Boolean))
  (for _array_element (Variables|Default|GetModules)
    (bind _output_get (LocalVariables|SetaModule _array_element))
    (if (Math|Boolean|ANDBoolean (!= _output_get Module) (>= (Variables|/Game/GameMode/NetworkBuilder/Modules/BP_BaseModule.BP_BaseModule_C|GetDepth _output_get) (Variables|/Game/GameMode/NetworkBuilder/Modules/BP_BaseModule.BP_BaseModule_C|GetDepth Module)) (<= (Variables|/Game/GameMode/NetworkBuilder/Modules/BP_BaseModule.BP_BaseModule_C|GetDepth _output_get) (LocalVariables|GetLowestDepth)))
      (if (or (> (Variables|/Game/GameMode/NetworkBuilder/Modules/BP_BaseModule.BP_BaseModule_C|GetDepth (LocalVariables|GetaModule)) (Variables|/Game/GameMode/NetworkBuilder/Modules/BP_BaseModule.BP_BaseModule_C|GetDepth Module)) AllowLateral)
        (if (or (== (Variables|/Game/GameMode/NetworkBuilder/Modules/BP_BaseModule.BP_BaseModule_C|GetDepth (LocalVariables|GetaModule)) (Variables|/Game/GameMode/NetworkBuilder/Modules/BP_BaseModule.BP_BaseModule_C|GetDepth Module)) (== (Variables|/Game/GameMode/NetworkBuilder/Modules/BP_BaseModule.BP_BaseModule_C|GetDepth (LocalVariables|GetaModule)) (LocalVariables|GetLowestDepth)))
          _
          (else
            (Utilities|Array|Clear (LocalVariables|GetFoundModules))
            (LocalVariables|SetLowestDepth (Variables|/Game/GameMode/NetworkBuilder/Modules/BP_BaseModule.BP_BaseModule_C|GetDepth (LocalVariables|GetaModule)))))
        (Utilities|Array|Add (LocalVariables|GetFoundModules) (LocalVariables|GetaModule)))))
  (return (LocalVariables|GetFoundModules)))

(fn GetNextInteriorModules
  (params (Module :type BP%20Base%20Module%20Object%20Reference) (AllowLateral :type Boolean))
  (for _array_element (Variables|Default|GetModules)
    (bind _output_get (LocalVariables|SetaModule _array_element))
    (if (Math|Boolean|ANDBoolean (!= _output_get Module) (<= (Variables|/Game/GameMode/NetworkBuilder/Modules/BP_BaseModule.BP_BaseModule_C|GetDepth _output_get) (Variables|/Game/GameMode/NetworkBuilder/Modules/BP_BaseModule.BP_BaseModule_C|GetDepth Module)) (>= (Variables|/Game/GameMode/NetworkBuilder/Modules/BP_BaseModule.BP_BaseModule_C|GetDepth _output_get) (LocalVariables|GetHighestDepth)))
      (if (or (< (Variables|/Game/GameMode/NetworkBuilder/Modules/BP_BaseModule.BP_BaseModule_C|GetDepth (LocalVariables|GetaModule)) (Variables|/Game/GameMode/NetworkBuilder/Modules/BP_BaseModule.BP_BaseModule_C|GetDepth Module)) AllowLateral)
        (if (or (== (Variables|/Game/GameMode/NetworkBuilder/Modules/BP_BaseModule.BP_BaseModule_C|GetDepth (LocalVariables|GetaModule)) (Variables|/Game/GameMode/NetworkBuilder/Modules/BP_BaseModule.BP_BaseModule_C|GetDepth Module)) (== (Variables|/Game/GameMode/NetworkBuilder/Modules/BP_BaseModule.BP_BaseModule_C|GetDepth (LocalVariables|GetaModule)) (LocalVariables|GetHighestDepth)))
          _
          (else
            (Utilities|Array|Clear (LocalVariables|GetFoundModules))
            (LocalVariables|SetHighestDepth (Variables|/Game/GameMode/NetworkBuilder/Modules/BP_BaseModule.BP_BaseModule_C|GetDepth (LocalVariables|GetaModule)))))
        (Utilities|Array|Add (LocalVariables|GetFoundModules) (LocalVariables|GetaModule)))))
  (return (LocalVariables|GetFoundModules)))