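; BP_DomainObject represents one domain in a dive, owning its networks, its shell registry and a Sovereign Authority Matrix (SAM).
; PrepareDomain spawns the SAM at a random offset and one random data-table network per anchor, then forwards shell, program, link and cleanup passes to those networks.
; Shells spawn through NetworkBuilder and register by name with shutdown bindings.
; ShutdownDomain pushes shells out, optionally moving those directly linked to the AccessShell into the PlayerDomain.
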(fn ConstructionScript)

(fn PrepareDomain
  (params (Data :type Struct%20Dive%20Option%20Structure))
  (Variables|Default|SetDiveData Data)
  (CallFunction|SpawnSAM)
  (LocalVariables|SetNetworksTable (.NetworksTable (Utilities|Struct|BreakStruct_DiveOption (Variables|Default|GetDiveData))))
  (for _index (range 1 (.Anchors (Utilities|Struct|BreakStruct_DiveOption (Variables|Default|GetDiveData))))
    (bind _outrownames (DataTable|GetDataTableRowNames (LocalVariables|GetNetworksTable)))
    (bind _returnvalue (Utilities|GetDataTableRow (LocalVariables|GetNetworksTable) (Utilities|Array|Get(acopy) _outrownames (Math|Random|RandomIntegerinRange 0 (Utilities|Array|LastIndex _outrownames))))
      (:then
        (bind _returnvalue_2 (Game|SpawnActorfromClass (Utilities|Struct|BreakStruct_NetworkData _returnvalue) (Transformation|GetActorTransform) "Undefined" "MultiplyWithRoot" 0 (Variables|Default|GetNetworkBuilder) _returnvalue self 0))
        (Utilities|Array|Add (Variables|Default|GetNetworks) _returnvalue_2)
        (Default|PrepNetwork _returnvalue_2 (Variables|Default|GetDiveData))))))

(fn SpawnSAM
  (bind _returnvalue (Math|Random|RandomFloatinRange 0.0 6.28))
  (if true
    (bind _returnvalue_2 (Game|SpawnActorfromClass "/Game/Blueprints/GameObjects/BP_SAM.BP_SAM_C" (Math|Transform|MakeTransform (Math|Vector|MakeVector (* (Math|Trig|Cos(Radians) _returnvalue) 4e+03) (* (Math|Trig|Sin(Radians) _returnvalue) 4e+03) 1e+03)) "Undefined" "MultiplyWithRoot" 0 0 0 0 0 true "Sovereign Authority Matrix" true 0))
    (bind _output_get (Variables|Default|SetSAM _returnvalue_2))
    (EventDispatchers|BindEventtoOnShutdownStarted _output_get (EventDispatchers|CreateEvent (Variables|Default|GetDiveManager) :!event SAMShutdown))))

(fn ShutdownDomain
  (params (KeepPlayerShells :type Boolean))
  (bind _keys (Utilities|Map|Keys (Variables|Default|GetDomainShells)))
  (for _array_element _keys
    (LocalVariables|SetShellName _array_element)
    (bind _output_get (LocalVariables|SetShell (.Value (Utilities|Map|Find (Variables|Default|GetDomainShells) _array_element))))
    (Utilities|IsValid _output_get
      (:Is%20Valid
        (LocalVariables|SetKeepShell false)
        (if KeepPlayerShells
          (bind _areconnected (CallFunction|AreShellsConnected (Variables|/Game/GameMode/NetworkBuilder/BP_NetworkBuilder.BP_NetworkBuilder_C|GetAccessShell (Variables|Default|GetNetworkBuilder)) (LocalVariables|GetShell) 0 true))
          (LocalVariables|SetKeepShell _areconnected))
        (if (LocalVariables|GetKeepShell)
          (CallFunction|RemoveShell (LocalVariables|GetShell))
          (CallFunction|AddShell (Variables|/Game/GameMode/NetworkBuilder/BP_NetworkBuilder.BP_NetworkBuilder_C|GetPlayerDomain (Variables|Default|GetNetworkBuilder)) (LocalVariables|GetShell))
          (else
            (Default|StartPush (LocalVariables|GetShell))
            (CallFunction|RemoveShell (LocalVariables|GetShell))))))))

(fn GenerateShells
  (for _array_element (Variables|Default|GetNetworks)
    (Default|GenerateShells _array_element (Variables|Default|GetDiveData))))

(fn GeneratePrograms
  (for _array_element (Variables|Default|GetNetworks)
    (Default|GeneratePrograms _array_element (Variables|Default|GetDiveData))))

(fn SpawnShell
  (params (Struct_ShellData :type Struct%20Shell%20Data%20Structure%20%28by%20ref%29) (Level :type Float%20%28double-precision%29))
  (bind _spawnedshell (Default|SpawnShell (Variables|Default|GetNetworkBuilder) Struct_ShellData Level))
  (bind _output_get (LocalVariables|SetShell _spawnedshell))
  (CallFunction|AddShell _output_get)
  (return (LocalVariables|GetShell)))

(fn ShellShutdown
  (params (Shell :type BP%20Shell%20Object%20Reference))
  (CallFunction|RemoveShell Shell))

(fn AddShell
  (params (Shell :type BP%20Shell%20Object%20Reference))
  (Utilities|Map|Add (Variables|Default|GetDomainShells) (Variables|/Game/Blueprints/GameObjects/BP_Shell.BP_Shell_C|GetName Shell) Shell)
  (Variables|/Game/Blueprints/GameObjects/BP_Shell.BP_Shell_C|SetDomain Shell self)
  (EventDispatchers|BindEventtoOnShutdownStarted Shell (EventDispatchers|CreateEvent :!event ShellShutdown)))

(fn RemoveShell
  (params (Shell :type BP%20Shell%20Object%20Reference))
  (Utilities|Map|Remove (Variables|Default|GetDomainShells) (Variables|/Game/Blueprints/GameObjects/BP_Shell.BP_Shell_C|GetName Shell))
  (Variables|/Game/Blueprints/GameObjects/BP_Shell.BP_Shell_C|SetDomain Shell 0)
  (EventDispatchers|UnbindEventfromOnShutdownStarted Shell (EventDispatchers|CreateEvent :!event ShellShutdown)))

(fn Cleanup
  (for _array_element (Variables|Default|GetNetworks)
    (Default|Cleanup _array_element)))

(fn GenerateLinks
  (for _array_element (Variables|Default|GetNetworks)
    (Default|GenerateLinks _array_element)))