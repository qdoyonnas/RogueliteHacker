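; Base network module that builds a predefined cluster of shells from its Data for the NetworkBuilder.
; BuildModule spawns shells under random names, mapped by template Id, creates non-duplicate links, then spawns their files, address files and programs.
; Programs can start immediately, with template Ids in their input swapped for spawned shell names.
; It appends the module's outer and inner connection shells to the lists passed in and returns them.
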(fn ConstructionScript)

(fn BuildModule
  (params (RemainingOuterConnections :type Array%20of%20BP%20Shell%20Object%20References) (RemainingInnerConnections :type Array%20of%20BP%20Shell%20Object%20References))
  (bind _data (Variables|Default|GetData))
  (bind (_shells _outerconnections _innerconnections) (Utilities|Struct|BreakStruct_ModuleData _data))
  (Variables|Default|SetRemaining%20Outer%20Connections RemainingOuterConnections)
  (Variables|Default|SetRemaining%20Inner%20Connections RemainingInnerConnections)
  (CallFunction|SpawnShells _shells)
  (CallFunction|CreateLinks _shells)
  (CallFunction|SpawnDataObjects _shells)
  (bind _outconnections (CallFunction|GetConnections _outerconnections))
  (Utilities|Array|AppendArray (Variables|Default|GetRemaining%20Outer%20Connections) _outconnections)
  (bind _outconnections_2 (CallFunction|GetConnections _innerconnections))
  (Utilities|Array|AppendArray (Variables|Default|GetRemaining%20Inner%20Connections) _outconnections_2)
  (return (Variables|Default|GetRemaining%20Outer%20Connections) (Variables|Default|GetRemaining%20Inner%20Connections)))

(fn SpawnShells
  (params (Shells :type Array%20of%20Struct%20Shell%20Data%20Structures))
  (bind (_data _memory _threads) (Utilities|GetClassDefaults "/Game/Blueprints/GameObjects/BP_Shell.BP_Shell_C"))
  (for _array_element Shells
    (bind _output_get (LocalVariables|SetShellId (.Id (Utilities|Struct|BreakStruct_ShellData _array_element))))
    (bind _name (Default|GetRandomShellName (Variables|Default|GetNetworkBuilder) _output_get))
    (bind _spawnedshell (Default|SpawnShell (Variables|Default|GetNetworkBuilder) (Utilities|Struct|MakeStruct_ShellData _name (Utilities|GetIntorDefault (.Data (Utilities|Struct|BreakStruct_ShellData _array_element)) _data) (Utilities|GetIntorDefault (.Memory (Utilities|Struct|BreakStruct_ShellData _array_element)) _memory) (Utilities|GetIntorDefault (.Threads (Utilities|Struct|BreakStruct_ShellData _array_element)) _threads) (.DataObjects (Utilities|Struct|BreakStruct_ShellData _array_element)) (.Links (Utilities|Struct|BreakStruct_ShellData _array_element)) (.HasReadAccess (Utilities|Struct|BreakStruct_ShellData _array_element)) (.Anchored (Utilities|Struct|BreakStruct_ShellData _array_element)) false) (LocalVariables|GetShellId)))
    (Utilities|Map|Add (Variables|Default|GetSpawnedShells) (LocalVariables|GetShellId) _spawnedshell)))

(fn SpawnDataObjects
  (params (Shells :type Array%20of%20Struct%20Shell%20Data%20Structures))
  (for _array_element Shells
    (LocalVariables|SetShell (.Value (Utilities|Map|Find (Variables|Default|GetSpawnedShells) (Utilities|String|ToLower (.Id (Utilities|Struct|BreakStruct_ShellData _array_element))))))
    (for _array_element_2 (.DataObjects (Utilities|Struct|BreakStruct_ShellData _array_element))
      (if (== (.ProcessType (Utilities|Struct|BreakStruct_DataObjectData _array_element_2)) 0)
        (CallFunction|SpawnFile (.Size (Utilities|Struct|BreakStruct_DataObjectData _array_element_2)) (.FileName (Utilities|Struct|BreakStruct_DataObjectData _array_element_2)) (.Tags (Utilities|Struct|BreakStruct_DataObjectData _array_element_2)) (.ShellAddress (Utilities|Struct|BreakStruct_DataObjectData _array_element_2)) (LocalVariables|GetShell) (.HasReadAccess (Utilities|Struct|BreakStruct_DataObjectData _array_element_2)))
        (else
          (CallFunction|SpawnProgram (.FileName (Utilities|Struct|BreakStruct_DataObjectData _array_element_2)) (.Size (Utilities|Struct|BreakStruct_DataObjectData _array_element_2)) (.Load (Utilities|Struct|BreakStruct_DataObjectData _array_element_2)) (.StartProcess (Utilities|Struct|BreakStruct_DataObjectData _array_element_2)) false (.Input (Utilities|Struct|BreakStruct_DataObjectData _array_element_2)) (.PacketCount (Utilities|Struct|BreakStruct_DataObjectData _array_element_2)) (.Timeout (Utilities|Struct|BreakStruct_DataObjectData _array_element_2)) (.PacketRate (Utilities|Struct|BreakStruct_DataObjectData _array_element_2)) (.PacketSpeed (Utilities|Struct|BreakStruct_DataObjectData _array_element_2)) (.Resilience (Utilities|Struct|BreakStruct_DataObjectData _array_element_2)) (.Integrity (Utilities|Struct|BreakStruct_DataObjectData _array_element_2)) (.Tags (Utilities|Struct|BreakStruct_DataObjectData _array_element_2)) (.Properties (Utilities|Struct|BreakStruct_DataObjectData _array_element_2)) (LocalVariables|GetShell) (.ProcessType (Utilities|Struct|BreakStruct_DataObjectData _array_element_2)) (.HasReadAccess (Utilities|Struct|BreakStruct_DataObjectData _array_element_2))))))))

(fn CreateLinks
  (params (Shells :type Array%20of%20Struct%20Shell%20Data%20Structures))
  (for _array_element Shells
    (LocalVariables|SetShell (.Value (Utilities|Map|Find (Variables|Default|GetSpawnedShells) (Utilities|String|ToLower (.Id (Utilities|Struct|BreakStruct_ShellData _array_element))))))
    (if (.ReturnValue (Utilities|Map|Find (Variables|Default|GetSpawnedShells) (Utilities|String|ToLower (.Id (Utilities|Struct|BreakStruct_ShellData _array_element)))))
      (for _array_element_2 (.Links (Utilities|Struct|BreakStruct_ShellData _array_element))
        (bind _output_get (LocalVariables|SetLink _array_element_2))
        (bind _doesexist (CallFunction|CheckLinkExists (LocalVariables|GetShell) _output_get))
        (if (and (not _doesexist) (.ReturnValue (Utilities|Map|Find (Variables|Default|GetSpawnedShells) (LocalVariables|GetLink))))
          (Default|SpawnLink (Variables|Default|GetNetworkBuilder) (LocalVariables|GetShell) (.Value (Utilities|Map|Find (Variables|Default|GetSpawnedShells) (LocalVariables|GetLink)))))))))

(fn SpawnFile
  (params (Size :type Integer) (FileName :type String) (Tags :type Array%20of%20Strings) (ShellAddress :type String) (Shell :type BP%20Shell%20Object%20Reference) (HasReadAccess :type Boolean))
  (bind _returnvalue (Utilities|String|ToLower ShellAddress))
  (bind _returnvalue_2 (Math|Transform|MakeTransform "0, 0, 0"))
  (bind _spawnedshells (Variables|Default|GetSpawnedShells))
  (bind (_value _returnvalue_3) (Utilities|Map|Find _spawnedshells _returnvalue))
  (if (and (not (Utilities|Array|IsEmpty FileName)) _returnvalue_3)
    (bind _returnvalue_4 (Game|SpawnActorfromClass "/Game/Blueprints/FileTypes/File_Address.File_Address_C" _returnvalue_2 "Undefined" "OverrideRootScale" 0 _value Size "_file" 0 Shell HasReadAccess true 0))
    (Default|SetupFile _returnvalue_4 Tags)
    (else
      (bind _returnvalue_5 (Game|SpawnActorfromClass "/Game/Blueprints/FileTypes/BP_File.BP_File_C" _returnvalue_2 "Undefined" "MultiplyWithRoot" 0 Size (Utilities|String|ToLower FileName) 0 Shell HasReadAccess true 0))
      (Default|SetupFile _returnvalue_5 Tags))))

(fn SpawnProgram
  (params (FileName :type String) (Size :type Integer) (Load :type Integer) (StartProcess :type Boolean) (FastForward :type Boolean) (Input :type String) (PacketCount :type Integer) (Timeout :type Integer) (PacketRate :type Float%20%28double-precision%29) (PacketSpeed :type Float%20%28double-precision%29) (Resilience :type Float%20%28double-precision%29) (Integrity :type Float%20%28double-precision%29) (Tags :type Array%20of%20Strings) (Properties :type Map%20of%20Strings%20to%20Strings) (Shell :type BP%20Shell%20Object%20Reference) (Type :type BP%20Process%20Class%20Reference) (HasReadAccess :type Boolean))
  (bind _returnvalue (Game|SpawnActorfromClass "/Game/Blueprints/GameObjects/BP_Program.BP_Program_C" (Math|Transform|MakeTransform "0, 0, 0") "Undefined" "MultiplyWithRoot" 0 Load PacketCount PacketRate Resilience Integrity Type PacketSpeed 1 Timeout Size FileName 0 Shell HasReadAccess true 0))
  (bind _output_get (LocalVariables|SetNewProgram _returnvalue))
  (Default|SetupProgram _output_get Tags Properties)
  (Utilities|FlowControl|Sequence
    (:then_0
      (if StartProcess
        (bind _params (CallFunction|ParseInput (Utilities|String|Append (Utilities|Array|Get(acopy) (Variables|/Game/Blueprints/GameObjects/BP_Program.BP_Program_C|GetAliases (LocalVariables|GetNewProgram))) " " Input)))
        (Default|StartProcess (LocalVariables|GetNewProgram) _params false 0 FastForward)))
    (:then_1
      (return (LocalVariables|GetNewProgram)))))

(fn ParseInput
  (params (Input :type String))
  (bind _output_get (LocalVariables|SetSplitInput (Utilities|String|ParseIntoArray Input " ")))
  (for (_array_element _array_index) _output_get
    (LocalVariables|SetIndex _array_index)
    (bind _output_get_2 (LocalVariables|SetParam (Utilities|String|ToLower _array_element)))
    (if (.ReturnValue (Utilities|Map|Find (Variables|Default|GetSpawnedShells) _output_get_2))
      (Utilities|Array|RemoveIndex (LocalVariables|GetSplitInput) (LocalVariables|GetIndex))
      (Utilities|Array|Insert (LocalVariables|GetSplitInput) (Variables|/Game/Blueprints/GameObjects/BP_Shell.BP_Shell_C|GetName (.Value (Utilities|Map|Find (Variables|Default|GetSpawnedShells) _output_get_2))) (LocalVariables|GetIndex))))
  (return (LocalVariables|GetSplitInput)))

(fn GetConnections
  (params (Connections :type Array%20of%20Strings))
  (for _array_element Connections
    (if (.ReturnValue (Utilities|Map|Find (Variables|Default|GetSpawnedShells) _array_element))
      (Utilities|Array|Add (LocalVariables|GetShells) (.Value (Utilities|Map|Find (Variables|Default|GetSpawnedShells) _array_element)))))
  (return (LocalVariables|GetShells)))