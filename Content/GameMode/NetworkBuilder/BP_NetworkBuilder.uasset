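; Network builder actor that spawns and manages the game's hacking network: domains, shells, files, programs, kernels and links.
; GenerateDomain runs a new domain object through staged shell, link and program generation, while spawn helpers create shells with level-based random stats and fill them with files or programs.
; It also creates the player's access shell and kernel, links shells with paired connection ends, and clears domains, optionally keeping the player's.
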(fn ConstructionScript)

(fn BuildNetwork
  (params (NetworkTable :type Data%20Table%20Object%20Reference) (NetworkName :type Name) (ModuleTable :type Data%20Table%20Object%20Reference)))

(fn ClearNetwork
  (params (KeepPlayerShells :type Boolean))
  (for (_array_element _array_index) (Variables|Default|GetDomains)
    (bind _output_get (LocalVariables|SetDomain _array_element))
    (if (or (!= _output_get (Variables|Default|GetPlayerDomain)) (not KeepPlayerShells))
      (Default|ShutdownDomain (LocalVariables|GetDomain) KeepPlayerShells)
      (Utilities|Array|RemoveIndex (Variables|Default|GetDomains) _array_index)
      (if (== (Variables|Default|GetActiveDomain) (LocalVariables|GetDomain))
        (Variables|Default|SetActiveDomain 0))
      (Actor|DestroyActor (LocalVariables|GetDomain)))))

(fn FindNewShellPosition
  (params (Range :type Float%20%28double-precision%29))
  (return (Math|Transform|MakeTransform (* (Math|Random|RandomUnitVector) Range))))

(fn SpawnShell
  (params (Struct_ShellData :type Struct%20Shell%20Data%20Structure%20%28by%20ref%29) (Level :type Float%20%28double-precision%29))
  (bind (_hasreadaccess _anchored) (Utilities|Struct|BreakStruct_ShellData Struct_ShellData))
  (bind (_name _data _memory _threads _ports) (CallFunction|GetShellStats Struct_ShellData Level))
  (bind _shelltransform (CallFunction|FindNewShellPosition 2e+03))
  (bind _returnvalue (Game|SpawnActorfromClass "/Game/Blueprints/GameObjects/BP_Shell.BP_Shell_C" _shelltransform "Undefined" "MultiplyWithRoot" 0 (Math|Float|Round _data) (Math|Float|Round _memory) (Math|Float|Round _threads) (Math|Float|Truncate _ports) _hasreadaccess _name _anchored 0))
  (bind _output_get (LocalVariables|SetNewShell _returnvalue))
  (Utilities|Array|AppendArray (Variables|/Script/Engine.Actor|GetTags _output_get) (Utilities|Struct|BreakStruct_ShellData Struct_ShellData))
  (return (LocalVariables|GetNewShell)))

(fn SpawnRandomShell
  (params (ReadAccess :type Boolean) (Level :type Float%20%28double-precision%29))
  (bind _spawnedshell (CallFunction|SpawnShell (Utilities|Struct|MakeStruct_ShellData "sh" 0 (Variables|Default|GetRandomShellData) (Variables|Default|GetRandomShellMemory) (Variables|Default|GetRandomShellThreads) (Variables|Default|GetRandomShellPorts) "(FileName_11_6BDFF353497752F9BF4778AA53F7EBCF=\"\",KernelProcess_12_C17036B943ACC2AFBB581FA468EDD919=None,ExtraPrograms_6_8322350047A0B366726E79BD3ECF7732=)" 0 0 ReadAccess) Level))
  (return _spawnedshell))

(fn SpawnPlayerAccess
  (params (BasicPrograms :type Data%20Table%20Object%20Reference) (TerminalCommands :type Data%20Table%20Object%20Reference))
  (if (not (Utilities|IsValid (Variables|Default|GetAccessShell)))
    (bind _returnvalue (Game|SpawnActorfromClass "/Game/GameMode/NetworkBuilder/BP_DomainObject.BP_DomainObject_C" (Transformation|GetActorTransform) "Undefined" "MultiplyWithRoot" 0 self 0 0))
    (bind _output_get (Variables|Default|SetPlayerDomain _returnvalue))
    (Utilities|Array|Add (Variables|Default|GetDomains) _output_get)
    (bind _returnvalue_2 (Game|SpawnActorfromClass "/Game/Blueprints/GameObjects/BP_Shell.BP_Shell_C" (Transformation|GetActorTransform) "Undefined" "MultiplyWithRoot" 0 200 200 5 3 true "AccessShell" true 0))
    (bind _output_get_2 (Variables|Default|SetAccessShell _returnvalue_2))
    (bind _processtypes (CallFunction|CreateAccessPrograms _output_get_2 BasicPrograms))
    (bind _returnvalue_3 (Game|SpawnActorfromClass "/Game/Blueprints/GameObjects/KrnP_Access.KrnP_Access_C" (Transformation|GetActorTransform) "Undefined" "MultiplyWithRoot" 0 TerminalCommands true 0 _processtypes "/Game/Blueprints/Processes/KernelProcesses/Krn_Access.Krn_Access_C" 0.0 0 "Access" 0 (Variables|Default|GetAccessShell) true true 0))
    (Default|SetupProgram _returnvalue_3 0 (Utilities|Map|MakeMap) (Utilities|Map|MakeMap))
    (Default|AddShell (Variables|Default|GetPlayerDomain) (Variables|Default|GetAccessShell))
    (Default|CallOnRootSpawned)))

(fn GetRandomShellName
  (params (Prefix :type String) (RandomizeName :type Boolean))
  (if RandomizeName
    (bind _allshells (CallFunction|GetAllShells))
    (LocalVariables|SetFindName (Utilities|GetRandomName Prefix))
    (while (.ReturnValue (Utilities|Map|Find _allshells (LocalVariables|GetFindName)))
      (LocalVariables|SetFindName (Utilities|GetRandomName Prefix)))
    (return (LocalVariables|GetFindName))
    (else
      (return Prefix))))

(fn AddRandomFilestoShell
  (params (Shell :type BP%20Shell%20Object%20Reference) (AmountMin :type Integer) (AmountMax :type Integer))
  (LocalVariables|SetCount 0)
  (LocalVariables|SetTotal (Math|Random|RandomIntegerinRange AmountMin AmountMax))
  (while (< (LocalVariables|GetCount) (LocalVariables|GetTotal))
    (bind _returnvalue (Game|SpawnActorfromClass "/Game/Blueprints/FileTypes/BP_File.BP_File_C" (Math|Transform|MakeTransform "0, 0, 0") "Undefined" "MultiplyWithRoot" 0 4 (Utilities|GetRandomName "_f") 0 Shell (Variables|/Game/Blueprints/GameObjects/BP_Shell.BP_Shell_C|GetReadAccess Shell) false 0))
    (Default|SetupFile _returnvalue)
    (Math|Integer|IncrementInt (LocalVariables|GetCount))))

(fn SpawnLinkEnd
  (params (PairedProcess :type Conn%20Link%20Object%20Reference) (Shell :type BP%20Shell%20Object%20Reference) (AddressShell :type BP%20Shell%20Object%20Reference) (readAccess :type Boolean))
  (bind _returnvalue (Game|SpawnActorfromClass "/Game/Blueprints/Processes/Subprocesses/Conn_Link.Conn_Link_C" (Math|Transform|MakeTransform "0, 0, 0") "Undefined" "MultiplyWithRoot" 0 PairedProcess 0 0 true 0 (Utilities|Array|MakeArray (Variables|/Game/Blueprints/GameObjects/BP_Shell.BP_Shell_C|GetName AddressShell)) 0.0 false false Shell readAccess true 0))
  (Default|SetupNavigation _returnvalue 1.0 -1.0 AddressShell)
  (return _returnvalue))

(fn SpawnLink
  (params (Shell :type BP%20Shell%20Object%20Reference) (Link :type BP%20Shell%20Object%20Reference))
  (if (not (.ReturnValue (Utilities|Map|Find (Variables|/Game/Blueprints/GameObjects/BP_Shell.BP_Shell_C|GetLocalConnections Shell) (Variables|/Game/Blueprints/GameObjects/BP_Shell.BP_Shell_C|GetName Link))))
    (LocalVariables|SetLinkReadAccess (and (Variables|/Game/Blueprints/GameObjects/BP_Shell.BP_Shell_C|GetReadAccess Shell) (Variables|/Game/Blueprints/GameObjects/BP_Shell.BP_Shell_C|GetReadAccess Link)))
    (bind _returnvalue (CallFunction|SpawnLinkEnd 0 Shell Link (LocalVariables|GetLinkReadAccess)))
    (CallFunction|SpawnLinkEnd _returnvalue Link Shell (LocalVariables|GetLinkReadAccess))
    (Default|StartPull Link Shell (LocalVariables|GetLinkReadAccess) (LocalVariables|GetLinkReadAccess))))

(fn GetShellStats
  (params (ShellStruct :type Struct%20Shell%20Data%20Structure) (Level :type Float%20%28double-precision%29))
  (bind (_id _tags _data _memory _threads _ports _kernel _randomizename) (Utilities|Struct|BreakStruct_ShellData ShellStruct))
  (Utilities|FlowControl|Sequence
    (:then_0
      (bind _name (CallFunction|GetRandomShellName _id _randomizename))
      (LocalVariables|SetShellName _name))
    (:then_1
      (bind _stat (CallFunction|RandomStat _data Level))
      (LocalVariables|SetShellData _stat))
    (:then_2
      (bind _stat_2 (CallFunction|RandomStat _memory Level))
      (LocalVariables|SetShellMemory _stat_2))
    (:then_3
      (bind _stat_3 (CallFunction|RandomStat _threads Level))
      (LocalVariables|SetShellThreads _stat_3))
    (:then_4
      (bind _stat_4 (CallFunction|RandomStat _ports Level))
      (LocalVariables|SetShellPorts _stat_4))
    (:then_5
      (return (LocalVariables|GetShellName) (LocalVariables|GetShellData) (LocalVariables|GetShellMemory) (LocalVariables|GetShellThreads) (LocalVariables|GetShellPorts)))))

(fn SpawnShellwithDataObjects
  (params (Struct_ShellData :type Struct%20Shell%20Data%20Structure%20%28by%20ref%29) (Level :type Float%20%28double-precision%29) (FastForward :type Boolean))
  (bind _spawnedshell (CallFunction|SpawnShell Struct_ShellData Level))
  (LocalVariables|SetSpawned _spawnedshell)
  (bind _allshells (CallFunction|GetAllShells))
  (CallFunction|AddDataObjectstoShell (LocalVariables|GetSpawned) (Utilities|Struct|BreakStruct_ShellData Struct_ShellData) _allshells FastForward)
  (return (LocalVariables|GetSpawned)))

(fn SpawnFile
  (params (Size :type Integer) (FileName :type String) (Tags :type Array%20of%20Strings) (ShellAddress :type String) (Shell :type BP%20Shell%20Object%20Reference) (HasReadAccess :type Boolean) (Shells :type Map%20of%20Strings%20to%20Objects))
  (bind _returnvalue (Utilities|String|ToLower ShellAddress))
  (bind (_value _returnvalue_2) (Utilities|Map|Find Shells _returnvalue))
  (if (and (not (Utilities|Array|IsEmpty FileName)) _returnvalue_2)
    (bind _returnvalue_3 (Game|SpawnActorfromClass "/Game/Blueprints/FileTypes/File_Address.File_Address_C" (Math|Transform|MakeTransform "0, 0, 0") "Undefined" "OverrideRootScale" 0 _value Size (Utilities|GetAddressFileName _value) 0 Shell HasReadAccess true 0))
    (bind _output_get (LocalVariables|SetLocalFile _returnvalue_3))
    (Default|SetupFile _output_get Tags)
    (else
      (bind _returnvalue_4 (Game|SpawnActorfromClass "/Game/Blueprints/FileTypes/BP_File.BP_File_C" (Math|Transform|MakeTransform "0, 0, 0") "Undefined" "MultiplyWithRoot" 0 Size (Utilities|String|ToLower FileName) 0 Shell HasReadAccess true 0))
      (bind _output_get_2 (LocalVariables|SetLocalFile _returnvalue_4))
      (Default|SetupFile _output_get_2 Tags)))
  (return (LocalVariables|GetLocalFile)))

(fn ParseInput
  (params (Input :type String) (Shells :type Map%20of%20Strings%20to%20Objects))
  (bind _output_get (LocalVariables|SetSplitInput (Utilities|String|ParseIntoArray Input " ")))
  (for (_array_element _array_index) _output_get
    (LocalVariables|SetIndex _array_index)
    (bind _output_get_2 (LocalVariables|SetParam (Utilities|String|ToLower _array_element)))
    (if (.ReturnValue (Utilities|Map|Find Shells _output_get_2))
      (Utilities|Array|RemoveIndex (LocalVariables|GetSplitInput) (LocalVariables|GetIndex))
      (Utilities|Array|Insert (LocalVariables|GetSplitInput) (Variables|/Game/Blueprints/GameObjects/BP_Shell.BP_Shell_C|GetName (.Value (Utilities|Map|Find Shells _output_get_2))) (LocalVariables|GetIndex))))
  (return (LocalVariables|GetSplitInput)))

(fn SpawnProgram
  (params (FileName :type String) (Size :type Integer) (RunProcess :type Integer) (FastForward :type Boolean) (Input :type String) (Tags :type Array%20of%20Strings) (Level :type Float%20%28double-precision%29) (Properties :type Map%20of%20Strings%20to%20Strings) (Shell :type BP%20Shell%20Object%20Reference) (Types :type Array%20of%20BP%20Process%20Class%20References) (HasReadAccess :type Boolean) (PlayerOwned :type Boolean) (Shells :type Map%20of%20Strings%20to%20Objects) (DeleteAfterStart :type Boolean))
  (bind _new_program (CallFunction|SpawnProgramfromType FileName Size Tags Level Shell Types HasReadAccess))
  (bind _output_get (LocalVariables|SetNewProgram _new_program))
  (Utilities|IsValid _output_get
    (:Is%20Valid
      (Default|SetupProgram _output_get Tags Properties (Utilities|Map|MakeMap))
      (return (LocalVariables|GetNewProgram)))))

(fn AddDataObjectstoShell
  (params (Shell :type BP%20Shell%20Object%20Reference) (Data :type Array%20of%20Struct%20Data%20Object%20Data%20Structures) (Shells :type Map%20of%20Strings%20to%20Objects) (FastForward :type Boolean))
  (for _array_element Data
    (CallFunction|AddDataObject _array_element Shell Shells FastForward)))

(fn GenerateDomain
  (params (Data :type Struct%20Dive%20Option%20Structure) (DiveManager :type BP%20Dive%20Manager%20Object%20Reference))
  (bind _returnvalue (Game|SpawnActorfromClass "/Game/GameMode/NetworkBuilder/BP_DomainObject.BP_DomainObject_C" (Math|Transform|MakeTransform "0, 0, 0") "Undefined" "MultiplyWithRoot" 0 self DiveManager 0))
  (bind _output_get (Variables|Default|SetActiveDomain _returnvalue))
  (Utilities|Array|Add (Variables|Default|GetDomains) _output_get)
  (Default|PrepareDomain (Variables|Default|GetActiveDomain) Data)
  (Default|GenerateShells (Variables|Default|GetActiveDomain))
  (Default|GenerateLinks (Variables|Default|GetActiveDomain))
  (Default|GeneratePrograms (Variables|Default|GetActiveDomain))
  (Default|Cleanup (Variables|Default|GetActiveDomain)))

(fn FindShell
  (params (Name :type String))
  (for _array_element (Variables|Default|GetDomains)
    (if (.ReturnValue (Utilities|Map|Find (Variables|/Game/GameMode/NetworkBuilder/BP_DomainObject.BP_DomainObject_C|GetDomainShells _array_element) (Utilities|String|ToLower Name)))
      (return true (.Value (Utilities|Map|Find (Variables|/Game/GameMode/NetworkBuilder/BP_DomainObject.BP_DomainObject_C|GetDomainShells _array_element) (Utilities|String|ToLower Name))))))
  (return false 0))

(fn GetAllShells
  (for _array_element (Variables|Default|GetDomains)
    (bind _output_get (LocalVariables|SetDomain _array_element))
    (bind _keys (Utilities|Map|Keys (Variables|/Game/GameMode/NetworkBuilder/BP_DomainObject.BP_DomainObject_C|GetDomainShells _output_get)))
    (for _array_element_2 _keys
      (Utilities|Map|Add (LocalVariables|GetAll) _array_element_2 (.Value (Utilities|Map|Find (Variables|/Game/GameMode/NetworkBuilder/BP_DomainObject.BP_DomainObject_C|GetDomainShells (LocalVariables|GetDomain)) _array_element_2)))))
  (return (LocalVariables|GetAll)))

(fn AddDataObject
  (params (DataObjectData :type Struct%20Data%20Object%20Data%20Structure%20%28by%20ref%29) (Shell :type BP%20Shell%20Object%20Reference) (Shells :type Map%20of%20Strings%20to%20Objects) (FastForward :type Boolean))
  (bind (_filename _processtypes _size _tags _runprocess _input _shelladdress _properties _hasreadaccess _playerowned _level _deleteafterstart) (Utilities|Struct|BreakStruct_DataObjectData DataObjectData))
  (if (Utilities|Array|IsEmpty _processtypes)
    (bind _file (CallFunction|SpawnFile _size _filename _tags _shelladdress Shell _hasreadaccess Shells))
    (LocalVariables|SetLocalDataObject _file)
    (else
      (bind _program (CallFunction|SpawnProgram _filename _size _runprocess FastForward _input _tags _level _properties Shell _processtypes _hasreadaccess _playerowned Shells _deleteafterstart))
      (LocalVariables|SetLocalDataObject _program)))
  (return (LocalVariables|GetLocalDataObject)))

(fn CreateAccessPrograms
  (params (AccessShell :type BP%20Shell%20Object%20Reference) (BasicPrograms :type Data%20Table%20Object%20Reference))
  (bind _outrownames (DataTable|GetDataTableRowNames BasicPrograms))
  (for _array_element _outrownames
    (bind _returnvalue (Utilities|GetDataTableRow BasicPrograms _array_element)
      (:then
        (Utilities|Array|Add (LocalVariables|GetTypes) (Utilities|Struct|BreakStruct_Command _returnvalue)))))
  (return (LocalVariables|GetTypes)))

(fn SpawnProgramfromType
  (params (FileName :type String) (Size :type Integer) (DataTags :type Array%20of%20Strings) (Level :type Float%20%28double-precision%29) (Shell :type BP%20Shell%20Object%20Reference) (ProcessTypes :type Array%20of%20BP%20Process%20Class%20References) (readAccess :type Boolean))
  (LocalVariables|SetSpawnTransform (Math|Transform|MakeTransform "0, 0, 0"))
  (if (> (Utilities|Array|Length ProcessTypes) 1)
    (bind _returnvalue (Game|SpawnActorfromClass "/Game/Blueprints/GameObjects/Prog_Packaged.Prog_Packaged_C" (LocalVariables|GetSpawnTransform) "Undefined" "MultiplyWithRoot" 0 0 ProcessTypes 0 Level Size FileName DataTags Shell readAccess true 0))
    (return _returnvalue)
    (else
      (bind _returnvalue_2 (Game|SpawnActorfromClass "/Game/Blueprints/GameObjects/BP_Program.BP_Program_C" (LocalVariables|GetSpawnTransform) "Undefined" "MultiplyWithRoot" 0 (Utilities|Array|Get(acopy) ProcessTypes) Level Size FileName DataTags Shell readAccess true 0))
      (return _returnvalue_2))))

(fn SpawnKernel
  (params (KernelType :type BP%20Process%20Class%20Reference) (ProcessTypes :type Array%20of%20BP%20Process%20Class%20References) (FileName :type String) (Shell :type BP%20Shell%20Object%20Reference))
  (if (Utilities|IsValidClass KernelType)
    (LocalVariables|SetTransform (Math|Transform|MakeTransform "0, 0, 0"))
    (if (== KernelType "/Game/Blueprints/Processes/KernelProcesses/Krn_Access.Krn_Access_C")
      (bind _returnvalue (Game|SpawnActorfromClass "/Game/Blueprints/GameObjects/KrnP_Access.KrnP_Access_C" (LocalVariables|GetTransform) "Undefined" "MultiplyWithRoot" 0 "/Game/Blueprints/Processes/TerminalProcesses/DT_TerminalCommands.DT_TerminalCommands" true 0 ProcessTypes KernelType 0.0 0 FileName 0 Shell true true 0))
      (Default|SetupProgram _returnvalue 0 (Utilities|Map|MakeMap) (Utilities|Map|MakeMap))
      (return _returnvalue)
      (else
        (bind _returnvalue_2 (Game|SpawnActorfromClass "/Game/Blueprints/GameObjects/Prog_Kernel.Prog_Kernel_C" (LocalVariables|GetTransform) "Undefined" "MultiplyWithRoot" 0 false 0 ProcessTypes KernelType 0.0 0 FileName 0 Shell (Variables|/Game/Blueprints/GameObjects/BP_Shell.BP_Shell_C|GetReadAccess Shell) true 0))
        (Default|SetupProgram _returnvalue_2 0 (Utilities|Map|MakeMap) (Utilities|Map|MakeMap))
        (return _returnvalue_2)))))