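; BP_Program is an executable program file actor, apparently for a hacking game, that launches a process of its configured ProcessType.
; SetupProgram merges supplied tags with the process class's default tags and copies its aliases.
; StartProcess drops the first parameter, spawns the process with the program's packet, load, thread and access settings, then plays a yaw timeline on Scale.
; Duplicate spawns a same-class copy carrying its stats and tags.
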(event Custom|PlayStart
  (bind _rotation (Timeline|StartTimeline PlayFromStart)
    (:Update
      (Transformation|SetRelativeRotation (Variables|Default|GetScale) (Math|Rotator|MakeRotator 0.0 0.0 _rotation) false false))))

(fn ConstructionScript
  (|CallParentFunction))

(fn SetupProgram
  (params (Tags :type Array%20of%20Strings) (Properties :type Map%20of%20Strings%20to%20Strings))
  (bind _processtype (Variables|Default|GetProcessType))
  (bind (_program _params _onoutput _nextsend _packetcount _packetrate _packetspeed _sendpackettimestamp _dosendpacket _aliases _targetedshellobject _landedpackets _load _datatags) (Utilities|GetClassDefaults _processtype))
  (for _array_element Tags
    (Utilities|Array|AddUnique (Variables|Default|GetDataTags) _array_element))
  (Variables|Default|SetAliases _aliases)
  (for _array_element_2 _datatags
    (Utilities|Array|AddUnique (Variables|Default|GetDataTags) _array_element_2)))

(fn StartProcess
  (params (Params :type Array%20of%20Strings) (IsPlayerOwned :type Boolean))
  (Utilities|Array|RemoveIndex Params)
  (bind _returnvalue (Game|SpawnActorfromClass (Variables|Default|GetProcessType) (Math|Transform|MakeTransform "0, 0, 0") "Undefined" "MultiplyWithRoot" 0 self Params (Variables|Default|GetPacketCount) (Variables|Default|GetPacketRate) (Variables|Default|GetPacketSpeed) (Variables|Default|GetLoad) (Variables|Default|GetThreads) IsPlayerOwned (Variables|Default|GetShell) (Variables|Default|GetreadAccess) false 0))
  (CallFunction|PlayStart)
  (return "" _returnvalue))

(fn Duplicate
  (bind _returnvalue (Game|SpawnActorfromClass (Utilities|GetClass self) (Math|Transform|MakeTransform "0, 0, 0") "Undefined" "MultiplyWithRoot" 0 (Variables|Default|GetLoad) (Variables|Default|GetPacketCount) (Variables|Default|GetPacketRate) (Variables|Default|GetResilience) (Variables|Default|GetIntegrity) (Variables|Default|GetProcessType) (Variables|Default|GetPacketSpeed) (Variables|Default|GetThreads) (Variables|Default|GetSize) (Variables|Default|GetFileName) (Variables|Default|GetDataTags) (Variables|Default|GetShell) (Variables|Default|GetreadAccess) false 0))
  (CallFunction|SetupProgram _returnvalue 0 (Utilities|Map|MakeMap "" ""))
  (return _returnvalue))