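; BP_Process runs a Program with given Params, sending packet actors that carry it and relaying its results through output events.
; When installation finishes it spawns a BP_Packet, and Tick sends another whenever sending is flagged and the PacketRate-based timestamp has passed.
; A packet's arrival at a shell parses the params, deleting packet and process on failure.
; CallProgram outputs the program's result, then deletes the process.
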(event EventTick
  (params (DeltaSeconds :type Float%20%28single-precision%29))
  (|CallParentFunction 0.0)
  (if (Variables|Default|GetDoSendPacket)
    (if (>= (Math|DateTime|Now) (Variables|Default|GetSendPacketTimestamp))
      (CallFunction|SendPacket))))

(fn ConstructionScript)

(fn CallProgram
  (bind _output (Default|Call (Variables|Default|GetProgram) (Variables|Default|GetParams)))
  (Default|CallOnOutput _output)
  (CallFunction|Delete))

(fn Setup
  (|CallParentFunction)
  (CallFunction|BindEvents))

(fn BindEvents
  (bind _asbp_game_manager (Utilities|Casting|CastToBP_GameManager (Game|GetGameMode)))
  (EventDispatchers|BindEventtoOnOutput (EventDispatchers|CreateEvent (Variables|/Game/UI/WBP_HUD.WBP_HUD_C|GetTerminal (Variables|/Game/GameMode/BP_GameManager.BP_GameManager_C|GetHUD _asbp_game_manager)) :!event Print)))

(fn DoneInstalling
  (|CallParentFunction)
  (CallFunction|SendPacket))

(fn SendPacket
  (bind _returnvalue (Game|SpawnActorfromClass "/Game/Blueprints/BP_Packet.BP_Packet_C" (Math|Transform|MakeTransform "0, 0, 0") "Undefined" "MultiplyWithRoot" 0 (Variables|Default|GetPacketSpeed) self (Variables|Default|GetProgram) 0))
  (bind _output_get (Variables|Default|SetActivePacket _returnvalue))
  (EventDispatchers|BindEventtoOnArriveatShell _output_get (EventDispatchers|CreateEvent :!event OnPacketArrived))
  (Variables|Default|SetDoSendPacket false))

(fn SetNextSendTimestamp
  (Variables|Default|SetSendPacketTimestamp (+ (Math|DateTime|Now) (Math|Timespan|FromSeconds (/ 1.0 (Variables|Default|GetPacketRate))))))

(fn OnPacketArrived
  (bind (_output _issuccess) (Default|Parse (Variables|Default|GetProgram) (Variables|Default|GetParams)))
  (Default|CallOnOutput _output)
  (if (not _issuccess)
    (Actor|DestroyActor (Variables|Default|GetActivePacket))
    (CallFunction|Delete)))

(fn SetupOrbit
  (Variables|Default|SetOrbitRotator (* (Math|Rotator|MakeRotator (Math|Float|SelectFloat 1.0 -1.0 (Math|Random|RandomBool)) (Math|Float|SelectFloat 1.0 -1.0 (Math|Random|RandomBool)) 0.0) (Variables|Default|GetOrbitSpeed))))