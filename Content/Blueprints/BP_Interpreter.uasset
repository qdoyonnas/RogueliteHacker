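; Terminal interpreter and camera rig that turns typed text into programs or commands and frames shells in the world.
; ParseInput tries programs in the active shell and ShellPaths, then data table aliases, spawning command process actors and broadcasting output to a log.
; On Tick, the camera anchor lerps to the focused shell, then orbits.
; An input opens the main menu; music-driven FOV is left unconnected.
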(event Input|EnhancedActionEvents|EnhancedInputActionIA_OpenMenu
  (params (ActionValue :type Boolean) (ElapsedSeconds :type Float%20%28double-precision%29) (TriggeredSeconds :type Float%20%28double-precision%29) (InputAction :type Input%20Action%20Object%20Reference :default "/Game/GameMode/Inputs/IA_OpenMenu.IA_OpenMenu"))
  (Game|OpenLevel(byName) "LVL_MainMenu"))

(event EventBeginPlay
  (Variables|Default|SetCurrentZoomTime (Variables|Default|GetZoomTime))
  (Variables|Default|SetDefaultFOV (Variables|/Script/Engine.CameraComponent|GetFieldOfView (Variables|Default|GetCamera))))

(event EventTick
  (params (DeltaSeconds :type Float%20%28single-precision%29))
  (CallFunction|Orbit DeltaSeconds)
  (CallFunction|Zoom DeltaSeconds))

(fn ConstructionScript)

(fn CreateTerminalCommand
  (params (Class :type BP%20Process%20Class%20Reference) (Params :type Array%20of%20Strings) (ReadAccess :type Boolean))
  (bind (_program _params _onoutput _nextsend _packetcount _packetrate _packetspeed _sendpackettimestamp _dosendpacket _aliases _targetedshellobject _landedpackets _load _datatags _navigationprocess _threads) (Utilities|GetClassDefaults Class))
  (if (Utilities|IsValidClass Class)
    (bind _returnvalue (Game|SpawnActorfromClass Class (Math|Transform|MakeTransform "0, 0, 0") "Undefined" "MultiplyWithRoot" 0 (Variables|Default|GetRootProgram) Params _packetcount _packetrate _packetspeed _load _threads true (Variables|Default|GetActiveShell) ReadAccess false 0))
    (if ReadAccess
      (Default|PlayStart (Variables|Default|GetRootProgram)))
    (return "" _returnvalue)
    (else
      (return "====EXCEPTION: Invalid process class=====" 0))))

(fn GetTerminalCommandfromInput
  (params (Input :type String) (DataTable :type Data%20Table%20Object%20Reference))
  (bind _outrownames (DataTable|GetDataTableRowNames DataTable))
  (for _array_element _outrownames
    (bind _returnvalue (Utilities|GetDataTableRow DataTable _array_element)
      (:then
        (switch int (Utilities|Array|FindItem (.Aliases (Utilities|GetClassDefaults (Utilities|Struct|BreakStruct_Command _returnvalue))) Input)
          (:Default
            (return (Utilities|Struct|BreakStruct_Command _returnvalue) true))))))
  (return 0 false))

(fn ParseInput
  (params (Input :type Text))
  (bind _returnvalue (Utilities|String|ToString(Text) Input))
  (bind _returnvalue_2 (Utilities|String|ParseIntoArray _returnvalue " "))
  (if (and (Utilities|IsValid (Variables|Default|GetRootProgram)) (not (Utilities|Text|TextIsEmpty Input)))
    (bind (_params _program _isfound) (CallFunction|SearchforProgram _returnvalue_2))
    (if _isfound
      (bind _output (Default|StartProcess _program _params true))
      (Default|CallOnOutputLog _output)
      (else
        (bind (_params_2 _process _isfound_2 _readaccess) (CallFunction|SearchforCommand _returnvalue_2))
        (if _isfound_2
          (bind _output_2 (CallFunction|CreateTerminalCommand _process _params_2 _readaccess))
          (Default|CallOnOutputLog _output_2)
          (else
            (Default|CallOnOutputLog "ERROR: Command not found")))))))

(fn GetProgramfromInput
  (params (Input :type String))
  (bind (_program _isfound) (CallFunction|FindProgram (Variables|Default|GetActiveShell) Input))
  (if _isfound
    (return _program true)
    (else
      (for _array_element (Variables|Default|GetShellPaths)
        (if (!= _array_element (Variables|Default|GetActiveShell))
          (bind (_program_2 _isfound_2) (CallFunction|FindProgram _array_element Input))
          (if _isfound_2
            (return _program_2 true)
            (else
              (return 0 false))))))))

(fn SearchforProgram
  (params (Input :type Array%20of%20Strings))
  (bind (_program _isfound) (CallFunction|GetProgramfromInput (Utilities|Array|Get(acopy) Input)))
  (if _isfound
    (LocalVariables|SetFoundProgram _program)
    (return Input (LocalVariables|GetFoundProgram) true)
    (else
      (return 0 0 false))))

(fn SearchforCommand
  (params (Input :type Array%20of%20Strings))
  (bind (_class _isfound) (CallFunction|GetTerminalCommandfromInput (Utilities|Array|Get(acopy) Input) (Variables|Default|GetTerminalCommands)))
  (if _isfound
    (LocalVariables|SetFoundProcess _class)
    (Utilities|Array|RemoveIndex Input)
    (return Input (LocalVariables|GetFoundProcess) true (LocalVariables|GetOutReadAccess))))

(fn Orbit
  (params (DeltaTime :type Float%20%28double-precision%29))
  (if (Variables|Default|GetDoOrbit)
    (Transformation|AddWorldRotation (Variables|Default|GetAnchor) (* (Math|Rotator|MakeRotator 0.0 0.0 1e+01) DeltaTime) false false)))

(fn Zoom
  (params (DeltaTime :type Float%20%28double-precision%29))
  (if (< (Variables|Default|GetCurrentZoomTime) (Variables|Default|GetZoomTime))
    (Variables|Default|SetCurrentZoomTime (+ DeltaTime (Variables|Default|GetCurrentZoomTime)))
    (Transformation|SetWorldLocation (Variables|Default|GetAnchor) (Math|Vector|Lerp(Vector) (Variables|Default|GetZoomStart) (Transformation|GetActorLocation (Variables|Default|GetFocusShell)) (/ (Variables|Default|GetCurrentZoomTime) (Variables|Default|GetZoomTime))) false false)
    (else
      (Variables|Default|SetDoOrbit true))))

(fn StartZoom
  (params (Shell :type BP%20Shell%20Object%20Reference) (Forced :type Boolean))
  (if (or Forced (!= Shell (Variables|Default|GetFocusShell)))
    (Variables|Default|SetFocusShell Shell)
    (Variables|Default|SetCurrentZoomTime 0.0)
    (Variables|Default|SetZoomStart (Transformation|GetWorldLocation (Variables|Default|GetAnchor)))
    (Variables|Default|SetDoOrbit false)))

(fn GetMusicFOV
  (bind _asbp_game_manager (Utilities|Casting|CastToBP_GameManager (Game|GetGameMode)))
  (return (+ (* (Variables|Default|GetBumpMult) (Math|Float|Power (- (Variables|/Game/GameMode/BP_GameManager.BP_GameManager_C|GetMusicLoudness _asbp_game_manager) 1.0) 2.0)) (Variables|Default|GetDefaultFOV))))