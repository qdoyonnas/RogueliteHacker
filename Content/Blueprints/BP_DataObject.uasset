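; BP_DataObject is a data file with name, size and tags that occupies space in a Shell.
; Setup destroys the actor if the Shell lacks capacity, while assigning and deleting register or remove it alongside the parent class logic.
; Its flat scale derives from SizeRatio on construction and assignment.
; GetInfo formats its details and can grant read access, and Duplicate spawns a copy with the same properties.
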(fn ConstructionScript
  (CallFunction|CalculateSize))

(fn CalculateSize
  (bind _ratio (Utilities|SizeRatio))
  (bind _returnvalue (* _ratio 2.0))
  (Transformation|SetRelativeScale3D (Variables|Default|GetScale) (Math|Vector|MakeVector _returnvalue _returnvalue 0.2)))

(fn Delete
  (Default|RemoveDataObject (Variables|Default|GetShell) self)
  (|CallParentFunction false))

(fn AssigntoShell
  (|CallParentFunction)
  (CallFunction|CalculateSize)
  (Default|AddDataObject (Variables|Default|GetShell) self))

(fn Setup
  (bind _canadd (Default|CanAddDataObject (Variables|Default|GetShell) (Variables|Default|GetSize)))
  (if _canadd
    (|CallParentFunction)
    (else
      (Actor|DestroyActor))))

(fn GetInfo
  (params (withReadAccess :type Boolean))
  (Variables|Default|SetreadAccess (or withReadAccess (Variables|Default|GetreadAccess)))
  (LocalVariables|SetTagOutput (Utilities|Array|Get(acopy) (Variables|Default|GetDataTags)))
  (for (_array_element _array_index) (Variables|Default|GetDataTags)
    (if (!= _array_index 0)
      (LocalVariables|SetTagOutput (Utilities|String|Append (LocalVariables|GetTagOutput) ", " _array_element))))
  (return (Utilities|Text|FormatText "{name} ... {tags} ... {size} " (Variables|Default|GetFileName) (LocalVariables|GetTagOutput) (Variables|Default|GetSize))))

(fn Duplicate
  (bind _returnvalue (Game|SpawnActorfromClass (Utilities|GetClass self) (Math|Transform|MakeTransform "0, 0, 0") "Undefined" "MultiplyWithRoot" 0 (Variables|Default|GetSize) (Variables|Default|GetFileName) (Variables|Default|GetDataTags) (Variables|Default|GetShell) (Variables|Default|GetreadAccess) false 0))
  (return _returnvalue))