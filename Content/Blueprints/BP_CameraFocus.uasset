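; Camera focus point that registers with the game manager's CameraPawn to compete for the camera's attention.
; Registration inserts it into the pawn's focus list by priority, and an optional timeline scales that priority over time by re-registering.
; After zoom ends, the anchor rotation eases to zero, then loops a yaw orbit while focus stays active.
; Losing focus stops the orbit and clears any linked secondary focus, which unregistering also clears.
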(event Custom|StartAnchorOrbit
  (bind _lerp (Timeline|AnchorOrbitTimeline PlayFromStart)
    (:Update
      (Transformation|SetRelativeRotation (Variables|Components|GetRotation) (Math|Rotator|Lerp(Rotator) (Variables|Default|GetAnchorStartRotator) (Variables|Default|GetAnchorOrbitRotator) _lerp) false false))
    (:Finished
      (if (== (Variables|/Game/Blueprints/BP_Camera.BP_Camera_C|GetActiveFocus (Variables|Default|GetCamera%20Pawn)) self)
        (CallFunction|PlayAnchorOrbit)))))

(event Custom|StartDegrade
  (params (Rate :type Float%20%28double-precision%29))
  (if (!= Rate 0.0)
    (Variables|Default|SetStartFocusPriority (Variables|Default|GetCurrentFocusPriority))
    (Components|Timeline|SetPlayRate (Variables|Default|GetDegradeTimeline) Rate)
    (bind _value (Timeline|DegradeTimeline PlayFromStart)
      (:Update
        (CallFunction|RegisterCameraFocus (* (Variables|Default|GetStartFocusPriority) _value) 0.0 (Variables|Default|GetZoomRate) true false false))
      (:Finished
        (if (<= (Variables|Default|GetCurrentFocusPriority) 0.0)
          (CallFunction|UnregisterCameraFocus false))))))

(event Custom|PlayAnchorOrbit
  (bind _angle (Timeline|Timeline PlayFromStart)
    (:Update
      (Transformation|SetRelativeRotation (Variables|Components|GetRotation) (Math|Vector|RotatorfromAxisandAngle "0.000000,0.000000,1.000000" _angle) false false))
    (:Finished
      (if (== (Variables|/Game/Blueprints/BP_Camera.BP_Camera_C|GetActiveFocus (Variables|Default|GetCamera%20Pawn)) self)
        (CallFunction|PlayAnchorOrbit)))))

(event Custom|StopAnchorOrbit
  (bind _angle (Timeline|Timeline Stop)
    (:Update
      (Transformation|SetRelativeRotation (Variables|Components|GetRotation) (Math|Vector|RotatorfromAxisandAngle "0.000000,0.000000,1.000000" _angle) false false))
    (:Finished
      (if (== (Variables|/Game/Blueprints/BP_Camera.BP_Camera_C|GetActiveFocus (Variables|Default|GetCamera%20Pawn)) self)
        (CallFunction|PlayAnchorOrbit)))))

(event EventDestroyed
  (CallFunction|UnregisterCameraFocus (== (Variables|/Game/Blueprints/BP_Camera.BP_Camera_C|GetActiveFocus (Variables|Default|GetCamera%20Pawn)) self)))

(event EventBeginPlay
  (bind _asbp_game_manager (Utilities|Casting|CastToBP_GameManager (Game|GetGameMode)))
  (Variables|Default|SetCamera%20Pawn (Variables|/Game/GameMode/BP_GameManager.BP_GameManager_C|GetCameraPawn _asbp_game_manager)))

(fn ConstructionScript)

(fn GetFocusAnchor
  (return (Variables|Components|GetCameraAnchor)))

(fn GetFocusPriority
  (return (Variables|Default|GetCurrentFocusPriority)))

(fn UnregisterCameraFocus
  (params (Interrupt :type Boolean))
  (Default|UnregisterFocus (Variables|Default|GetCamera%20Pawn) self Interrupt)
  (CallFunction|ClearSecondaryFocus))

(fn RegisterCameraFocus
  (params (Priority :type Float%20%28double-precision%29) (DegradeRate :type Float%20%28double-precision%29) (ZoomRate :type Float%20%28double-precision%29) (BeforeEqual :type Boolean) (Interrupt :type Boolean) (Fallback :type Boolean))
  (Variables|Default|SetCurrentFocusPriority Priority)
  (Variables|Default|SetZoomRate ZoomRate)
  (CallFunction|UnregisterCameraFocus false)
  (bind _index (CallFunction|GetPriorityIndex BeforeEqual))
  (Default|RegisterFocus (Variables|Default|GetCamera%20Pawn) self _index Interrupt Fallback)
  (CallFunction|StartDegrade DegradeRate)
  (return))

(fn SetSecondaryFocus
  (params (CameraFocus :type BP%20Camera%20Focus%20Object%20Reference) (Input :type Array%20of%20Strings))
  (if (and (!= CameraFocus self) (!= CameraFocus (Variables|Default|GetSecondaryFocus)))
    (CallFunction|ClearSecondaryFocus)
    (Variables|Default|SetSecondaryFocus CameraFocus)
    (return true)
    (else
      (return false))))

(fn ClearSecondaryFocus
  (Utilities|FlowControl|Sequence
    (:then_0
      (if (and (Utilities|IsValid (Variables|Default|GetSecondaryFocus)) (!= (Variables|Default|GetSecondaryFocus) self))
        (CallFunction|UnregisterCameraFocus (Variables|Default|GetSecondaryFocus) false)))
    (:then_1
      (Variables|Default|SetSecondaryFocus 0))))

(fn GetPriorityIndex
  (params (BeforeEqual :type Boolean))
  (bind _camera_pawn (Variables|Default|GetCamera%20Pawn))
  (bind _focusobjects (Variables|/Game/Blueprints/BP_Camera.BP_Camera_C|GetFocusObjects _camera_pawn))
  (for (_array_element _array_index) _focusobjects
    (LocalVariables|SetCurrentIndex _array_index)
    (bind _priority (CallFunction|GetFocusPriority _array_element))
    (Math|Float|CompareFloat _priority (Variables|Default|GetCurrentFocusPriority)
      (:==
        (if BeforeEqual
          (return (LocalVariables|GetCurrentIndex))))
      (:<
        (return (LocalVariables|GetCurrentIndex)))))
  (return (Utilities|Array|Length _focusobjects)))

(fn FocusUpdate
  (params (DeltaTime :type Float%20%28double-precision%29)))

(fn CameraZoomEnded
  (CallFunction|SetupAnchorOrbit))

(fn GetAnchorasSecondaryFocus
  (return (Variables|Components|GetDefaultSceneRoot)))

(fn CameraZoomStarted
  (bind _rotation (CallFunction|Pointat (Variables|/Game/Blueprints/BP_Camera.BP_Camera_C|GetDefaultSceneRoot (Variables|Default|GetCamera%20Pawn)) (Variables|Components|GetRotation)))
  (Transformation|SetWorldRotation (Variables|Components|GetRotation) (Math|Rotator|MakeRotator (.Roll (Math|Rotator|BreakRotator _rotation)) (+ (.Pitch (Math|Rotator|BreakRotator _rotation)) 7e+01) (.Yaw (Math|Rotator|BreakRotator _rotation))) false false))

(fn LostCameraFocus
  (params (ToFocus :type BP%20Camera%20Focus%20Object%20Reference))
  (CallFunction|StopAnchorOrbit)
  (CallFunction|ClearSecondaryFocus))

(fn SetupAnchorOrbit
  (Variables|Default|SetAnchorOrbitRotator "0, 0, 0")
  (Variables|Default|SetAnchorStartRotator (Variables|/Script/Engine.SceneComponent|GetRelativeRotation (Variables|Components|GetRotation)))
  (CallFunction|StartAnchorOrbit))

(fn GetPopupInfo
  (params (Parameters :type Array%20of%20Strings))
  (return "DEFAULT TEXT"))