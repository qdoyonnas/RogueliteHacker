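; Prog_Root is the root program of the player's interpreter, resolving command aliases into spawned process actors, with its deletion printing "GAME OVER".
; Setup maps each alias from the RootPrograms data table's process classes to its class, and binds to the network-loaded event.
; Once the network loads, it makes its shell the interpreter's active, focused shell and grants read access to its data objects.
; StartProcess looks up the first parameter and spawns that class using its defaults.
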(fn ConstructionScript
  (|CallParentFunction))

(fn SetupProgram
  (params (Tags :type Array%20of%20Strings) (Properties :type Map%20of%20Strings%20to%20Strings))
  (bind _asbp_game_manager (Utilities|Casting|CastToBP_GameManager (Game|GetGameMode)))
  (EventDispatchers|BindEventtoNetworkLoaded (Variables|/Game/GameMode/BP_GameManager.BP_GameManager_C|GetNetworkBuilder _asbp_game_manager) (EventDispatchers|CreateEvent :!event OnNetworkLoaded))
  (CallFunction|SetupRootProgram)
  (return))

(fn OnNetworkLoaded
  (CallFunction|SetupInterpreter)
  (CallFunction|SetupRootShell))

(fn SetupRootProgram
  (bind _outrownames (DataTable|GetDataTableRowNames (Variables|Default|GetRootPrograms)))
  (for _array_element _outrownames
    (bind _returnvalue (Utilities|GetDataTableRow (Variables|Default|GetRootPrograms) _array_element)
      (:then
        (for _array_element_2 (.Aliases (Utilities|GetClassDefaults (Utilities|Struct|BreakStruct_Command _returnvalue)))
          (Utilities|Array|AddUnique (Variables|Default|GetAliases) _array_element_2)
          (Utilities|Map|Add (Variables|Default|GetMappedAliases) _array_element_2 (Utilities|Struct|BreakStruct_Command _returnvalue)))))))

(fn SetupInterpreter
  (bind _asbp_interpreter (Utilities|Casting|CastToBP_Interpreter (Game|Player|GetPlayerPawn 0)))
  (bind _output_get (Variables|Default|SetInterpreter _asbp_interpreter))
  (Variables|/Game/Blueprints/BP_Interpreter.BP_Interpreter_C|SetFocusShell _output_get (Variables|Default|GetShell))
  (bind _output_get_2 (Variables|/Game/Blueprints/BP_Interpreter.BP_Interpreter_C|SetActiveShell _output_get (Variables|Default|GetShell)))
  (Utilities|Array|Add (Variables|/Game/Blueprints/BP_Interpreter.BP_Interpreter_C|GetShellPaths _output_get) _output_get_2)
  (Variables|/Game/Blueprints/BP_Interpreter.BP_Interpreter_C|SetRootProgram (Variables|Default|GetInterpreter) self))

(fn SetupRootShell
  (bind _shell (Variables|Default|GetShell))
  (Variables|/Game/Blueprints/BP_Shell.BP_Shell_C|SetReadAccess _shell true)
  (for _array_element (Variables|/Game/Blueprints/BP_Shell.BP_Shell_C|GetDataObjects _shell)
    (Variables|/Game/Blueprints/BP_ShellObject.BP_ShellObject_C|SetreadAccess _array_element true)))

(fn Delete
  (|CallParentFunction)
  (Development|PrintString "GAME OVER"))

(fn Setup
  (|CallParentFunction)
  (CallFunction|SetupProgram 0 (Utilities|Map|MakeMap "" "")))

(fn StartProcess
  (params (Params :type Array%20of%20Strings) (IsPlayerOwned :type Boolean))
  (bind _process (CallFunction|StartProcessfromType Params (.Value (Utilities|Map|Find (Variables|Default|GetMappedAliases) (Utilities|Array|Get(acopy) Params))) IsPlayerOwned))
  (CallFunction|PlayStart)
  (return "" _process))

(fn StartProcessfromType
  (params (Params :type Array%20of%20Strings) (Type :type BP%20Process%20Class%20Reference) (IsPlayerOwned :type Boolean))
  (bind (_program _params _onoutput _nextsend _packetcount _packetrate _packetspeed _sendpackettimestamp _dosendpacket _aliases _targetedshellobject _landedpackets _load _datatags _navigationprocess _threads) (Utilities|GetClassDefaults Type))
  (Utilities|Array|RemoveIndex Params)
  (bind _returnvalue (Game|SpawnActorfromClass Type (Math|Transform|MakeTransform "0, 0, 0") "Undefined" "MultiplyWithRoot" 0 self Params _packetcount _packetrate _packetspeed _load _threads IsPlayerOwned (Variables|Default|GetShell) (Variables|Default|GetreadAccess) false 0))
  (return _returnvalue))