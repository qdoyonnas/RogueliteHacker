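; BP_Packet is an actor representing a packet that a Process sends through a network of Shells, visible only where there is read access.
; One timeline lerps its point between components, and each finish advances a travel-state machine unless an Interceptor takes over.
; It follows a Path by link name, detours through any NavigationProcess, reports arrival and landing to its Process, then destroys itself.
; It also dies with its Process.
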(event Custom|StartTransition
  (bind _alpha (Timeline|TransitionTimeline PlayFromStart)
    (:Update
      (CallFunction|Transition _alpha))
    (:Finished
      (CallFunction|CalcNextStep))))

(event EventBeginPlay
  (CallFunction|Setup))

(fn ConstructionScript)

(fn Setup
  (CallFunction|StartShellObjectTransition (Variables|Default|GetProcess) false (Variables|Default|GetSpeed))
  (EventDispatchers|BindEventtoOnDelete (Variables|Default|GetProcess) (EventDispatchers|CreateEvent :!event OnProcessDeleted))
  (Variables|Default|SetTravelState "NewEnumerator0")
  (Variables|Default|SetOriginShell (Variables|Default|GetShell))
  (CallFunction|SetVisible (Variables|Default|GetReadAccess)))

(fn Transition
  (params (Alpha :type Float%20%28double-precision%29))
  (bind _targetcomponent (Variables|Default|GetTargetComponent))
  (Utilities|IsValid _targetcomponent
    (:Is%20Valid
      (Transformation|SetWorldLocation (Variables|Default|GetPoint) (Math|Vector|Lerp(Vector) (Variables|Default|GetStartingLocation) (Transformation|GetWorldLocation _targetcomponent) Alpha) false false)
      (Variables|Default|GetShell
        (:then
          (CallFunction|PointatShell))
        (:else)))))

(fn StartShellObjectTransition
  (params (Object :type BP%20Shell%20Object%20Object%20Reference) (isGoingTo :type Boolean) (InSpeed :type Float%20%28double-precision%29))
  (bind _output_get (Variables|Default|SetTargetShellObject Object))
  (Transformation|AttachComponentToComponent (Variables|/Game/Blueprints/BP_ShellObject.BP_ShellObject_C|GetAnchor _output_get) "None" "SnapToTarget" "SnapToTarget" "KeepRelative" true)
  (bind _output_get_2 (Variables|Default|SetStartingLocation (Transformation|GetWorldLocation (Utilities|GetTargetComponent (not isGoingTo)))))
  (Transformation|SetWorldLocation (Variables|Default|GetPoint) _output_get_2 false false)
  (Variables|Default|SetTargetComponent (Utilities|GetTargetComponent isGoingTo))
  (Components|Timeline|SetPlayRate (Variables|Default|GetTransitionTimeline) InSpeed)
  (CallFunction|StartTransition))

(fn StartShellTransition
  (params (InShell :type BP%20Shell%20Object%20Reference) (InSpeed :type Float%20%28double-precision%29) (StartLocation :type Vector) (UsingLink :type Boolean))
  (Variables|Default|SetTargetShellObject 0)
  (Transformation|AttachComponentToComponent (Variables|/Game/Blueprints/BP_Shell.BP_Shell_C|GetPoint InShell) "None" "SnapToTarget" "KeepRelative" "KeepRelative" true)
  (bind _output_get (Variables|Default|SetStartingLocation StartLocation))
  (Transformation|SetWorldLocation (Variables|Default|GetPoint) _output_get false false)
  (Variables|Default|SetTargetComponent (Variables|/Game/Blueprints/BP_Shell.BP_Shell_C|GetPoint InShell))
  (Variables|Default|SetUsingLink UsingLink)
  (Variables|Default|SetIsHandled false)
  (Components|Timeline|SetPlayRate (Variables|Default|GetTransitionTimeline) InSpeed)
  (CallFunction|StartTransition)
  (Default|PacketApproaching InShell self (Variables|Default|GetShell))
  (Variables|Default|SetLastShell (Variables|Default|GetShell))
  (Variables|Default|SetShell InShell)
  (CallFunction|PointatShell)
  (CallFunction|SetVisible (Variables|/Game/Blueprints/BP_Shell.BP_Shell_C|GetReadAccess InShell)))

(fn HandleNavigation
  (bind _shell (Variables|Default|GetShell))
  (bind _navigationprocess (Variables|Default|GetNavigationProcess)
    (:then
      (if (== (Variables|Default|GetShell) (Variables|/Game/Blueprints/BP_ShellObject.BP_ShellObject_C|GetShell _navigationprocess))
        (CallFunction|StartShellObjectTransition _navigationprocess true (Variables|Default|GetSpeed))
        (Variables|Default|SetTravelState "NewEnumerator3")
        (else
          (if (== (Utilities|Array|Length (Variables|Default|GetPath)) (Variables|Default|GetPathIndex)) :!label _label
            (Variables|Default|SetTravelState "NewEnumerator2")
            (Default|CallOnArriveatShell _shell)
            (bind _process (Variables|Default|GetProcess)
              (:then
                (Default|OnPacketArrived _process _shell self))
              (:else))
            (else
              (CallFunction|PathtoNextShell))))))
    (:else
      (goto _label))))

(fn PointatShell
  (bind _shell (Variables|Default|GetShell))
  (Utilities|IsValid _shell
    (:Is%20Valid
      (bind _rotation (CallFunction|Pointat (Variables|Default|GetPoint) (Variables|/Game/Blueprints/BP_Shell.BP_Shell_C|GetPoint _shell)))
      (Transformation|SetWorldRotation (Variables|Default|GetAnchor) _rotation false false))))

(fn CalcNextStep
  (bind _shell (Variables|Default|GetShell))
  (bind _interceptor (Variables|Default|GetInterceptor)
    (:then
      (Default|InterceptPacket _interceptor self))
    (:else
      (switch Utilities|FlowControl|Switch|SwitchonEnum_PacketTravelState (Variables|Default|GetTravelState)
        (:NewEnumerator0
          (bind _shell_2 (Variables|Default|GetShell :!label _label)
            (:then
              (Default|PlayPulse _shell_2))
            (:else
              _))
          (CallFunction|HandleNavigation))
        (:NewEnumerator1
          (goto _label))
        (:NewEnumerator3
          (Default|ForwardPacket (Variables|Default|GetNavigationProcess) self))
        (:NewEnumerator2
          (Default|CallOnLandatTarget _shell)
          (Default|OnPacketLanded (Variables|Default|GetProcess) _shell self)
          (Actor|DestroyActor)
          (bind _targetshellobject (Variables|Default|GetTargetShellObject)
            (:then
              (Default|PlayPulse _targetshellobject))
            (:else)))))))

(fn PathtoNextShell
  (Variables|Default|SetTravelState "NewEnumerator1")
  (bind (_isfound _link) (CallFunction|FindLinkonShell (Variables|Default|GetShell) (Utilities|Array|Get(acopy) (Variables|Default|GetPath) (Variables|Default|GetPathIndex))))
  (if _isfound
    (Default|ForwardPacket _link self)
    (Math|Integer|IncrementInt (Variables|Default|GetPathIndex))
    (else
      (Default|Delete (Variables|Default|GetProcess) false)
      (Actor|DestroyActor)
      (Default|Print (Variables|Default|GetProcess) (Utilities|Text|FormatText "Error: Link to \"{path}\" not found" (Utilities|Array|Get(acopy) (Variables|Default|GetPath) (Variables|Default|GetPathIndex)))))))

(fn Intercept
  (params (InterceptorProcess :type BP%20Process%20Object%20Reference))
  (bind _process (Variables|Default|GetProcess)
    (:then
      (Default|PacketIntercepted _process self InterceptorProcess))
    (:else)))

(fn Delete
  (params (SkipAnimation :type Boolean))
  (Default|CallOnDelete)
  (Actor|DestroyActor))

(fn SetVisible
  (params (NewState :type Boolean))
  (bind _output_get (Variables|Default|SetReadAccess NewState))
  (Rendering|SetActorHiddenInGame (not _output_get)))

(fn OnProcessDeleted
  (params (ShellObject :type BP%20Shell%20Object%20Object%20Reference) (SkipAnimation :type Boolean))
  (CallFunction|Delete SkipAnimation))