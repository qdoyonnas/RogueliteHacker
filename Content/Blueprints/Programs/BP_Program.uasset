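; BP_Program is a base program for a shell-style terminal system, with placeholder Parse, Validate and Call functions that report failure or return empty text.
; StartProcess either calls a terminal command directly or spawns a ProcessType actor with the program, parameters, packet settings and shell, returning a starting message.
; Terminal commands skip parent shell assignment, and their base Call destroys the actor.
; SetupProgram copies supplied tags into DataTags.
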(fn ConstructionScript
  (|CallParentFunction))

(fn Parse
  (params (Params :type Array%20of%20Strings))
  (return "BaseParse" false))

(fn Call
  (params (Params :type Array%20of%20Strings))
  (if (Variables|Default|GetIsTerminalCommand)
    (Actor|DestroyActor))
  (return ""))

(fn Validate
  (params (Params :type Array%20of%20Strings))
  (return false ""))

(fn SetupProgram
  (params (Tags :type Array%20of%20Strings) (Properties :type Map%20of%20Strings%20to%20Strings))
  (for _array_element Tags
    (Utilities|Array|Add (Variables|Default|GetDataTags) _array_element)))

(fn StartProcess
  (params (Params :type Array%20of%20Strings))
  (if (Variables|Default|GetIsTerminalCommand)
    (bind _output (CallFunction|Call Params))
    (return _output)
    (else
      (Game|SpawnActorfromClass (Variables|Default|GetProcessType) (Math|Transform|MakeTransform "0, 0, 0" (Transformation|GetWorldRotation (Variables|Default|GetAnchor))) "Undefined" "MultiplyWithRoot" 0 self Params (Variables|Default|GetPacketCount) (Variables|Default|GetPacketRate) (Variables|Default|GetPacketSpeed) 0 (Variables|Default|GetShell) 0)
      (return (Utilities|Text|FormatText "Starting {fileName} process..." (Utilities|String|ToLower (Variables|Default|GetFileName)))))))

(fn AssigntoShell
  (if (not (Variables|Default|GetIsTerminalCommand))
    (|CallParentFunction)))