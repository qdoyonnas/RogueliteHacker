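; Root access program that gives the player's interpreter a readable starting point in its Shell once the network has loaded.
; On BeginPlay it binds OnNetworkLoaded to the game manager's NetworkBuilder event.
; When that fires, it makes its Shell the interpreter's active shell, appends it to the shell paths, and grants read access to the Shell and all its data objects.
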(event EventBeginPlay
  (|CallParentFunction)
  (bind _asbp_game_manager (Utilities|Casting|CastToBP_GameManager (Game|GetGameMode)))
  (EventDispatchers|BindEventtoNetworkLoaded (Variables|/Game/GameMode/BP_GameManager.BP_GameManager_C|GetNetworkBuilder _asbp_game_manager) (EventDispatchers|CreateEvent :!event OnNetworkLoaded)))

(fn ConstructionScript
  (|CallParentFunction))

(fn OnNetworkLoaded
  (bind _shell (Variables|Default|GetShell))
  (bind _asbp_interpreter (Utilities|Casting|CastToBP_Interpreter (Game|Player|GetPlayerPawn 0)))
  (bind _output_get (Variables|/Game/Blueprints/BP_Interpreter.BP_Interpreter_C|SetActiveShell _asbp_interpreter (Variables|Default|GetShell)))
  (Utilities|Array|Add (Variables|/Game/Blueprints/BP_Interpreter.BP_Interpreter_C|GetShellPaths _asbp_interpreter) _output_get)
  (Variables|/Game/Blueprints/BP_Shell.BP_Shell_C|SetReadAccess _shell true)
  (for _array_element (Variables|/Game/Blueprints/BP_Shell.BP_Shell_C|GetDataObjects _shell)
    (Variables|/Game/Blueprints/BP_DataObject.BP_DataObject_C|SetReadAccess _array_element true)))