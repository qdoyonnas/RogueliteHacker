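; Camera actor that travels between registered focus objects, keeping an ordered focus list with a fallback for when it empties.
; StartZoom targets the first entry, lerping to its anchor on a timeline at that focus's ZoomRate, or jumping for high rates.
; EndZoom attaches to the anchor and starts a delay timer, while Tick updates the active focus.
; It also computes a music-loudness-driven FOV and opens the main menu on input.
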(event Custom|PlayZoom
  (bind _activefocus (Variables|Default|GetActiveFocus))
  (Utilities|IsValid (Variables|Default|GetActiveFocus)
    (:Is%20Valid
      (Default|CameraZoomStarted (Variables|Default|GetActiveFocus))
      (bind _alpha (Timeline|ZoomTimeline PlayFromStart)
        (:Update
          (CallFunction|Zoom _alpha))
        (:Finished
          (Utilities|IsValid _activefocus
            (:Is%20Valid
              (Default|CameraZoomEnded _activefocus))
            (:Is%20Not%20Valid
              _))
          (CallFunction|EndZoom))))
    (:Is%20Not%20Valid
      (CallFunction|EndZoom))))

(event Input|EnhancedActionEvents|EnhancedInputActionIA_OpenMenu
  (params (ActionValue :type Boolean) (ElapsedSeconds :type Float%20%28double-precision%29) (TriggeredSeconds :type Float%20%28double-precision%29) (InputAction :type Input%20Action%20Object%20Reference :default "/Game/GameMode/Inputs/IA_OpenMenu.IA_OpenMenu"))
  (Game|OpenLevel(byName) "LVL_MainMenu"))

(event EventTick
  (params (DeltaSeconds :type Float%20%28single-precision%29))
  (bind _activefocus (Variables|Default|GetActiveFocus)
    (:then
      (Default|FocusUpdate _activefocus DeltaSeconds))
    (:else)))

(fn ConstructionScript)

(fn Zoom
  (params (Alpha :type Float%20%28double-precision%29))
  (bind _activefocus (Variables|Default|GetActiveFocus)
    (:then
      (bind _focus (Default|GetFocusAnchor _activefocus))
      (Transformation|SetWorldTransform (Variables|Default|GetDefaultSceneRoot) (Math|Transform|Lerp(Transform) (Variables|Default|GetZoomStart) (Math|Transform|MakeTransform (.Location (Math|Transform|BreakTransform (Transformation|GetWorldTransform _focus))) (Math|Rotator|MakeRotator 0.0 (.Pitch (Math|Rotator|BreakRotator (.Rotation (Math|Transform|BreakTransform (Transformation|GetWorldTransform _focus))))) (.Yaw (Math|Rotator|BreakRotator (.Rotation (Math|Transform|BreakTransform (Transformation|GetWorldTransform _focus)))))) (.Scale (Math|Transform|BreakTransform (Transformation|GetWorldTransform _focus)))) Alpha) false false)
      (Variables|Default|SetActiveZoom (> Alpha 0.001)))
    (:else)))

(fn StartZoom
  (if (!= (Utilities|Array|Get(acopy) (Variables|Default|GetFocusObjects)) (Variables|Default|GetActiveFocus))
    (Transformation|DetachFromActor "KeepWorld" "KeepWorld" "KeepWorld")
    (Utilities|FlowControl|Sequence
      (:then_0
        (bind _activefocus (Variables|Default|GetActiveFocus)
          (:then
            (LocalVariables|SetTempFocus _activefocus)
            (Variables|Default|SetActiveFocus 0)
            (Default|LostCameraFocus (LocalVariables|GetTempFocus) (Utilities|Array|Get(acopy) (Variables|Default|GetFocusObjects))))
          (:else)))
      (:then_1
        (Variables|Default|SetActiveFocus (Utilities|Array|Get(acopy) (Variables|Default|GetFocusObjects)))
        (CallFunction|SetStartZoom)
        (if (< (Variables|/Game/Blueprints/BP_CameraFocus.BP_CameraFocus_C|GetZoomRate (Variables|Default|GetActiveFocus)) 1e+02)
          (Components|Timeline|SetPlayRate (Variables|Default|GetZoomTimeline) (Variables|/Game/Blueprints/BP_CameraFocus.BP_CameraFocus_C|GetZoomRate (Variables|Default|GetActiveFocus)))
          (CallFunction|PlayZoom)
          (else
            (CallFunction|JumpCamera)))))
    (else
      (bind _returnvalue (Utilities|Time|SetTimerbyEvent (EventDispatchers|CreateEvent :!event StartZoom) (Variables|Default|GetDelayAfterZoom)))
      (Variables|Default|SetNextZoomTimer _returnvalue))))

(fn GetMusicFOV
  (bind _asbp_game_manager (Utilities|Casting|CastToBP_GameManager (Game|GetGameMode)))
  (return (+ (* (Variables|Default|GetBumpMult) (Math|Float|Power (- (Variables|/Game/GameMode/BP_GameManager.BP_GameManager_C|GetMusicLoudness _asbp_game_manager) 1.0) 2.0)) (Variables|Default|GetDefaultFOV))))

(fn EndZoom
  (Variables|Default|SetActiveZoom false)
  (CallFunction|SetStartZoom)
  (Utilities|FlowControl|Sequence
    (:then_0
      (bind _activefocus (Variables|Default|GetActiveFocus)
        (:then
          (bind _focus (Default|GetFocusAnchor _activefocus))
          (Transformation|AttachComponentToComponent _focus "None" "SnapToTarget" "KeepWorld" "KeepWorld" false))
        (:else)))
    (:then_1
      (bind _returnvalue (Utilities|Time|SetTimerbyEvent (EventDispatchers|CreateEvent :!event StartZoom) (Variables|Default|GetDelayAfterZoom)))
      (Variables|Default|SetNextZoomTimer _returnvalue))))

(fn Setup
  (Variables|Default|SetDefaultFOV (Variables|/Script/Engine.CameraComponent|GetFieldOfView (Variables|Default|GetCamera)))
  (Transformation|SetWorldLocation (Variables|Default|GetDefaultSceneRoot) (* (Math|Random|RandomUnitVector) 1e+04) false true))

(fn RegisterFocus
  (params (Focus :type BP%20Camera%20Focus%20Object%20Reference) (Index :type Integer) (Interrupt :type Boolean) (Fallback :type Boolean))
  (Utilities|IsValid Focus
    (:Is%20Valid
      (Utilities|FlowControl|Sequence
        (:then_0
          (if Fallback
            (CallFunction|SetFallback Focus)))
        (:then_1
          (if (< Index (Utilities|Array|Length (Variables|Default|GetFocusObjects)))
            (Utilities|Array|Insert (Variables|Default|GetFocusObjects) Focus Index)
            (else
              (Utilities|Array|Add (Variables|Default|GetFocusObjects) Focus)))
          (if Interrupt
            (Utilities|FlowControl|Sequence
              (:then_0
                (bind _activefocus (Variables|Default|GetActiveFocus)
                  (:then
                    (Default|CameraZoomEnded _activefocus))
                  (:else)))
              (:then_1
                (CallFunction|StartZoom)))))))))

(fn UnregisterFocus
  (params (Focus :type BP%20Camera%20Focus%20Object%20Reference) (Interrupt :type Boolean))
  (bind _returnvalue (Utilities|Array|RemoveItem (Variables|Default|GetFocusObjects) Focus))
  (if _returnvalue
    (Utilities|FlowControl|Sequence
      (:then_0
        (if (== (Utilities|Array|Length (Variables|Default|GetFocusObjects)) 0)
          (Utilities|Array|Add (Variables|Default|GetFocusObjects) (Variables|Default|GetFallbackObject))
          (CallFunction|StartZoom)))
      (:then_1
        (if Interrupt
          (CallFunction|StartZoom))))))

(fn SetFallback
  (params (Focus :type BP%20Camera%20Focus%20Object%20Reference))
  (Utilities|Array|RemoveItem (Variables|Default|GetFocusObjects) (Variables|Default|GetFallbackObject))
  (bind _output_get (Variables|Default|SetFallbackObject Focus))
  (if (== _output_get 0)
    (bind _asbp_game_manager (Utilities|Casting|CastToBP_GameManager (Game|GetGameMode)))
    (Variables|Default|SetFallbackObject (Variables|/Game/Blueprints/BP_Interpreter.BP_Interpreter_C|GetRootShell (Variables|/Game/GameMode/BP_GameManager.BP_GameManager_C|GetInterpreter _asbp_game_manager)))))

(fn JumpCamera
  (bind _activefocus (Variables|Default|GetActiveFocus)
    (:then
      (bind _focus (Default|GetFocusAnchor _activefocus))
      (Transformation|SetWorldTransform (Variables|Default|GetDefaultSceneRoot) (Transformation|GetWorldTransform _focus) false false)
      (CallFunction|EndZoom))
    (:else)))

(fn SetStartZoom
  (bind _returnvalue (Transformation|GetActorTransform))
  (bind (_location _rotation _scale) (Math|Transform|BreakTransform _returnvalue))
  (bind (_roll _pitch _yaw) (Math|Rotator|BreakRotator _rotation))
  (Variables|Default|SetZoomStart (Math|Transform|MakeTransform _location (Math|Rotator|MakeRotator 0.01 _pitch _yaw) _scale)))