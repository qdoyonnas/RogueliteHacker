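; BP_NetworkEvent broadcasts an event from an origin shell across the network of linked shells on behalf of a sender process.
; It follows Link processes to each untravelled shell and spawns a packet actor carrying the event details.
; Each arrival notifies that shell and floods onward, with a visited list preventing repeats.
; It destroys itself when no packets remain active, and binds to the sender's deletion.
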(event EventBeginPlay
  (Utilities|Array|Add (Variables|Default|GetTravelledShells) (Variables|Default|GetOrigin))
  (CallFunction|SendThroughLinks (Variables|Default|GetOrigin))
  (EventDispatchers|BindEventtoOnDelete (Variables|Default|GetSender) (EventDispatchers|CreateEvent :!event SenderDeleted)))

(fn ConstructionScript)

(fn SendThroughLinks
  (params (Shell :type BP%20Shell%20Object%20Reference))
  (for _array_element (Variables|/Game/Blueprints/GameObjects/BP_Shell.BP_Shell_C|GetProcesses Shell)
    (bind _output_get (LocalVariables|SetAProc _array_element))
    (if (Utilities|Array|ContainsItem (Variables|/Game/Blueprints/Processes/BP_Process.BP_Process_C|GetDataTags _output_get) "Link")
      (bind _assub_proc_connection (Utilities|Casting|CastToSubProc_Connection (LocalVariables|GetAProc)))
      (bind _addressshell (Default|GetAddressShell _assub_proc_connection))
      (bind _output_get_2 (LocalVariables|SetAddressShell _addressshell))
      (if (not (Utilities|Array|ContainsItem (Variables|Default|GetTravelledShells) _output_get_2))
        (Utilities|Array|Add (Variables|Default|GetTravelledShells) (LocalVariables|GetAddressShell))
        (CallFunction|SendEventPacket Shell (LocalVariables|GetAddressShell)))))
  (if (== (Variables|Default|GetActivePackets) 0)
    (Actor|DestroyActor)))

(fn PacketArrived
  (params (AtShell :type BP%20Shell%20Object%20Reference) (Packet :type BP%20Packet%20Object%20Reference))
  (Default|PacketArrived AtShell Packet (Variables|/Game/Blueprints/GameObjects/BP_Packet.BP_Packet_C|GetLastShell Packet))
  (Math|Integer|DecrementInt (Variables|Default|GetActivePackets)
    (:%20%20
      (CallFunction|SendThroughLinks AtShell))))

(fn SenderDeleted
  (params (Object :type BP%20Shell%20Object%20Object%20Reference) (SkipAnimation :type Boolean))
  (Actor|DestroyActor))

(fn SendEventPacket
  (params (SendingShell :type BP%20Shell%20Object%20Reference) (AddressShell :type BP%20Shell%20Object%20Reference))
  (bind _sender (Variables|Default|GetSender))
  (Game|SpawnActorfromClass "/Game/Blueprints/GameObjects/BP_Packet.BP_Packet_C" (Transformation|GetActorTransform SendingShell) "Undefined" "MultiplyWithRoot" 0 (Variables|Default|GetSender) (Utilities|Array|MakeArray (Variables|/Game/Blueprints/GameObjects/BP_Shell.BP_Shell_C|GetName AddressShell)) 0 SendingShell (Variables|/Game/Blueprints/GameObjects/BP_ShellObject.BP_ShellObject_C|GetreadAccess _sender) (Variables|Default|GetEventDetails) (Variables|/Game/Blueprints/Processes/BP_Process.BP_Process_C|GetPacketSpeed _sender) self 0)
  (Math|Integer|IncrementInt (Variables|Default|GetActivePackets)))

(fn HasDetail
  (params (Key :type String) (Value :type String))
  (return (Utilities|Enum|Equal(Enum) (.Value (Utilities|Map|Find (Variables|Default|GetEventDetails) Key)) Value)))

(fn ProcessCount
  (params (Process :type BP%20Process%20Object%20Reference))
  (Utilities|IsValid Process
    (:Is%20Valid
      (bind _count (Default|ProcessCount (Variables|Default|GetOrigin) (Default|GetFirstAlias Process)))
      (return _count))))

(fn ProcessCountbyKey
  (params (Key :type String))
  (return (Helper|ProcessCount (.Value (Utilities|Map|Find (Variables|Default|GetEventProcesses) Key)))))