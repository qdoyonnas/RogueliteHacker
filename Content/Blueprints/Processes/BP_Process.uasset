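; BP_Process is a base program process that runs on a Shell, with Validate, Parse and Run as stubs for child overrides.
; Setup validates params or self-destructs; after installing, it spawns a BP_Packet, parsed on arrival and sent to the targeted shell object, or deleted with the process on failure.
; Landed packets schedule the next timed send until PacketCount is reached, then Run fires.
; It registers threads with its Shell and emits name-tagged output.
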(event EventTick
  (params (DeltaSeconds :type Float%20%28single-precision%29))
  (|CallParentFunction 0.0)
  (if (Variables|Default|GetDoSendPacket)
    (if (>= (Math|DateTime|Now) (Variables|Default|GetSendPacketTimestamp))
      (CallFunction|SendPacket))))

(fn ConstructionScript)

(fn Setup
  (CallFunction|BindEvents)
  (bind (_isvalid _output) (CallFunction|Validate (Variables|Default|GetParams)))
  (if _isvalid
    (|CallParentFunction)
    (Transformation|SetRelativeRotation (Variables|Default|GetAnchor) (Variables|/Script/Engine.SceneComponent|GetRelativeRotation (Variables|/Game/Blueprints/BP_ShellObject.BP_ShellObject_C|GetAnchor (Variables|Default|GetProgram))) false false)
    (bind _output_2 (CallFunction|GetStartMessage))
    (CallFunction|Print _output_2)
    (else
      (CallFunction|Print _output)
      (Actor|DestroyActor))))

(fn BindEvents
  (bind _asbp_game_manager (Utilities|Casting|CastToBP_GameManager (Game|GetGameMode)))
  (EventDispatchers|BindEventtoOnOutput (EventDispatchers|CreateEvent (Variables|/Game/UI/WBP_HUD.WBP_HUD_C|GetTerminal (Variables|/Game/GameMode/BP_GameManager.BP_GameManager_C|GetHUD _asbp_game_manager)) :!event Print)))

(fn DoneInstalling
  (|CallParentFunction)
  (CallFunction|SendPacket))

(fn SendPacket
  (params (Path :type Array%20of%20Strings) (Values :type Array%20of%20Strings))
  (bind _returnvalue (Game|SpawnActorfromClass "/Game/Blueprints/BP_Packet.BP_Packet_C" (Math|Transform|MakeTransform "0, 0, 0") "Undefined" "MultiplyWithRoot" 0 (Variables|Default|GetPacketSpeed) self (Variables|Default|GetProgram) Path (Variables|Default|GetNavigationProcess) (Variables|Default|GetShell) (Variables|Default|GetreadAccess) Values 0))
  (Variables|Default|SetActivePacket _returnvalue)
  (Variables|Default|SetDoSendPacket false)
  (Class|ActorSequenceComponent|PlaySequence (Variables|Default|GetPulseAnimation)))

(fn SetNextSendTimestamp
  (Variables|Default|SetSendPacketTimestamp (+ (Math|DateTime|Now) (Math|Timespan|FromSeconds (/ 1.0 (Variables|Default|GetPacketRate)))))
  (Variables|Default|SetDoSendPacket true))

(fn OnPacketArrived
  (params (AtShell :type BP%20Shell%20Object%20Reference) (Packet :type BP%20Packet%20Object%20Reference))
  (bind (_output _issuccess) (CallFunction|Parse (Variables|Default|GetParams) AtShell))
  (CallFunction|Print _output)
  (if _issuccess
    (CallFunction|TransitionPackettoTarget Packet)
    (else
      (Actor|DestroyActor Packet)
      (CallFunction|Delete))))

(fn SetupOrbit
  (Variables|Default|SetOrbitRotator (* (Math|Rotator|MakeRotator (Math|Float|SelectFloat 1.0 -1.0 (Math|Random|RandomBool)) (Math|Float|SelectFloat 1.0 -1.0 (Math|Random|RandomBool)) 0.0) (Variables|Default|GetOrbitSpeed))))

(fn Validate
  (params (Params :type Array%20of%20Strings))
  (return false ""))

(fn Parse
  (params (Params :type Array%20of%20Strings) (AtShell :type BP%20Shell%20Object%20Reference))
  (return "" true))

(fn Run
  (params (Params :type Array%20of%20Strings) (AtShell :type BP%20Shell%20Object%20Reference)))

(fn OnPacketLanded
  (params (AtShell :type BP%20Shell%20Object%20Reference) (Packet :type BP%20Packet%20Object%20Reference))
  (bind _landedpackets (Variables|Default|GetLandedPackets))
  (Math|Integer|IncrementInt _landedpackets
    (:%20%20
      (if (>= _landedpackets (Variables|Default|GetPacketCount))
        (CallFunction|Run (Variables|Default|GetParams) AtShell)
        (else
          (CallFunction|SetNextSendTimestamp))))))

(fn TransitionPackettoTarget
  (params (Packet :type BP%20Packet%20Object%20Reference))
  (Default|StartShellObjectTransition Packet (Variables|Default|GetTargetedShellObject) true))

(fn AssigntoShell
  (|CallParentFunction)
  (Default|AddProcess (Variables|Default|GetShell) self (Variables|Default|GetThreads)))

(fn Delete
  (|CallParentFunction)
  (Default|RemoveProcess (Variables|Default|GetShell) self (Variables|Default|GetThreads))
  (bind _activepacket (Variables|Default|GetActivePacket)
    (:then
      (Actor|DestroyActor _activepacket))
    (:else)))

(fn GetInfo
  (params (withReadAccess :type Boolean))
  (Variables|Default|SetreadAccess (or withReadAccess (Variables|Default|GetreadAccess)))
  (return (Utilities|Text|FormatText "{name} ... {pck}/{need} ... {load}" (Utilities|Array|Get(acopy) (Variables|Default|GetAliases)) (Variables|Default|GetLandedPackets) (Variables|Default|GetPacketCount) (Variables|Default|GetLoad))))

(fn ParseParam
  (params (Param :type String))
  (bind _returnvalue (Utilities|String|ParseIntoArray Param "." false))
  (bind _returnvalue_2 (Utilities|Array|Length _returnvalue))
  (bind _returnvalue_3 (- _returnvalue_2 1))
  (bind _output_get (LocalVariables|SetSplitInput _returnvalue))
  (LocalVariables|SetValue (Utilities|Array|Get(acopy) _output_get _returnvalue_3))
  (Utilities|Array|RemoveIndex (LocalVariables|GetSplitInput) _returnvalue_3)
  (return (LocalVariables|GetSplitInput) (LocalVariables|GetValue)))

(fn Print
  (params (Output :type Text))
  (if (not (Utilities|Text|TextIsEmpty Output))
    (Default|CallOnOutput (Utilities|Text|FormatText "[{name}] {out}" (Class|KismetStringLibrary|ToUpper (Utilities|Array|Get(acopy) (Variables|Default|GetAliases))) Output))))

(fn GetStartMessage
  (return "Starting..."))