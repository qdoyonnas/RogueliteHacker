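; Base actor Blueprint for a terminal process, which runs a command from its Params and then removes itself.
; Setup binds events and, unless the process is flagged Temp, chains Validate, Parse and Run, then destroys the actor.
; A failed Validate or Parse prints its output to both popup and terminal.
; Validate here always passes with empty output.
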(event EventBeginPlay
  (|CallParentFunction) ; This node is disabled and will not be called.\nDrag off pins to build functionality.
)

(event Collision|EventActorBeginOverlap
  (params (OtherActor :type Actor%20Object%20Reference)))

(event EventTick
  (params (DeltaSeconds :type Float%20%28single-precision%29))
  (|CallParentFunction DeltaSeconds) ; This node is disabled and will not be called.\nDrag off pins to build functionality.
)

(fn ConstructionScript
  (|CallParentFunction))

(fn Setup
  (CallFunction|BindEvents)
  (if (not (Variables|Default|GetTemp))
    (bind (_isvalid _output) (CallFunction|Validate (Variables|Default|GetParams)))
    (if _isvalid
      (bind (_output_2 _issuccess) (CallFunction|Parse (Variables|Default|GetParams)))
      (if _issuccess
        (CallFunction|Run (Variables|Default|GetParams))
        (else
          (CallFunction|Print _output_2 true true)))
      (else
        (CallFunction|Print _output true true)))
    (Actor|DestroyActor)))

(fn Validate
  (params (Params :type Array%20of%20Strings))
  (return true ""))