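; Hidden process for the Access program that opens a "dive link" on its shell and sends packets to programs on shells.
; Setup registers program and shell with the game manager's Interpreter, reveals the shell and its data objects, and claims fallback camera focus.
; Packets spawn with navigation, seek their named program on arrival, then notify the shell on landing.
; Missing targets and interceptions destroy packets with terminal errors; Delete is a no-op.
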(fn ConstructionScript
  (|CallParentFunction))

(fn Setup
  (CallFunction|SetupInterpreter)
  (CallFunction|SetVisible false)
  (CallFunction|AssigntoShell (Variables|Default|GetShell))
  (CallFunction|BindEvents)
  (bind _output (CallFunction|GetStartMessage))
  (CallFunction|Print _output true true))

(fn GetInfo
  (params (withReadAccess :type Boolean))
  (CallFunction|SetVisible false)
  (return (Utilities|Text|FormatText "<input>[</>{index}<input>]</><process>Access</> <input>.</> {load}" (Variables|Default|GetProcessIndex) (Variables|Default|GetLoad))))

(fn GetStartMessage
  (return "ESTABLISHING DIVE LINK..."))

(fn SetupInterpreter
  (bind _shell (Variables|Default|GetShell))
  (bind _asbp_game_manager (Utilities|Casting|CastToBP_GameManager (Game|GetGameMode)))
  (Variables|Default|SetInterpreter (Variables|/Game/GameMode/BP_GameManager.BP_GameManager_C|GetInterpreter _asbp_game_manager))
  (bind _asprog_access (Utilities|Casting|CastToProg_Access (Variables|Default|GetProgram)))
  (Variables|/Game/Blueprints/BP_Interpreter.BP_Interpreter_C|SetAccessProgram (Variables|Default|GetInterpreter) _asprog_access)
  (Variables|/Game/Blueprints/BP_Interpreter.BP_Interpreter_C|SetAccessShell (Variables|Default|GetInterpreter) (Variables|Default|GetShell))
  (EventDispatchers|BindEventtoOnDelete (Variables|Default|GetProgram) (EventDispatchers|CreateEvent (Variables|Default|GetInterpreter) :!event AccessDeleted))
  (Default|SetVisible _shell true)
  (for _array_element (Variables|/Game/Blueprints/GameObjects/BP_Shell.BP_Shell_C|GetDataObjects _shell)
    (CallFunction|SetVisible _array_element true))
  (Default|RegisterCameraFocus (Variables|Default|GetShell) 0.0 0.0 3.0 false true true))

(fn SetVisible
  (params (NewState :type Boolean))
  (Variables|Default|SetreadAccess NewState)
  (Rendering|SetActorHiddenInGame true))

(fn SendPacket
  (params (Path :type Array%20of%20Strings) (Values :type Map%20of%20Strings%20to%20Strings))
  (bind _packet (CallFunction|SpawnPacket Path Values true))
  (Default|StartShellObjectTransition _packet (Variables|Default|GetProgram) false (Variables|Default|GetPacketSpeed))
  (Default|PlayPulse (Variables|Default|GetProgram))
  (return))

(fn PacketArrived
  (params (AtShell :type BP%20Shell%20Object%20Reference) (Packet :type BP%20Packet%20Object%20Reference))
  (bind _values (Variables|/Game/Blueprints/GameObjects/BP_Packet.BP_Packet_C|GetValues Packet))
  (bind _value (Utilities|Map|Find _values "program"))
  (bind (_program _isfound) (CallFunction|FindProgramonShell AtShell _value))
  (Variables|Default|SetTargetedShellObject _program)
  (if _isfound
    (CallFunction|TransitionPackettoTarget Packet)
    (else
      (CallFunction|Print (Utilities|Text|FormatText "<error>ERROR</>: <program>{p}</> not found on <shell>{s}</>" _value (Variables|/Game/Blueprints/GameObjects/BP_Shell.BP_Shell_C|GetNickname AtShell)) false true)
      (Actor|DestroyActor Packet))))

(fn PacketLanded
  (params (AtShell :type BP%20Shell%20Object%20Reference) (Packet :type BP%20Packet%20Object%20Reference))
  (Default|CallOnPacketLanded self Packet)
  (bind _packet (LocalVariables|GetPacket)
    (:then
      (Default|PacketLanded AtShell _packet))
    (:else)))

(fn PacketIntercepted
  (params (Packet :type BP%20Packet%20Object%20Reference) (InterceptorProcess :type BP%20Process%20Object%20Reference))
  (Actor|DestroyActor Packet)
  (CallFunction|SetVisible InterceptorProcess (or (Variables|/Game/Blueprints/GameObjects/BP_ShellObject.BP_ShellObject_C|GetreadAccess InterceptorProcess) (Variables|Default|GetreadAccess)))
  (Default|CallOnIntercepted self InterceptorProcess)
  (CallFunction|Print (Utilities|Text|FormatText "<error> ACCESS INTERCEPTED</> when trying to reach <program>{p}</>  program" (.Value (Utilities|Map|Find (Variables|/Game/Blueprints/GameObjects/BP_Packet.BP_Packet_C|GetValues Packet) "program"))) false true))

(fn Delete
  (params (SkipAnimation :type Boolean)))