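; BP_Intercept is a subprocess Blueprint that intercepts packets on behalf of its Process.
; InterceptPacket checks for a valid Shell, notifies it of the interception, calls Intercept on the packet with the Process, then starts PlayIntercept.
; PlayIntercept runs a timeline that animates the scale of the Point component and calls OnInterceptFinished when done.
; OnPacketApproach and OnInterceptFinished are empty here, and nothing in this Blueprint calls InterceptPacket.
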(event Custom|PlayIntercept
  (bind _scale (Timeline|InterceptAnimTimeline PlayFromStart)
    (:Update
      (Transformation|SetRelativeScale3D (Variables|Default|GetPoint) _scale))
    (:Finished
      (CallFunction|OnInterceptFinished))))

(fn ConstructionScript
  (|CallParentFunction))

(fn OnPacketApproach
  (params (Packet :type BP%20Packet%20Object%20Reference) (FromShell :type BP%20Shell%20Object%20Reference)))

(fn InterceptPacket
  (params (Packet :type BP%20Packet%20Object%20Reference))
  (bind _shell (Variables|Default|GetShell)
    (:then
      (Default|PacketIntercepted _shell Packet (Variables|Default|GetProcess))
      (Default|Intercept Packet (Variables|Default|GetProcess))
      (CallFunction|PlayIntercept))
    (:else)))

(fn OnInterceptFinished)