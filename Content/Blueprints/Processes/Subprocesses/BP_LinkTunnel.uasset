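; BP_LinkTunnel is an actor that visually links two shells, shown only while ReadAccess is true.
; Each tick it moves to their midpoint, aims Point at Shell2 and stretches it along Z by their distance, less a fixed offset.
; Nested components separate the scaling: Point handles length, Bounce pulses the width through an oscillation, and Scale plays uniform deploy and delete timeline animations.
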(event Custom|PlayDeploy
  (bind _scale (Timeline|DeployTimeline PlayFromStart)
    (:Update
      (Transformation|SetRelativeScale3D (Variables|Default|GetScale) (Math|Vector|MakeVector _scale _scale _scale)))))

(event Custom|PlayDelete
  (bind _scale (Timeline|DeleteTimeline PlayFromStart)
    (:Update
      (Transformation|SetRelativeScale3D (Variables|Default|GetScale) (Math|Vector|MakeVector _scale _scale _scale)))))

(event EventBeginPlay
  (CallFunction|SetVisible (Variables|Default|GetReadAccess)))

(event EventTick
  (params (DeltaSeconds :type Float%20%28single-precision%29))
  (CallFunction|SetPosition)
  (CallFunction|SetRotation)
  (CallFunction|SetScale)
  (CallFunction|Oscillate))

(fn ConstructionScript)

(fn SetPosition
  (Transformation|SetActorLocation (* (+ (Transformation|GetActorLocation (Variables|Default|GetShell1)) (Transformation|GetActorLocation (Variables|Default|GetShell2))) (Math|Float|MakeLiteralFloat 0.5)) false false))

(fn SetRotation
  (bind _shell2 (Variables|Default|GetShell2))
  (bind _point (Variables|Default|GetPoint))
  (bind _returnvalue (Transformation|GetWorldLocation _point))
  (bind _point_2 (Variables|/Game/Blueprints/BP_Shell.BP_Shell_C|GetPoint _shell2))
  (bind _returnvalue_2 (Transformation|GetWorldLocation _point_2))
  (bind _returnvalue_3 (Math|Rotator|FindLookatRotation _returnvalue _returnvalue_2))
  (bind (_roll _pitch _yaw) (Math|Rotator|BreakRotator _returnvalue_3))
  (Transformation|SetWorldRotation (Variables|Default|GetPoint) (Math|Rotator|MakeRotator _roll (- _pitch 9e+01) _yaw) false false))

(fn SetScale
  (Transformation|SetRelativeScale3D (Variables|Default|GetPoint) (Math|Vector|MakeVector 1.0 1.0 (+ (/ (- (Transformation|GetDistanceTo (Variables|Default|GetShell1) (Variables|Default|GetShell2)) 3.5e+02) 1e+02) 1.0))))

(fn Oscillate
  (bind _returnvalue (CallFunction|Oscillate3DVector (Variables|Default|GetOscillationRate) 0.0 (Variables|Default|GetOscillationDistance)))
  (Transformation|SetRelativeScale3D (Variables|Default|GetBounce) (Math|Vector|MakeVector (+ (.Z (Math|Vector|BreakVector _returnvalue)) 1.0) (+ (.Z (Math|Vector|BreakVector _returnvalue)) 1.0) 1.0)))

(fn SetVisible
  (params (NewState :type Boolean))
  (bind _output_get (Variables|Default|SetReadAccess NewState))
  (Rendering|SetActorHiddenInGame (not _output_get)))