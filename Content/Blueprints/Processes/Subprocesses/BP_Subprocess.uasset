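; BP_Subprocess is a child visual actor of a Process that attaches to a Shell and orbits with oscillation.
; Setup sets visibility from read access, snaps to the Shell, copies the Process anchor rotation before randomizing its orbit, then runs install and updates its label.
; It forwards alerts to its Process, narrows music bumping to a fixed index range, and leaves SendPacket as an empty stub.
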(fn ConstructionScript
  (|CallParentFunction))

(fn DoneInstalling
  (Variables|Default|SetInstalled true)
  (Default|CallOnDoneInstalling))

(fn SendPacket
  (params (Path :type Array%20of%20Strings) (Values :type Map%20of%20Strings%20to%20Strings) (NetworkEvent :type BP%20Network%20Event%20Object%20Reference))
  (return))

(fn Setup
  (CallFunction|SetVisible (Variables|Default|GetreadAccess))
  (Transformation|AttachActorToActor (Variables|Default|GetShell) "None" "SnapToTarget" "KeepRelative" "KeepRelative" true)
  (CallFunction|PlayOscillate)
  (CallFunction|SetupOrbit)
  (CallFunction|Install)
  (CallFunction|UpdateTextLabel))

(fn BumptoMusic
  (params (StartIndex :type Integer) (EndIndex :type Integer))
  (|CallParentFunction 0 5))

(fn SetupOrbit
  (Transformation|SetRelativeRotation (Variables|Default|GetAnchor) (Variables|/Script/Engine.SceneComponent|GetRelativeRotation (Variables|/Game/Blueprints/GameObjects/BP_ShellObject.BP_ShellObject_C|GetAnchor (Variables|Default|GetProcess))) false false)
  (Variables|Default|SetDoOrbit true)
  (CallFunction|SetupRandomOrbit))

(fn GenerateAlert
  (params (Packet :type BP%20Packet%20Object%20Reference))
  (CallFunction|GenerateAlert (Variables|Default|GetProcess) Packet))