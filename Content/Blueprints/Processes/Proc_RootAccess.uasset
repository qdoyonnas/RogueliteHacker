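; Root access process Blueprint for a shell-based hacking system, announcing a dive link as it starts.
; Setup snaps and attaches the actor to its Shell, then assigns itself to it.
; It reports a root label with its load while returning no read access, and forwards printed text through an output call.
; Delete is empty, so calling it does nothing.
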(fn ConstructionScript
  (|CallParentFunction))

(fn Setup
  (Transformation|AttachActorToActor (Variables|Default|GetShell) "None" "SnapToTarget" "SnapToTarget" "KeepRelative" true)
  (CallFunction|AssigntoShell))

(fn GetInfo
  (params (withReadAccess :type Boolean))
  (Variables|Default|SetreadAccess false)
  (return (Utilities|Text|FormatText "Root ... {load}" (Variables|Default|GetLoad))))

(fn Print
  (params (Output :type Text))
  (Default|CallOnOutput Output))

(fn GetStartMessage
  (return "ESTABLISHING DIVE LINK..."))

(fn Delete)