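; Blueprint function library that builds the valid-input candidates for intellisense in an in-game shell and program network.
; RunIntellisense optionally gathers reachable shells as path inputs, then selects a collector by function name and merges its name-to-object map into the result.
; Collectors scan the shell's objects, files, programs, links and processes, or network shells, mostly filtering by read access.
; The root shell also exposes root program aliases alongside data objects.
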(fn RunIntellisense
  (params (Program :type BP%20Program%20Object%20Reference) (Shell :type BP%20Shell%20Object%20Reference) (UsePath :type Boolean) (FunctionName :type String))
  (Utilities|FlowControl|Sequence
    (:then_0
      (if UsePath
        (bind _validparameters (CallFunction|ReachableShells Program Shell))
        (bind _result (CallFunction|MergeValidInput (LocalVariables|GetCollectedParams) _validparameters))
        (LocalVariables|SetCollectedParams _result)))
    (:then_1
      (switch string FunctionName
        (:Default
          (return (LocalVariables|GetCollectedParams)))
        (:DataObjects
          (bind _validparameters_2 (CallFunction|DataObjects Program Shell))
          (bind _result_2 (CallFunction|MergeValidInput (LocalVariables|GetCollectedParams) _validparameters_2))
          (return _result_2))
        (:AddressFiles
          (bind _validparameters_3 (CallFunction|AddressFiles Program Shell))
          (bind _result_3 (CallFunction|MergeValidInput (LocalVariables|GetCollectedParams) _validparameters_3))
          (return _result_3))
        (:Programs
          (bind _validparameters_4 (CallFunction|Programs Program Shell))
          (bind _result_4 (CallFunction|MergeValidInput (LocalVariables|GetCollectedParams) _validparameters_4))
          (return _result_4))
        (:Links
          (bind _validparameters_5 (CallFunction|Links Program Shell))
          (bind _result_5 (CallFunction|MergeValidInput (LocalVariables|GetCollectedParams) _validparameters_5))
          (return _result_5))
        (:Processes
          (bind _validparameters_6 (CallFunction|Processes Program Shell))
          (bind _result_6 (CallFunction|MergeValidInput (LocalVariables|GetCollectedParams) _validparameters_6))
          (return _result_6))
        (:AllReadableShells
          (bind _validparameters_7 (CallFunction|AllReadableShells Program Shell))
          (bind _result_7 (CallFunction|MergeValidInput (LocalVariables|GetCollectedParams) _validparameters_7))
          (return _result_7))
        (:ReachableShells
          (if (not UsePath)
            (bind _validparameters_8 (CallFunction|ReachableShells Program Shell))
            (bind _result_8 (CallFunction|MergeValidInput (LocalVariables|GetCollectedParams) _validparameters_8))
            (return _result_8)))
        (:DataAndRootObjects
          (bind _validparameters_9 (CallFunction|DataandRootObjects Program Shell))
          (bind _result_9 (CallFunction|MergeValidInput (LocalVariables|GetCollectedParams) _validparameters_9))
          (return _result_9))))))

(fn DataObjects
  (params (Program :type BP%20Program%20Object%20Reference) (Shell :type BP%20Shell%20Object%20Reference))
  (for _array_element (Variables|/Game/Blueprints/GameObjects/BP_Shell.BP_Shell_C|GetDataObjects Shell)
    (if (and (Variables|/Game/Blueprints/GameObjects/BP_ShellObject.BP_ShellObject_C|GetreadAccess _array_element) (!= _array_element Program))
      (Utilities|Map|Add (LocalVariables|GetObjectNames) (Variables|/Game/Blueprints/GameObjects/BP_DataObject.BP_DataObject_C|GetFileName _array_element) _array_element)))
  (return (Utilities|Struct|MakeStruct_ValidInput (LocalVariables|GetObjectNames))))

(fn AddressFiles
  (params (Program :type BP%20Program%20Object%20Reference) (Shell :type BP%20Shell%20Object%20Reference))
  (bind _keys (Utilities|Map|Keys (Variables|/Game/Blueprints/GameObjects/BP_Shell.BP_Shell_C|GetLocalFiles Shell)))
  (for _array_element _keys
    (bind _output_get (LocalVariables|SetFileName _array_element))
    (if (Variables|/Game/Blueprints/GameObjects/BP_ShellObject.BP_ShellObject_C|GetreadAccess (.Value (Utilities|Map|Find (Variables|/Game/Blueprints/GameObjects/BP_Shell.BP_Shell_C|GetLocalFiles Shell) _output_get)))
      (bind _asfile_address (Utilities|Casting|CastToFile_Address (.Value (Utilities|Map|Find (Variables|/Game/Blueprints/GameObjects/BP_Shell.BP_Shell_C|GetLocalFiles Shell) _output_get))))
      (Utilities|Map|Add (LocalVariables|GetObjectNames) (LocalVariables|GetFileName) _asfile_address)))
  (return (Utilities|Struct|MakeStruct_ValidInput (LocalVariables|GetObjectNames))))

(fn Programs
  (params (Program :type BP%20Program%20Object%20Reference) (Shell :type BP%20Shell%20Object%20Reference))
  (bind _keys (Utilities|Map|Keys (Variables|/Game/Blueprints/GameObjects/BP_Shell.BP_Shell_C|GetLocalPrograms Shell)))
  (for _array_element _keys
    (bind _output_get (LocalVariables|SetAlias _array_element))
    (if (Variables|/Game/Blueprints/GameObjects/BP_ShellObject.BP_ShellObject_C|GetreadAccess (.Value (Utilities|Map|Find (Variables|/Game/Blueprints/GameObjects/BP_Shell.BP_Shell_C|GetLocalPrograms Shell) _output_get)))
      (Utilities|Map|Add (LocalVariables|GetCollectedPrograms) (LocalVariables|GetAlias) (.Value (Utilities|Map|Find (Variables|/Game/Blueprints/GameObjects/BP_Shell.BP_Shell_C|GetLocalPrograms Shell) _output_get)))))
  (return (Utilities|Struct|MakeStruct_ValidInput (LocalVariables|GetCollectedPrograms))))

(fn Links
  (params (Program :type BP%20Program%20Object%20Reference) (Shell :type BP%20Shell%20Object%20Reference))
  (bind _keys (Utilities|Map|Keys (Variables|/Game/Blueprints/GameObjects/BP_Shell.BP_Shell_C|GetLocalLinks Shell)))
  (for _array_element _keys
    (bind _output_get (LocalVariables|SetName _array_element))
    (if (Variables|/Game/Blueprints/GameObjects/BP_ShellObject.BP_ShellObject_C|GetreadAccess (.Value (Utilities|Map|Find (Variables|/Game/Blueprints/GameObjects/BP_Shell.BP_Shell_C|GetLocalLinks Shell) _output_get)))
      (Utilities|Map|Add (LocalVariables|GetCollectedLinks) (LocalVariables|GetName) (.Value (Utilities|Map|Find (Variables|/Game/Blueprints/GameObjects/BP_Shell.BP_Shell_C|GetLocalLinks Shell) _output_get)))))
  (return (Utilities|Struct|MakeStruct_ValidInput (LocalVariables|GetCollectedLinks))))

(fn Processes
  (params (Program :type BP%20Program%20Object%20Reference) (Shell :type BP%20Shell%20Object%20Reference))
  (bind _keys (Utilities|Map|Keys (Variables|/Game/Blueprints/GameObjects/BP_Shell.BP_Shell_C|GetLocalProcesses Shell)))
  (for _array_element _keys
    (bind _output_get (LocalVariables|SetAlias _array_element))
    (Utilities|IsValid (.Value (Utilities|Map|Find (Variables|/Game/Blueprints/GameObjects/BP_Shell.BP_Shell_C|GetLocalProcesses Shell) _output_get))
      (:Is%20Valid
        (if (Variables|/Game/Blueprints/GameObjects/BP_ShellObject.BP_ShellObject_C|GetreadAccess (.Value (Utilities|Map|Find (Variables|/Game/Blueprints/GameObjects/BP_Shell.BP_Shell_C|GetLocalProcesses Shell) _output_get)))
          (Utilities|Map|Add (LocalVariables|GetCollectedProcesses) (LocalVariables|GetAlias) (.Value (Utilities|Map|Find (Variables|/Game/Blueprints/GameObjects/BP_Shell.BP_Shell_C|GetLocalProcesses Shell) _output_get)))))))
  (return (Utilities|Struct|MakeStruct_ValidInput (LocalVariables|GetCollectedProcesses))))

(fn AllReadableShells
  (params (Program :type BP%20Program%20Object%20Reference) (Shell :type BP%20Shell%20Object%20Reference))
  (bind _asbp_game_manager (Utilities|Casting|CastToBP_GameManager (Game|GetGameMode)))
  (bind _output_get (LocalVariables|SetNetworkShells (Variables|/Game/GameMode/NetworkBuilder/BP_NetworkBuilder.BP_NetworkBuilder_C|GetNetworkShells (Variables|/Game/GameMode/BP_GameManager.BP_GameManager_C|GetNetworkBuilder _asbp_game_manager))))
  (bind _keys (Utilities|Map|Keys _output_get))
  (for _array_element _keys
    (LocalVariables|SetName _array_element)
    (if (Variables|/Game/Blueprints/GameObjects/BP_Shell.BP_Shell_C|GetReadAccess (.Value (Utilities|Map|Find (LocalVariables|GetNetworkShells) _array_element)))
      (Utilities|Map|Add (LocalVariables|GetCollectedShells) (LocalVariables|GetName) (.Value (Utilities|Map|Find (LocalVariables|GetNetworkShells) _array_element)))))
  (return (Utilities|Struct|MakeStruct_ValidInput (LocalVariables|GetCollectedShells))))

(fn ReachableShells
  (params (Program :type BP%20Program%20Object%20Reference) (Shell :type BP%20Shell%20Object%20Reference))
  (bind _shells (Default|CollectReachableShells Shell (Utilities|Map|MakeMap) (not (Variables|/Game/Blueprints/GameObjects/BP_Shell.BP_Shell_C|GetReachableFlag Shell)) true))
  (bind _output_get (LocalVariables|SetReachableShells _shells))
  (bind _keys (Utilities|Map|Keys _output_get))
  (for _array_element _keys
    (LocalVariables|SetTempName _array_element)
    (if (Utilities|Enum|NotEqual(Enum) (LocalVariables|GetTempName) (Variables|/Game/Blueprints/GameObjects/BP_Shell.BP_Shell_C|GetName Shell))
      (Utilities|Map|Add (LocalVariables|GetCollectedShells) (LocalVariables|GetTempName) (.Value (Utilities|Map|Find (LocalVariables|GetReachableShells) (LocalVariables|GetTempName))))))
  (return (Utilities|Struct|MakeStruct_ValidInput (LocalVariables|GetCollectedShells))))

(fn DataandRootObjects
  (params (Program :type BP%20Program%20Object%20Reference) (Shell :type BP%20Shell%20Object%20Reference))
  (bind _validparameters (CallFunction|DataObjects Program Shell))
  (LocalVariables|SetCollectedObjects (Utilities|Struct|BreakStruct_ValidInput _validparameters))
  (bind _asbp_game_manager (Utilities|Casting|CastToBP_GameManager (Game|GetGameMode)))
  (if (== Shell (Variables|/Game/Blueprints/BP_Interpreter.BP_Interpreter_C|GetRootShell (Variables|/Game/GameMode/BP_GameManager.BP_GameManager_C|GetInterpreter _asbp_game_manager)))
    (for _array_element (Variables|/Game/Blueprints/GameObjects/BP_Program.BP_Program_C|GetAliases (Variables|/Game/Blueprints/BP_Interpreter.BP_Interpreter_C|GetRootProgram (Variables|/Game/GameMode/BP_GameManager.BP_GameManager_C|GetInterpreter _asbp_game_manager)))
      (Utilities|Map|Add (LocalVariables|GetCollectedObjects) _array_element (Variables|/Game/Blueprints/BP_Interpreter.BP_Interpreter_C|GetRootProgram (Variables|/Game/GameMode/BP_GameManager.BP_GameManager_C|GetInterpreter _asbp_game_manager))))
    (return (Utilities|Struct|MakeStruct_ValidInput (LocalVariables|GetCollectedObjects)))))

(fn MergeValidInput
  (params (ValidInputA :type Struct%20Valid%20Input%20Structure) (ValidInputB :type Struct%20Valid%20Input%20Structure))
  (bind _keys (Utilities|Map|Keys (Utilities|Struct|BreakStruct_ValidInput ValidInputB)))
  (for _array_element _keys
    (Utilities|Map|Add (Utilities|Struct|BreakStruct_ValidInput ValidInputA) _array_element (.Value (Utilities|Map|Find (Utilities|Struct|BreakStruct_ValidInput ValidInputB) _array_element))))
  (return ValidInputA))