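; BP_ShellObject is an actor that attaches to a Shell, animates around it, and is visible only while both have read access.
; Setup randomizes a bobbing offset and an Anchor orbit, binds sequence-finished events, then plays the install sequence.
; Tick updates visibility, oscillates the Bounce component and rotates Anchor by a fixed per-frame step.
; Delete stops both motions and plays a delete sequence, with completion handlers for re-attaching and destroying the actor.
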(event EventBeginPlay
  (CallFunction|Setup))

(event EventTick
  (params (DeltaSeconds :type Float%20%28single-precision%29))
  (CallFunction|DoTick))

(fn ConstructionScript)

(fn Oscillate
  (bind _returnvalue (CallFunction|Oscillate3DVector 2.0 (Variables|Default|GetOscillationOffset) 1e+01))
  (Transformation|SetRelativeLocation (Variables|Default|GetBounce) _returnvalue false false))

(fn SetupOscillation
  (Variables|Default|SetOscillationOffset (Math|Random|RandomFloatinRange -1e+01 1e+01)))

(fn Orbit
  (Transformation|AddLocalRotation (Variables|Default|GetAnchor) (Variables|Default|GetOrbitRotator) false false))

(fn SetupOrbit
  (Transformation|SetRelativeRotation (Variables|Default|GetAnchor) (Math|Random|RandomRotator true) false false)
  (Variables|Default|SetOrbitRotator (* (Math|Rotator|MakeRotator (Math|Float|SelectFloat 1.0 -1.0 (Math|Random|RandomBool)) (Math|Float|SelectFloat 1.0 -1.0 (Math|Random|RandomBool)) 0.0) (Variables|Default|GetOrbitSpeed))))

(fn Setup
  (Transformation|AttachActorToActor (Variables|Default|GetShell) "None" "SnapToTarget" "SnapToTarget" "KeepRelative" true)
  (CallFunction|SetupOscillation)
  (CallFunction|SetupOrbit)
  (CallFunction|BindSequenceEvents)
  (CallFunction|Install))

(fn DoTick
  (Rendering|SetActorHiddenInGame (not (and (Variables|Default|GetreadAccess) (Variables|/Game/Blueprints/BP_Shell.BP_Shell_C|GetReadAccess (Variables|Default|GetShell)))))
  (if (Variables|Default|GetDoOscillation)
    (CallFunction|Oscillate))
  (if (Variables|Default|GetDoOrbit)
    (CallFunction|Orbit)))

(fn Install
  (Class|ActorSequenceComponent|PlaySequence (Variables|Default|GetInstallAnimation)))

(fn Delete
  (Variables|Default|SetDoOrbit false)
  (Variables|Default|SetDoOscillation false)
  (Class|ActorSequenceComponent|PlaySequence (Variables|Default|GetDeleteAnimation)))

(fn AssigntoShell
  (Transformation|AttachActorToActor (Variables|Default|GetShell) "None" "SnapToTarget" "KeepRelative" "KeepRelative" true))

(fn DoneDeleting
  (Actor|DestroyActor))

(fn DoneInstalling
  (CallFunction|AssigntoShell))

(fn BindSequenceEvents
  (EventDispatchers|BindEventtoOnFinished (Variables|/Script/ActorSequence.ActorSequenceComponent|GetSequencePlayer (Variables|Default|GetInstallAnimation)) (EventDispatchers|CreateEvent :!event DoneInstalling))
  (EventDispatchers|BindEventtoOnFinished (Variables|/Script/ActorSequence.ActorSequenceComponent|GetSequencePlayer (Variables|Default|GetDeleteAnimation)) (EventDispatchers|CreateEvent :!event DoneDeleting)))