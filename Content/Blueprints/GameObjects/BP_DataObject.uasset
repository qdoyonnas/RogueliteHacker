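; Data file object that lives inside a Shell, with a name, size, tags and read access.
; Setup destroys it if the Shell lacks room; reassignment and deletion update the Shell's object list.
; It builds rich-text info for Interpreter popups and can spawn duplicates.
; As a camera focus, it swings its anchor by timelines toward a secondary focus, skipping this for same-Shell objects, and resumes random orbit when cleared.
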(event Custom|PlayRotateCameraAnchor
  (bind _rotation (Timeline|RotateAnchorTimeline Play)
    (:Update
      (Transformation|SetRelativeRotation (Variables|Default|GetShellObjectCameraAnchor) (Math|Vector|RotatorfromAxisandAngle "0.000000,1.000000,0.000000" _rotation) false false))))

(event Custom|ReverseCameraAnchor
  (bind _rotation (Timeline|RotateAnchorTimeline Reverse)
    (:Update
      (Transformation|SetRelativeRotation (Variables|Default|GetShellObjectCameraAnchor) (Math|Vector|RotatorfromAxisandAngle "0.000000,1.000000,0.000000" _rotation) false false))))

(event Custom|PlayPointAtFocus
  (bind _lerp (Timeline|PointAtFocusTimeline PlayFromStart)
    (:Update
      (CallFunction|Orbit _lerp))))

(fn ConstructionScript
  (Helper|CalculateSize))

(fn CalculateSize
  (bind _ratio (Utilities|SizeRatio))
  (bind _returnvalue (* _ratio 2.0))
  (Transformation|SetRelativeScale3D (Variables|Default|GetScale) (Math|Vector|MakeVector _returnvalue _returnvalue 0.2)))

(fn Delete
  (params (SkipAnimation :type Boolean))
  (Default|RemoveDataObject (Variables|Default|GetShell) self)
  (|CallParentFunction false))

(fn AssigntoShell
  (params (NewShell :type BP%20Shell%20Object%20Reference))
  (Utilities|FlowControl|Sequence
    (:then_0
      (bind _shell (Variables|Default|GetShell)
        (:then
          (Default|RemoveDataObject _shell self))
        (:else)))
    (:then_1
      (|CallParentFunction NewShell)
      (Helper|CalculateSize)
      (bind _shell_2 (Variables|Default|GetShell)
        (:then
          (Default|AddDataObject _shell_2 self))
        (:else)))))

(fn Setup
  (bind _asbp_game_manager (Utilities|Casting|CastToBP_GameManager (Game|GetGameMode)))
  (Variables|Reference|SetInterpreter (Variables|/Game/GameMode/BP_GameManager.BP_GameManager_C|GetInterpreter _asbp_game_manager))
  (bind _canadd (Default|CanAddDataObject (Variables|Default|GetShell) (Variables|ShellInterface|GetSize)))
  (if _canadd
    (|CallParentFunction)
    (Animation|UpdateTextLabel)
    (else
      (Actor|DestroyActor))))

(fn GetInfo
  (params (withReadAccess :type Boolean))
  (CallFunction|SetVisible (or withReadAccess (Variables|Default|GetreadAccess)))
  (bind _tags (Info|GetTagInfo))
  (bind _name (Info|GetDisplayName))
  (return (Utilities|Text|FormatText "{name} <input>.</> {tags} <input>.</> {size}" _name _tags (Variables|ShellInterface|GetSize))))

(fn Duplicate
  (params (Input :type Array%20of%20Strings))
  (bind _returnvalue (Game|SpawnActorfromClass (Utilities|GetClass self) (Math|Transform|MakeTransform "0, 0, 0") "Undefined" "MultiplyWithRoot" 0 (Variables|ShellInterface|GetSize) (Variables|ShellInterface|GetFileName) (Variables|ShellInterface|GetDataTags) (Variables|Default|GetShell) (Variables|Default|GetreadAccess) false 0))
  (return _returnvalue))

(fn UpdateTextLabel
  (Rendering|Components|TextRender|SetText (Variables|Default|GetNameText) (Utilities|Text|FormatText "{name}:rw" (Variables|ShellInterface|GetFileName))))

(fn GetRotatortoSecondaryFocus
  (bind _secondaryfocus (Variables|Default|GetSecondaryFocus)
    (:then
      (bind _anchor (Default|GetAnchorasSecondaryFocus _secondaryfocus))
      (bind _rotation (CallFunction|Pointat (Variables|Default|GetAnchor) _anchor))
      (return (Math|Rotator|MakeRotator (.Roll (Math|Rotator|BreakRotator _rotation)) (+ (.Pitch (Math|Rotator|BreakRotator _rotation)) 7e+01) (.Yaw (Math|Rotator|BreakRotator _rotation)))))
    (:else)))

(fn SetSecondaryFocus
  (params (CameraFocus :type BP%20Camera%20Focus%20Object%20Reference) (Input :type Array%20of%20Strings))
  (bind _output_get (LocalVariables|SetSubInput Input))
  (Utilities|Array|RemoveIndex _output_get)
  (bind _valid (|CallParentFunction CameraFocus Input))
  (if (and _valid (!= CameraFocus 0))
    (Default|DisplaySecondaryInfoPopup (Variables|Reference|GetInterpreter) CameraFocus (LocalVariables|GetSubInput))
    (bind _asbp_shell_object (Utilities|Casting|CastToBP_ShellObject CameraFocus)
      (:then
        (if (== (Variables|/Game/Blueprints/GameObjects/BP_ShellObject.BP_ShellObject_C|GetShell _asbp_shell_object) (Variables|Default|GetShell))
          (Variables|Runtime|SetDoNotClear true)
          (Default|RegisterCameraFocus CameraFocus 1e+02 0.0 1.0 true false false)
          (return true)
          (else
            _)))
      (:CastFailed
        _))
    (Animation|StartSecondaryFocusAnimation)
    (return true)
    (else
      (bind _secondaryfocus (Variables|Default|GetSecondaryFocus)
        (:then
          (Default|DisplaySecondaryInfoPopup (Variables|Reference|GetInterpreter) _secondaryfocus (LocalVariables|GetSubInput))
          (return true))
        (:else
          (return false))))))

(fn ClearSecondaryFocus
  (bind _secondaryfocus (Variables|Default|GetSecondaryFocus))
  (Variables|Runtime|SetDoNotClear false)
  (Utilities|FlowControl|Sequence
    (:then_0
      (if (and (Utilities|IsValid _secondaryfocus) (!= _secondaryfocus self))
        (Default|UnregisterCameraFocus (Variables|Default|GetSecondaryFocus) false)))
    (:then_1
      (bind _secondaryinfopopup (Variables|/Game/Blueprints/BP_Interpreter.BP_Interpreter_C|GetSecondaryInfoPopup (Variables|Reference|GetInterpreter))
        (:then
          (Default|ClosePopup _secondaryinfopopup))
        (:else)))
    (:then_2
      (|CallParentFunction)
      (if (not (Variables|Default|GetDoOrbit))
        (Variables|Default|SetDoOrbit true)
        (CallFunction|ReverseCameraAnchor)
        (CallFunction|SetupRandomOrbit)))))

(fn GetPopupInfo
  (params (Parameters :type Array%20of%20Strings))
  (|CallParentFunction Parameters)
  (bind _info (Info|GetDataInfo))
  (return _info))

(fn GetTagInfo
  (LocalVariables|SetTagOutput (Utilities|Array|Get(acopy) (Variables|ShellInterface|GetDataTags)))
  (for (_array_element _array_index) (Variables|ShellInterface|GetDataTags)
    (if (!= _array_index 0)
      (LocalVariables|SetTagOutput (Utilities|String|Append (LocalVariables|GetTagOutput) "<input>,</> " _array_element))))
  (return (LocalVariables|GetTagOutput)))

(fn GetDisplayName
  (return (Utilities|String|ToString(Text) (Utilities|Text|FormatText "<file>{name}</>" (Variables|ShellInterface|GetFileName)))))

(fn GetDataInfo
  (bind _name (Info|GetDisplayName))
  (bind _tags (Info|GetTagInfo))
  (return (Utilities|Text|FormatText "<input>Name:</> {name}    <input>Size:</> {size} 
<input>Types:</> {tags}" _name (Variables|ShellInterface|GetSize) _tags)))

(fn StartSecondaryFocusAnimation
  (CallFunction|PlayRotateCameraAnchor)
  (CallFunction|StopOrbit)
  (bind _rotator (Helper|GetRotatortoSecondaryFocus))
  (Variables|Default|SetOrbitRotator _rotator)
  (Variables|Default|SetOrbitStart (Transformation|GetWorldRotation (Variables|Default|GetAnchor)))
  (CallFunction|PlayPointatFocus))

(fn LostCameraFocus
  (params (ToFocus :type BP%20Camera%20Focus%20Object%20Reference))
  (CallFunction|StopAnchorOrbit)
  (if (not (Variables|Runtime|GetDoNotClear))
    (CallFunction|ClearSecondaryFocus)))