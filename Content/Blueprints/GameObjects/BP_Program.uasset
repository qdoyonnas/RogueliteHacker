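; Program file object that lives in a shell and spawns process actors of its ProcessType, passing on level, stats and parameters.
; Setup merges tags with process class defaults and can roll stats through a temporary process actor; duplicates reroll theirs.
; It formats name, level, tag and size text, and runs intellisense from the process's parameter definitions.
; Timelines animate process start and swing the camera anchor and orbit toward a secondary focus.
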(event Custom|PlayStart
  (bind _rotation (Timeline|StartTimeline PlayFromStart)
    (:Update
      (Transformation|SetRelativeRotation (Variables|Default|GetScale) (Math|Rotator|MakeRotator 0.0 0.0 _rotation) false false))))

(event Custom|PlayRotateCameraAnchor
  (bind _rotation (Timeline|AnchorRotateTimeline Play)
    (:Update
      (Transformation|SetRelativeRotation (Variables|Default|GetShellObjectCameraAnchor) (Math|Vector|RotatorfromAxisandAngle "0.000000,1.000000,0.000000" _rotation) false false))))

(event Custom|ReverseCameraAnchor
  (bind _rotation (Timeline|AnchorRotateTimeline Reverse)
    (:Update
      (Transformation|SetRelativeRotation (Variables|Default|GetShellObjectCameraAnchor) (Math|Vector|RotatorfromAxisandAngle "0.000000,1.000000,0.000000" _rotation) false false))))

(event Custom|PlayPointAtFocus
  (Variables|Default|SetDoOrbit true)
  (bind _lerp (Timeline|PointAtFocusTimeline PlayFromStart)
    (:Update
      (CallFunction|Orbit _lerp))))

(fn ConstructionScript
  (|CallParentFunction))

(fn SetupProgram
  (params (Tags :type Array%20of%20Strings) (Properties :type Map%20of%20Strings%20to%20Strings) (RandomizeStats :type Boolean))
  (bind _processtype (Variables|Default|GetProcessType))
  (bind (_aliases _datatags) (Utilities|GetClassDefaults _processtype))
  (for _array_element Tags
    (Utilities|Array|AddUnique (Variables|Default|GetDataTags) _array_element))
  (Variables|Default|SetAliases _aliases)
  (for _array_element_2 _datatags
    (Utilities|Array|AddUnique (Variables|Default|GetDataTags) _array_element_2))
  (if RandomizeStats
    (CallFunction|RandomizeStats (Variables|Default|GetLevel))))

(fn StartProcess
  (params (Params :type Array%20of%20Strings) (IsPlayerOwned :type Boolean) (AtShell :type BP%20Shell%20Object%20Reference) (FastForward :type Boolean))
  (LocalVariables|SetProcessParams Params)
  (LocalVariables|SetTargetShell (select (Utilities|IsValid AtShell) AtShell (Variables|Default|GetShell)))
  (Utilities|Array|RemoveIndex (LocalVariables|GetProcessParams))
  (bind _returnvalue (Game|SpawnActorfromClass (Variables|Default|GetProcessType) (Math|Transform|MakeTransform "0, 0, 0") "Undefined" "MultiplyWithRoot" 0 self (LocalVariables|GetProcessParams) IsPlayerOwned FastForward (Variables|Default|GetProcessStats) (Variables|Default|GetLevel) false (LocalVariables|GetTargetShell) (Variables|Default|GetreadAccess) FastForward 0))
  (bind _output_get (LocalVariables|SetnewProcess _returnvalue))
  (Default|CallOnStartProcess _output_get)
  (CallFunction|PlayStart)
  (return (LocalVariables|GetnewProcess)))

(fn Duplicate
  (bind _returnvalue (Game|SpawnActorfromClass (Utilities|GetClass self) (Math|Transform|MakeTransform "0, 0, 0") "Undefined" "MultiplyWithRoot" 0 (Variables|Default|GetProcessType) 0.0 (Variables|Default|GetSize) (Variables|Default|GetFileName) (Variables|Default|GetDataTags) (Variables|Default|GetShell) (Variables|Default|GetreadAccess) false 0))
  (CallFunction|SetupProgram _returnvalue 0 (Utilities|Map|MakeMap "" "") true)
  (return _returnvalue))

(fn CanAddProcess
  (params (AtShell :type BP%20Shell%20Object%20Reference) (Params :type Array%20of%20Strings))
  (bind (_canadd _isthreads) (Default|CanAddProcess AtShell))
  (return _canadd _isthreads))

(fn RandomizeStats
  (params (InLevel :type Float%20%28double-precision%29))
  (Variables|Default|SetLevel InLevel)
  (bind _returnvalue (Game|SpawnActorfromClass (Variables|Default|GetProcessType) (Math|Transform|MakeTransform "0, 0, 0") "Undefined" "MultiplyWithRoot" 0 self 0 false false (Utilities|Map|MakeMap) 0.0 true (Variables|Default|GetShell) false false 0))
  (bind _output_get (LocalVariables|SetTempProcess _returnvalue))
  (bind _stats (Default|RandomizeStats _output_get (Variables|Default|GetLevel)))
  (Variables|Default|SetProcessStats _stats)
  (Actor|DestroyActor (LocalVariables|GetTempProcess)))

(fn GetInfo
  (params (withReadAccess :type Boolean))
  (CallFunction|SetVisible (or withReadAccess (Variables|Default|GetreadAccess)))
  (LocalVariables|SetTagOutput (Utilities|Array|Get(acopy) (Variables|Default|GetDataTags)))
  (for (_array_element _array_index) (Variables|Default|GetDataTags)
    (if (!= _array_index 0)
      (LocalVariables|SetTagOutput (Utilities|String|Append (LocalVariables|GetTagOutput) ", " _array_element))))
  (return (Utilities|Text|FormatText "{name}v{v} . {tags} . {size} " (Variables|Default|GetFileName) (Variables|Default|GetLevel) (LocalVariables|GetTagOutput) (Variables|Default|GetSize))))

(fn CollectValidParameters
  (params (AtShell :type BP%20Shell%20Object%20Reference) (Input :type Array%20of%20Strings))
  (bind _output_get (LocalVariables|SetParamIndex (Utilities|Array|LastIndex Input)))
  (bind _output_get_2 (LocalVariables|SetParameters (.Parameters (Utilities|GetClassDefaults (Variables|Default|GetProcessType)))))
  (bind _validparameters (CallFunction|CollectfromParam (- _output_get 1) _output_get_2 AtShell))
  (return _validparameters))

(fn CollectfromParam
  (params (ParamIndex :type Integer) (ParamMap :type Map%20of%20Strings%20to%20Structs) (AtShell :type BP%20Shell%20Object%20Reference))
  (if (Math|Integer|InRange(Integer) ParamIndex 0 (Utilities|Map|Length ParamMap) true false)
    (bind _keys (Utilities|Map|Keys ParamMap))
    (bind _validparameters (CallFunction|RunIntellisense self AtShell (.UsesPath (Utilities|Struct|BreakStruct_Parameter (.Value (Utilities|Map|Find ParamMap (Utilities|Array|Get(acopy) _keys ParamIndex))))) (.IntellisenseFunction (Utilities|Struct|BreakStruct_Parameter (.Value (Utilities|Map|Find ParamMap (Utilities|Array|Get(acopy) _keys ParamIndex)))))))
    (return _validparameters)
    (else
      (return ""))))

(fn SetSecondaryFocus
  (params (CameraFocus :type BP%20Camera%20Focus%20Object%20Reference))
  (|CallParentFunction CameraFocus)
  (if (!= CameraFocus 0)
    (bind _asbp_shell_object (Utilities|Casting|CastToBP_ShellObject CameraFocus)
      (:then
        (if (== (Variables|/Game/Blueprints/GameObjects/BP_ShellObject.BP_ShellObject_C|GetShell _asbp_shell_object) (Variables|Default|GetShell))
          (return false)
          (else
            _)))
      (:CastFailed
        _))
    (CallFunction|PlayRotateCameraAnchor)
    (CallFunction|StopOrbit)
    (bind _rotator (CallFunction|GetRotatortoSecondaryFocus))
    (Variables|Default|SetOrbitRotator _rotator)
    (Variables|Default|SetOrbitStart (Transformation|GetWorldRotation (Variables|Default|GetAnchor)))
    (CallFunction|PlayPointatFocus)
    (return true)))

(fn ClearSecondaryFocus
  (|CallParentFunction)
  (CallFunction|ReverseCameraAnchor)
  (Variables|Default|SetDoOrbit true)
  (CallFunction|SetupRandomOrbit))

(fn UpdateTextLabel
  (Rendering|Components|TextRender|SetText (Variables|Default|GetNameText) (Utilities|Text|FormatText ".{name}v{level}" (Variables|Default|GetFileName) (Variables|Default|GetLevel))))

(fn GetRotatortoSecondaryFocus
  (bind _secondaryfocus (Variables|Default|GetSecondaryFocus)
    (:then
      (bind _rotation (CallFunction|Pointat (Variables|Default|GetAnchor) (Variables|/Game/Blueprints/BP_CameraFocus.BP_CameraFocus_C|GetDefaultSceneRoot _secondaryfocus)))
      (return (Math|Rotator|MakeRotator (.Roll (Math|Rotator|BreakRotator _rotation)) (+ (.Pitch (Math|Rotator|BreakRotator _rotation)) 7e+01) (.Yaw (Math|Rotator|BreakRotator _rotation)))))
    (:else)))