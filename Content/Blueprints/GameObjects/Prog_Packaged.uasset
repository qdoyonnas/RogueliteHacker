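; A packaged program: a single shell data object that bundles several programs, spawned from its process types if none are supplied.
; Setup hides the contained programs, merges their tags and aliases, and sums their sizes.
; Process, parameter and stat calls route to the matching program through an alias map, while duplication copies either the whole package or one program.
; Deleting removes the contents too, unless unpacking, which returns them to the shell.
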(fn ConstructionScript
  (|CallParentFunction))

(fn SetAliases
  (params (InProgram :type BP%20Program%20Object%20Reference))
  (bind _output_get (LocalVariables|SetProgram InProgram))
  (for _array_element (Variables|/Game/Blueprints/GameObjects/BP_Program.BP_Program_C|GetAliases _output_get)
    (bind _output_get_2 (LocalVariables|SetAlias _array_element))
    (Utilities|Map|Add (Variables|Default|GetMappedAliases) _output_get_2 (LocalVariables|GetProgram))
    (Utilities|Array|AddUnique (Variables|Default|GetAliases) (LocalVariables|GetAlias))))

(fn HidePrograms
  (for _array_element (Variables|Default|GetPrograms)
    (bind _output_get (LocalVariables|SetProgram _array_element))
    (Default|RemoveDataObject (Variables|Default|GetShell) _output_get)
    (Variables|/Game/Blueprints/GameObjects/BP_ShellObject.BP_ShellObject_C|SetShell (LocalVariables|GetProgram) (Variables|Default|GetShell))
    (Default|SetVisible (LocalVariables|GetProgram) false)
    (Variables|/Game/Blueprints/GameObjects/BP_ShellObject.BP_ShellObject_C|SetDoOrbit (LocalVariables|GetProgram) false)
    (Variables|/Game/Blueprints/GameObjects/BP_ShellObject.BP_ShellObject_C|SetDoOscillation (LocalVariables|GetProgram) false)))

(fn CalculateSize
  (Variables|Default|SetSize 0)
  (for _array_element (Variables|Default|GetPrograms)
    (Variables|Default|SetSize (+ (Variables|Default|GetSize) (Variables|/Game/Blueprints/GameObjects/BP_DataObject.BP_DataObject_C|GetSize _array_element))))
  (|CallParentFunction))

(fn Delete
  (params (SkipAnimation :type Boolean))
  (if (Variables|Default|GetUnpacking)
    (Helper|ShowPrograms)
    (|CallParentFunction SkipAnimation)
    (else
      (for _array_element (Variables|Default|GetPrograms)
        (CallFunction|Delete _array_element true))
      (|CallParentFunction SkipAnimation))))

(fn ShowPrograms
  (for _array_element (Variables|Default|GetPrograms)
    (bind _output_get (LocalVariables|SetProgram _array_element))
    (Default|AddDataObject (Variables|Default|GetShell) _output_get)
    (Default|SetVisible (LocalVariables|GetProgram) (Variables|Default|GetreadAccess))
    (Default|SetupOrbit (LocalVariables|GetProgram))
    (Variables|/Game/Blueprints/GameObjects/BP_ShellObject.BP_ShellObject_C|SetDoOscillation (LocalVariables|GetProgram) true)
    (Default|PlayOscillate (LocalVariables|GetProgram))))

(fn Unpack
  (Variables|Default|SetUnpacking true)
  (CallFunction|Delete false))

(fn StartProcess
  (params (Params :type Array%20of%20Strings) (IsPlayerOwned :type Boolean) (AtShell :type BP%20Shell%20Object%20Reference) (FastForward :type Boolean))
  (bind (_isfound _program) (CallFunction|GetProgram Params))
  (if _isfound
    (bind _process (CallFunction|StartProcess _program Params IsPlayerOwned AtShell FastForward))
    (Utilities|IsValid _process
      (:Is%20Valid
        (bind _output_get (LocalVariables|SetNewProcess _process))
        (Default|SetVisible _output_get (Variables|Default|GetreadAccess))
        (Default|CallOnStartProcess (LocalVariables|GetNewProcess))
        (CallFunction|PlayStart)
        (return (LocalVariables|GetNewProcess)))
      (:Is%20Not%20Valid
        (return 0)))))

(fn StartTemporaryProcess
  (params (Input :type Array%20of%20Strings))
  (bind (_isfound _program) (CallFunction|GetProgram Input))
  (if _isfound
    (bind (_temporaryprocess _isfound_2) (CallFunction|StartTemporaryProcess _program Input))
    (return _temporaryprocess _isfound_2)))

(fn GetDisplayName
  (return (Utilities|String|ToString(Text) (Utilities|Text|FormatText "<Program>{name}</>" (Variables|Default|GetFileName)))))

(fn GetPopupInfo
  (params (Parameters :type Array%20of%20Strings))
  (bind _info (CallFunction|GetDataInfo))
  (LocalVariables|SetDataText _info)
  (for _array_element (Variables|Default|GetPrograms)
    (LocalVariables|SetProgramText (Utilities|Text|FormatText "{text} 
{prog}" (LocalVariables|GetProgramText) (CallFunction|GetDisplayName _array_element))))
  (return (Utilities|Text|FormatText "{data} 
<input>--------------------</> 
{process}" (LocalVariables|GetDataText) (LocalVariables|GetProgramText))))

(fn SetupProgram
  (params (Tags :type Array%20of%20Strings) (Properties :type Map%20of%20Strings%20to%20Strings) (InStats :type Map%20of%20Strings%20to%20Reals))
  (if (== (Utilities|Array|Length (Variables|Default|GetPrograms)) 0)
    (CallFunction|SpawnPrograms))
  (CallFunction|SetupTagsandAliases Tags)
  (Helper|HidePrograms)
  (CallFunction|CalculateSize)
  (Default|AddDataObject (Variables|Default|GetShell) self)
  (return))

(fn SetupTagsandAliases
  (params (Tags :type Array%20of%20Strings))
  (for _array_element Tags
    (Utilities|Array|AddUnique (Variables|Default|GetDataTags) _array_element))
  (for _array_element_2 (Variables|Default|GetPrograms)
    (bind _output_get (LocalVariables|SetAProgram _array_element_2))
    (for _array_element_3 (Variables|/Game/Blueprints/GameObjects/BP_DataObject.BP_DataObject_C|GetDataTags _output_get)
      (Utilities|Array|AddUnique (Variables|Default|GetDataTags) _array_element_3))
    (Setup|SetAliases (LocalVariables|GetAProgram)))
  (return))

(fn CanAddProcess
  (params (AtShell :type BP%20Shell%20Object%20Reference) (Params :type Array%20of%20Strings))
  (bind (_isfound _program) (CallFunction|GetProgram Params))
  (if _isfound
    (bind (_canadd _cause) (CallFunction|CanAddProcess _program AtShell Params))
    (return _canadd _cause)))

(fn RandomizeStats
  (params (InLevel :type Float%20%28double-precision%29) (Params :type Array%20of%20Strings))
  (bind (_isfound _program) (CallFunction|GetProgram Params))
  (if _isfound
    (CallFunction|RandomizeStats _program (Variables|Default|GetLevel) Params)))

(fn CollectValidParameters
  (params (AtShell :type BP%20Shell%20Object%20Reference) (Input :type Array%20of%20Strings))
  (bind (_isfound _program) (CallFunction|GetProgram Input))
  (if _isfound
    (bind _validparameters (CallFunction|CollectValidParameters _program AtShell Input))
    (return _validparameters)))

(fn Duplicate
  (params (AtShell :type BP%20Shell%20Object%20Reference) (Input :type Array%20of%20Strings))
  (if (Utilities|Enum|Equal(Enum) (Utilities|Array|Get(acopy) Input) (Variables|Default|GetFileName))
    (bind _newobject (ShellInterface|DuplicatePackage AtShell Input))
    (return _newobject)
    (else
      (bind _newobject_2 (ShellInterface|DuplicateProgram AtShell Input))
      (return _newobject_2))))

(fn DuplicatePackage
  (params (AtShell :type BP%20Shell%20Object%20Reference) (Inputs :type Array%20of%20Strings))
  (for _array_element (Variables|Default|GetPrograms)
    (bind _newobject (CallFunction|Duplicate _array_element AtShell (Utilities|Array|MakeArray (Utilities|Array|Get(acopy) (Variables|/Game/Blueprints/GameObjects/BP_Program.BP_Program_C|GetAliases _array_element)))))
    (bind _asbp_program (Utilities|Casting|CastToBP_Program _newobject))
    (Utilities|Array|Add (LocalVariables|GetNewPrograms) _asbp_program))
  (bind _returnvalue (Game|SpawnActorfromClass (Utilities|GetClass self) (Transformation|GetActorTransform AtShell) "Undefined" "MultiplyWithRoot" 0 (LocalVariables|GetNewPrograms) 0 "/Game/Blueprints/Processes/BP_Process.BP_Process_C" (Variables|Default|GetLevel) 0 (Variables|Default|GetFileName) (Variables|Default|GetDataTags) AtShell (Variables|Default|GetreadAccess) false 0))
  (CallFunction|PostDuplicate _returnvalue AtShell)
  (return _returnvalue))

(fn DuplicateProgram
  (params (AtShell :type BP%20Shell%20Object%20Reference) (Inputs :type Array%20of%20Strings))
  (bind (_isfound _program) (CallFunction|GetProgram Inputs))
  (if _isfound
    (bind _newobject (CallFunction|Duplicate _program AtShell Inputs))
    (return _newobject)))

(fn GetProgram
  (params (Params :type Array%20of%20Strings))
  (bind _output (Utilities|Array|Get(acopy) Params))
  (bind _mappedaliases (Variables|Default|GetMappedAliases))
  (bind _returnvalue (Utilities|String|ParseIntoArray _output "/"))
  (bind _returnvalue_2 (Utilities|Array|LastIndex _returnvalue))
  (bind _output_2 (Utilities|Array|Get(acopy) _returnvalue _returnvalue_2))
  (bind (_value _returnvalue_3) (Utilities|Map|Find _mappedaliases _output_2))
  (return _returnvalue_3 _value))

(fn Orbit
  (params (Alpha :type Float%20%28single-precision%29))
  (bind _output_get (LocalVariables|SetNewRotation (Math|Rotator|Lerp(Rotator) (Variables|Default|GetOrbitStart) (Variables|Default|GetOrbitRotator) Alpha true)))
  (Transformation|SetRelativeRotation (Variables|Default|GetAnchor) _output_get false false)
  (for _array_element (Variables|Default|GetPrograms)
    (Transformation|SetRelativeRotation (Variables|/Game/Blueprints/GameObjects/BP_ShellObject.BP_ShellObject_C|GetAnchor _array_element) (LocalVariables|GetNewRotation) false false)))

(fn SpawnPrograms
  (bind _asbp_game_manager (Utilities|Casting|CastToBP_GameManager (Game|GetGameMode)))
  (LocalVariables|SetNetworkBuilder (Variables|/Game/GameMode/BP_GameManager.BP_GameManager_C|GetNetworkBuilder _asbp_game_manager))
  (for _array_element (Variables|Default|GetProcessTypes)
    (bind _program (Default|SpawnProgram (LocalVariables|GetNetworkBuilder) (Utilities|Array|Get(acopy) (.Aliases (Utilities|GetClassDefaults _array_element))) (.Load (Utilities|GetClassDefaults _array_element)) 0 true "" 0 (Variables|Default|GetLevel) (Utilities|Map|MakeMap) (Variables|Default|GetShell) (Utilities|Array|MakeArray _array_element) (Variables|Default|GetreadAccess) false (Utilities|Map|MakeMap) false))
    (Utilities|Array|Add (Variables|Default|GetPrograms) _program)))