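; BP_Shell is a network node actor holding data objects and processes within data, memory and thread capacities.
; It indexes files, programs (highest level per alias), processes and navigation links by lowercase name, enabling recursive flagged reachability searches across linked shells.
; Read access drives visibility; timelines animate bobbing, pulses, and pull or push slides.
; Shells also relay packet events and raise alerts, and isolated ones slide away, then delete their contents and themselves.
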(event Custom|PlayPulse
  (bind _scale (Timeline|PulseTimeline PlayFromStart)
    (:Update
      (Transformation|SetRelativeScale3D (Variables|Default|GetBounce) _scale))))

(event Custom|PlaySlide
  (bind _alpha (Timeline|SlideTimeline PlayFromStart)
    (:Update
      (Animation|DoSlide _alpha))
    (:Finished
      (if (Variables|Runtime|GetBeingShutdown)
        (Setup|ShutdownShell)))))

(event EventBeginPlay
  (|CallParentFunction)
  (CallFunction|Setup)
  (bind _height (Timeline|OscillateTimeline SetNewTime)
    (:Update
      (Animation|Oscillate _height))))

(fn ConstructionScript)

(fn AddDataObject
  (params (DataObject :type BP%20Data%20Object%20Object%20Reference))
  (Utilities|IsValid DataObject
    (:Is%20Valid
      (Utilities|Array|AddUnique (Variables|Runtime|GetDataObjects) DataObject)
      (bind _asbp_program (Utilities|Casting|CastToBP_Program DataObject)
        (:then
          (bind _output_get (LocalVariables|SetNewProgram _asbp_program))
          (for _array_element (Variables|/Game/Blueprints/GameObjects/BP_Program.BP_Program_C|GetAliases _output_get)
            (bind _output_get_2 (LocalVariables|Setalias (Utilities|String|ToLower _array_element)))
            (if (.ReturnValue (Utilities|Map|Find (Variables|ShellInterface|GetLocalPrograms) _output_get_2))
              (if (> (Variables|/Game/Blueprints/GameObjects/BP_Program.BP_Program_C|GetLevel (LocalVariables|GetNewProgram)) (Variables|/Game/Blueprints/GameObjects/BP_Program.BP_Program_C|GetLevel (.Value (Utilities|Map|Find (Variables|ShellInterface|GetLocalPrograms) _output_get_2))))
                (Utilities|Map|Add (Variables|ShellInterface|GetLocalPrograms) (LocalVariables|Getalias) (LocalVariables|GetNewProgram)))
              (else
                (Utilities|Map|Add (Variables|ShellInterface|GetLocalPrograms) (LocalVariables|Getalias) (LocalVariables|GetNewProgram))))))
        (:CastFailed
          (Utilities|Map|Add (Variables|ShellInterface|GetLocalFiles) (Utilities|String|ToLower (Variables|/Game/Blueprints/GameObjects/BP_DataObject.BP_DataObject_C|GetFileName DataObject)) DataObject))))))

(fn AddProcess
  (params (Process :type BP%20Process%20Object%20Reference))
  (Utilities|IsValid Process
    (:Is%20Valid
      (Utilities|Array|AddUnique (Variables|Runtime|GetProcesses) Process)
      (bind _asbpi_navigation (Utilities|Casting|CastToBPI_Navigation Process)
        (:then
          (bind _output_get (LocalVariables|SetLink _asbpi_navigation))
          (bind _islink (Default|IsLink _output_get))
          (if _islink
            (bind _shell (Default|GetAddressShell (LocalVariables|GetLink)))
            (Utilities|IsValid _shell
              (:Is%20Valid
                (Utilities|Map|Add (Variables|ShellInterface|GetLocalLinks) (Utilities|String|ToLower (Variables|BP_Shell_C|GetName _shell)) Process)))
            (else
              (for _array_element (Variables|/Game/Blueprints/Processes/BP_Process.BP_Process_C|GetAliases Process) :!label _label
                (Utilities|Map|Add (Variables|ShellInterface|GetLocalProcesses) (Utilities|String|ToLower _array_element) Process)))))
        (:CastFailed
          (goto _label))))))

(fn CollectChildren
  (for _array_element (Actor|GetAttachedActors true false)
    (bind _asbp_data_object (Utilities|Casting|CastToBP_DataObject _array_element))
    (ShellInterface|AddDataObject _asbp_data_object)))

(fn RemoveDataObject
  (params (DataObject :type BP%20Data%20Object%20Object%20Reference))
  (Utilities|IsValid DataObject
    (:Is%20Valid
      (Utilities|Array|RemoveItem (Variables|Runtime|GetDataObjects) DataObject)
      (Variables|/Game/Blueprints/GameObjects/BP_ShellObject.BP_ShellObject_C|SetShell DataObject 0)
      (bind _asbp_program (Utilities|Casting|CastToBP_Program DataObject)
        (:then
          (for _array_element (Variables|/Game/Blueprints/GameObjects/BP_Program.BP_Program_C|GetAliases _asbp_program)
            (bind _returnvalue (Utilities|Map|Remove (Variables|ShellInterface|GetLocalPrograms) _array_element))
            (if _returnvalue
              (LocalVariables|SetDoAliasUpdate true)))
          (if (LocalVariables|GetDoAliasUpdate)
            (for _array_element_2 (Variables|Runtime|GetDataObjects)
              (ShellInterface|AddDataObject _array_element_2))))
        (:CastFailed
          (Utilities|Map|Remove (Variables|ShellInterface|GetLocalFiles) (Variables|/Game/Blueprints/GameObjects/BP_DataObject.BP_DataObject_C|GetFileName DataObject)))))))

(fn RemoveProcess
  (params (Process :type BP%20Process%20Object%20Reference))
  (Utilities|IsValid Process
    (:Is%20Valid
      (Utilities|Array|RemoveItem (Variables|Runtime|GetProcesses) Process)
      (bind _process (LocalVariables|GetProcess)
        (:then
          (Variables|/Game/Blueprints/GameObjects/BP_ShellObject.BP_ShellObject_C|SetShell _process 0)
          (bind _asbpi_navigation (Utilities|Casting|CastToBPI_Navigation Process)
            (:then
              (bind _shell (Default|GetAddressShell _asbpi_navigation))
              (Utilities|IsValid _shell
                (:Is%20Valid
                  (bind _returnvalue (Utilities|Map|Remove (Variables|ShellInterface|GetLocalLinks) (Utilities|String|ToLower (Variables|BP_Shell_C|GetName _shell))))
                  (if _returnvalue
                    (Setup|CheckIsolation)
                    (for _array_element (Variables|Runtime|GetProcesses)
                      (ShellInterface|AddProcess _array_element))))))
            (:CastFailed
              (for _array_element_2 (Variables|/Game/Blueprints/Processes/BP_Process.BP_Process_C|GetAliases Process)
                (bind _returnvalue_2 (Utilities|Map|Remove (Variables|ShellInterface|GetLocalProcesses) (Utilities|String|ToLower _array_element_2)))
                (if _returnvalue_2
                  (LocalVariables|SetDoUpdateProcesses true)))
              (if (LocalVariables|GetDoUpdateProcesses)
                (for _array_element_3 (Variables|Runtime|GetProcesses)
                  (ShellInterface|AddProcess _array_element_3))))))
        (:else)))))

(fn CanAddDataObject
  (params (Size :type Integer))
  (bind _data (ShellInterface|GetUsedData))
  (return (>= (Variables|ShellInterface|GetData) (+ _data Size))))

(fn ShutdownShell
  (Variables|Runtime|SetHasShutdown true)
  (bind _asbp_game_manager (Utilities|Casting|CastToBP_GameManager (Game|GetGameMode)))
  (Utilities|Map|Remove (Variables|/Game/GameMode/NetworkBuilder/BP_NetworkBuilder.BP_NetworkBuilder_C|GetNetworkShells (Variables|/Game/GameMode/BP_GameManager.BP_GameManager_C|GetNetworkBuilder _asbp_game_manager)) (Utilities|String|ToLower (Variables|ShellInterface|GetName)))
  (Default|CallOnShutdownStarted)
  (Utilities|FlowControl|Sequence
    (:then_0
      (EventDispatchers|UnbindallEventsfromOnShutdownStarted))
    (:then_1
      (bind _output_get (LocalVariables|SetDataObjectsCopy (Variables|Runtime|GetDataObjects)))
      (for _array_element _output_get
        (Default|Delete _array_element true)))
    (:then_2
      (bind _output_get_2 (LocalVariables|SetProcessesCopy (Variables|Runtime|GetProcesses)))
      (for _array_element_2 _output_get_2
        (Default|Delete _array_element_2 true)))
    (:then_3
      (bind _output_get_3 (LocalVariables|SetFileCopy (Variables|ShellInterface|GetAddressFiles)))
      (for _array_element_3 _output_get_3
        (Default|Delete _array_element_3 true)))
    (:then_4
      (Actor|DestroyActor))))

(fn CanAddProcess
  (params (RequiredLoad :type Integer) (RequiredThreads :type Integer))
  (bind _memory (ShellInterface|GetUsedMemory))
  (bind _threads (ShellInterface|GetUsedThreads))
  (return (and (>= (Variables|ShellInterface|GetThreads) (+ RequiredThreads _threads)) (>= (Variables|ShellInterface|GetMemory) (+ _memory RequiredLoad))) (>= (Variables|ShellInterface|GetMemory) (+ _memory RequiredLoad))))

(fn Oscillate
  (params (Height :type Float%20%28double-precision%29))
  (Transformation|SetRelativeLocation (Variables|Default|GetBounce) (Math|Vector|MakeVector 0.0 0.0 (* Height (Variables|Animation|GetOscillationRange))) false false)
  (Components|Timeline|SetPlayRate (Variables|Default|GetOscillateTimeline) (Variables|Animation|GetOscillationRate)))

(fn StartPull
  (params (ToShell :type BP%20Shell%20Object%20Reference) (Forced :type Boolean) (GiveReadAccess :type Boolean))
  (if (or (not (Variables|ShellInterface|GetReadAccess)) Forced)
    (Variables|Animation|SetSlideEndTransform (Math|Transform|MakeTransform (+ (Transformation|GetActorLocation ToShell) (* (Math|Random|RandomUnitVector) (Variables|Animation|GetPullRange)))))
    (Variables|Animation|SetSlideStartTransform (Math|Transform|MakeTransform (Transformation|GetActorLocation)))
    (ShellInterface|SetVisible GiveReadAccess)
    (CallFunction|PlaySlide)))

(fn DoSlide
  (params (Alpha :type Float%20%28double-precision%29))
  (Transformation|SetActorTransform (Math|Transform|Lerp(Transform) (Variables|Animation|GetSlideStartTransform) (Variables|Animation|GetSlideEndTransform) Alpha)))

(fn GetUsedMemory
  (for _array_element (Variables|Runtime|GetProcesses)
    (LocalVariables|SetMemoryCount (+ (Variables|/Game/Blueprints/Processes/BP_Process.BP_Process_C|GetLoad _array_element) (LocalVariables|GetMemoryCount))))
  (return (LocalVariables|GetMemoryCount)))

(fn GetUsedData
  (for _array_element (Variables|Runtime|GetDataObjects)
    (LocalVariables|SetDataCount (+ (Variables|/Game/Blueprints/GameObjects/BP_DataObject.BP_DataObject_C|GetSize _array_element) (LocalVariables|GetDataCount))))
  (return (LocalVariables|GetDataCount)))

(fn GetUsedThreads
  (for _array_element (Variables|Runtime|GetProcesses)
    (LocalVariables|SetThreadsCount (+ (Variables|/Game/Blueprints/Processes/BP_Process.BP_Process_C|GetThreads _array_element) (LocalVariables|GetThreadsCount))))
  (return (LocalVariables|GetThreadsCount)))

(fn GetInfo
  (params (IgnoreProcess :type BP%20Process%20Object%20Reference) (HasReadAccess :type Boolean))
  (ShellInterface|SetVisible (or HasReadAccess (Variables|ShellInterface|GetReadAccess)))
  (bind _output (Info|CollectDataInfo HasReadAccess))
  (bind _output_2 (Info|CollectMemoryInfo IgnoreProcess HasReadAccess))
  (return (Utilities|Text|FormatText "{list} 
 
{ps} 
" _output _output_2)))

(fn CollectDataObjectInfo
  (params (HasReadAccess :type Boolean))
  (for _array_element (Variables|Runtime|GetDataObjects)
    (bind _output (Default|GetInfo _array_element HasReadAccess))
    (if (not (Utilities|Text|TextIsEmpty _output))
      (LocalVariables|SetListOutput (Utilities|Text|FormatText "{input} 
{output}" (LocalVariables|GetListOutput) _output))))
  (return (LocalVariables|GetListOutput)))

(fn CollectProcessInfo
  (params (IgnoreProcess :type BP%20Process%20Object%20Reference) (HasReadAccess :type Boolean))
  (for _array_element (Variables|Runtime|GetProcesses)
    (if (!= _array_element IgnoreProcess)
      (bind _output (Default|GetInfo _array_element HasReadAccess))
      (if (not (Utilities|Text|TextIsEmpty _output))
        (LocalVariables|SetOutputText (Utilities|Text|FormatText "{input} 
{output}" (LocalVariables|GetOutputText) _output)))))
  (return (LocalVariables|GetOutputText)))

(fn CollectMemoryInfo
  (params (IgnoreProcess :type BP%20Process%20Object%20Reference) (HasReadAccess :type Boolean))
  (bind _output (Info|CollectProcessInfo IgnoreProcess HasReadAccess))
  (bind _threads (ShellInterface|GetUsedThreads))
  (bind _memory (ShellInterface|GetUsedMemory))
  (return (Utilities|Text|FormatText "Active Processes: 
Threads: {threads} <input>/</> {maxthreads} 
<input>-------</> {used} <input>/</> {max} <input>-------</>{ps}" _threads (Variables|ShellInterface|GetThreads) _memory (Variables|ShellInterface|GetMemory) _output)))

(fn CollectDataInfo
  (params (HasReadAccess :type Boolean))
  (bind _returnvalue (Info|CollectDataObjectInfo HasReadAccess))
  (bind _data (ShellInterface|GetUsedData))
  (return (Utilities|Text|FormatText "<shell>{name}</>: 
<input>-------</> {used} <input>/</> {max} <input>-------</>{ls}" (Variables|ShellInterface|GetName) _data (Variables|ShellInterface|GetData) _returnvalue)))

(fn PacketApproaching
  (params (Packet :type BP%20Packet%20Object%20Reference) (FromShell :type BP%20Shell%20Object%20Reference))
  (Default|CallOnPacketApproach Packet FromShell))

(fn BumptoMusic
  (bind _asbp_game_manager (Utilities|Casting|CastToBP_GameManager (Game|GetGameMode)))
  (bind _outvalue (CallFunction|AverageRange 0 5 (Variables|/Game/GameMode/BP_GameManager.BP_GameManager_C|GetMusicConstants _asbp_game_manager)))
  (Transformation|SetRelativeScale3D (Variables|Default|GetBump) (Math|Vector|MakeVector (Math|Float|Clamp(Float) (+ (/ (- _outvalue 0.5) 2.0) 0.8) 0.8 1.1) (Math|Float|Clamp(Float) (+ (/ (- _outvalue 0.5) 2.0) 0.8) 0.8 1.1) (Math|Float|Clamp(Float) (+ (/ (- _outvalue 0.5) 2.0) 0.8) 0.8 1.1))))

(fn PacketIntercepted
  (params (Packet :type BP%20Packet%20Object%20Reference) (Process :type BP%20Process%20Object%20Reference))
  (Default|CallOnPacketIntercepted Packet Process))

(fn CheckIsolation
  (if (not (Variables|Runtime|GetBeingShutdown))
    (bind _isisolated (Setup|GetIsIsolated))
    (if _isisolated
      (Animation|StartPush))))

(fn StartPush
  (Default|CallOnPushStarted)
  (Utilities|FlowControl|Sequence
    (:then_0
      (EventDispatchers|UnbindallEventsfromOnPushStarted)
      (EventDispatchers|UnbindallEventsfromOnPacketApproach)
      (EventDispatchers|UnbindallEventsfromOnPacketIntercepted)
      (Variables|Runtime|SetBeingShutdown true)
      (CallFunction|UnregisterCameraFocus false))
    (:then_1
      (Variables|Animation|SetSlideStartTransform (Math|Transform|MakeTransform (Transformation|GetActorLocation)))
      (bind _shelltransform (Default|FindNewShellPosition (Variables|/Game/GameMode/BP_GameManager.BP_GameManager_C|GetNetworkBuilder (Variables|Runtime|GetGameManager))))
      (Variables|Animation|SetSlideEndTransform (Math|Transform|MakeTransform (.Location (Math|Transform|BreakTransform _shelltransform)) (.Rotation (Math|Transform|BreakTransform _shelltransform)) "0.000000,0.000000,0.000000"))
      (Utilities|Map|Remove (Variables|/Game/GameMode/NetworkBuilder/BP_NetworkBuilder.BP_NetworkBuilder_C|GetNetworkShells (Variables|/Game/GameMode/BP_GameManager.BP_GameManager_C|GetNetworkBuilder (Variables|Runtime|GetGameManager))) (Utilities|String|ToLower (Variables|ShellInterface|GetName)))
      (CallFunction|PlaySlide))))

(fn GetIsIsolated
  (for _array_element (Variables|Runtime|GetProcesses)
    (Utilities|Casting|CastToBPI_Navigation _array_element)
    (return false))
  (return (and (== (Utilities|Array|Length (Variables|ShellInterface|GetAddressFiles)) 0) (not (Variables|ShellInterface|GetAnchored)))))

(fn SetName
  (params (NewName :type String))
  (Default|CallOnNameChange NewName (Variables|ShellInterface|GetName))
  (bind _asbp_game_manager (Utilities|Casting|CastToBP_GameManager (Game|GetGameMode)))
  (bind _output_get (LocalVariables|SetNetworkBuilder (Variables|/Game/GameMode/BP_GameManager.BP_GameManager_C|GetNetworkBuilder _asbp_game_manager)))
  (if (not (.ReturnValue (Utilities|Map|Find (Variables|/Game/GameMode/NetworkBuilder/BP_NetworkBuilder.BP_NetworkBuilder_C|GetNetworkShells _output_get) (Utilities|String|ToLower NewName))))
    (Utilities|Map|Remove (Variables|/Game/GameMode/NetworkBuilder/BP_NetworkBuilder.BP_NetworkBuilder_C|GetNetworkShells (LocalVariables|GetNetworkBuilder)) (Variables|ShellInterface|GetName))
    (bind _output_get_2 (Variables|ShellInterface|SetName NewName))
    (Utilities|Map|Add (Variables|/Game/GameMode/NetworkBuilder/BP_NetworkBuilder.BP_NetworkBuilder_C|GetNetworkShells (LocalVariables|GetNetworkBuilder)) (Utilities|String|ToLower _output_get_2) self)
    (Animation|UpdateTextLabel)
    (for _array_element (Variables|ShellInterface|GetAddressFiles)
      (Variables|/Game/Blueprints/GameObjects/BP_DataObject.BP_DataObject_C|SetFileName _array_element (Utilities|GetAddressFileName self)))))

(fn SetVisible
  (params (NewState :type Boolean))
  (bind _output_get (Variables|ShellInterface|SetReadAccess NewState))
  (Rendering|SetActorHiddenInGame (not _output_get)))

(fn PacketArrived
  (params (Packet :type BP%20Packet%20Object%20Reference) (FromShell :type BP%20Shell%20Object%20Reference))
  (Default|CallOnPacketArrived Packet FromShell)
  (if (Variables|ShellInterface|GetReadAccess)
    (CallFunction|RegisterCameraFocus 5.0 0.02 3.0 false false false)))

(fn PacketLanded
  (params (Packet :type BP%20Packet%20Object%20Reference))
  (Default|CallOnPacketLanded Packet))

(fn PacketSending
  (params (Packet :type BP%20Packet%20Object%20Reference) (ToShell :type BP%20Shell%20Object%20Reference))
  (Default|CallOnPacketSending Packet ToShell))

(fn Setup
  (bind _asbp_game_manager (Utilities|Casting|CastToBP_GameManager (Game|GetGameMode)))
  (Variables|Runtime|SetGameManager _asbp_game_manager)
  (Animation|UpdateTextLabel)
  (Setup|CollectChildren)
  (ShellInterface|SetVisible (Variables|ShellInterface|GetReadAccess)))

(fn CollectReachableShells
  (params (InMap :type Map%20of%20Strings%20to%20Objects) (Flag :type Boolean) (ReadAccessOnly :type Boolean))
  (LocalVariables|SetCollectedShells InMap)
  (if (!= Flag (Variables|Runtime|GetReachableFlag))
    (Variables|Runtime|SetReachableFlag Flag)
    (bind _keys (Utilities|Map|Keys (Variables|ShellInterface|GetLocalLinks)))
    (for _array_element _keys
      (bind _output_get (LocalVariables|SetTempName _array_element))
      (LocalVariables|SetTempProcess (.Value (Utilities|Map|Find (Variables|ShellInterface|GetLocalLinks) _output_get)))
      (if (or (Variables|/Game/Blueprints/GameObjects/BP_ShellObject.BP_ShellObject_C|GetreadAccess (.Value (Utilities|Map|Find (Variables|ShellInterface|GetLocalLinks) _output_get))) (not ReadAccessOnly))
        (bind _asbpi_navigation (Utilities|Casting|CastToBPI_Navigation (LocalVariables|GetTempProcess)))
        (bind _shell (Default|GetAddressShell _asbpi_navigation))
        (bind _output_get_2 (LocalVariables|SetTempShell _shell))
        (Utilities|Map|Add (LocalVariables|GetCollectedShells) (LocalVariables|GetTempName) _output_get_2)
        (bind _shells (ShellInterface|CollectReachableShells (LocalVariables|GetTempShell) (LocalVariables|GetCollectedShells) Flag ReadAccessOnly))
        (LocalVariables|SetCollectedShells _shells)))
    (return (LocalVariables|GetCollectedShells))
    (else
      (return (LocalVariables|GetCollectedShells)))))

(fn UpdateTextLabel
  (Rendering|Components|TextRender|SetText (Variables|Default|GetNameText) (Utilities|Text|FormatText "//{name}" (Variables|ShellInterface|GetName))))

(fn GetPopupInfo
  (params (Parameters :type Array%20of%20Strings))
  (|CallParentFunction Parameters)
  (bind _output (Info|GetInfo 0 false))
  (return _output))

(fn InitiateNeighbourPull
  (bind _keys (Utilities|Map|Keys (Variables|ShellInterface|GetLocalLinks)))
  (for _array_element _keys
    (bind _asbpi_navigation (Utilities|Casting|CastToBPI_Navigation (.Value (Utilities|Map|Find (Variables|ShellInterface|GetLocalLinks) _array_element))))
    (bind _shell (Default|GetAddressShell _asbpi_navigation))
    (Utilities|IsValid _shell
      (:Is%20Valid
        (Animation|StartPull _shell self true (Variables|/Game/Blueprints/GameObjects/BP_ShellObject.BP_ShellObject_C|GetreadAccess (.Value (Utilities|Map|Find (Variables|ShellInterface|GetLocalLinks) _array_element))))))))

(fn GenerateAlert
  (params (Value :type Float%20%28double-precision%29))
  (Variables|Default|SetAccumulatedAlert (+ (Variables|Default|GetAccumulatedAlert) Value))
  (Default|GenerateAlert (Variables|Runtime|GetGameManager) Value self))

(fn GetAccumulatedAlert
  (return (Math|Float|Max(Float) (- (Variables|Default|GetAccumulatedAlert) (* (- (Actor|GetGameTimeSinceCreation) (Variables|Default|GetAlertTimestamp)) (Variables|Default|GetAlertDecayRate))) 0.0)))