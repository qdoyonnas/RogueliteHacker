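; Root program actor that turns typed command aliases into process actors on the player's root shell.
; Setup maps aliases from the RootPrograms table; when the network's root spawns, it registers with the Interpreter and reveals and focuses the shell.
; Starting a process checks that map, then the Interpreter's terminal commands, while Duplicate spawns new program copies from mapped types.
; Parameter collection and popup info come from short-lived temporary process actors.
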(fn ConstructionScript
  (|CallParentFunction))

(fn SetupProgram
  (params (Tags :type Array%20of%20Strings) (Properties :type Map%20of%20Strings%20to%20Strings) (InStats :type Map%20of%20Strings%20to%20Reals))
  (bind _asbp_game_manager (Utilities|Casting|CastToBP_GameManager (Game|GetGameMode)))
  (EventDispatchers|BindEventtoOnRootSpawned (Variables|/Game/GameMode/BP_GameManager.BP_GameManager_C|GetNetworkBuilder _asbp_game_manager) (EventDispatchers|CreateEvent :!event OnRootSpawned))
  (CallFunction|SetupRootProgram)
  (CallFunction|CalculateSize)
  (Default|AddDataObject (Variables|Default|GetShell) self)
  (return))

(fn OnRootSpawned
  (CallFunction|SetupInterpreter)
  (CallFunction|SetupRootShell)
  (Default|RegisterCameraFocus (Variables|Default|GetShell) 0.0 0.0 2.0 false true true))

(fn SetupRootProgram
  (bind _outrownames (DataTable|GetDataTableRowNames (Variables|Default|GetRootPrograms)))
  (for _array_element _outrownames
    (bind _returnvalue (Utilities|GetDataTableRow (Variables|Default|GetRootPrograms) _array_element)
      (:then
        (for _array_element_2 (.Aliases (Utilities|GetClassDefaults (Utilities|Struct|BreakStruct_Command _returnvalue)))
          (Utilities|Array|AddUnique (Variables|Default|GetAliases) _array_element_2)
          (Utilities|Map|Add (Variables|Default|GetMappedAliases) _array_element_2 (Utilities|Struct|BreakStruct_Command _returnvalue)))))))

(fn SetupInterpreter
  (bind _asbp_game_manager (Utilities|Casting|CastToBP_GameManager (Game|GetGameMode)))
  (Variables|Default|SetInterpreter (Variables|/Game/GameMode/BP_GameManager.BP_GameManager_C|GetInterpreter _asbp_game_manager))
  (Variables|/Game/Blueprints/BP_Interpreter.BP_Interpreter_C|SetRootShell (Variables|Default|GetInterpreter) (Variables|Default|GetShell))
  (Variables|/Game/Blueprints/BP_Interpreter.BP_Interpreter_C|SetRootProgram (Variables|Default|GetInterpreter) self)
  (EventDispatchers|BindEventtoOnDelete (EventDispatchers|CreateEvent (Variables|Default|GetInterpreter) :!event RootDeleted)))

(fn SetupRootShell
  (bind _shell (Variables|Default|GetShell))
  (Default|SetVisible _shell true)
  (for _array_element (Variables|/Game/Blueprints/GameObjects/BP_Shell.BP_Shell_C|GetDataObjects _shell)
    (Default|SetVisible _array_element true)
    (Variables|/Game/Blueprints/GameObjects/BP_Shell.BP_Shell_C|SetAnchored (Variables|Default|GetShell) true)))

(fn Setup
  (|CallParentFunction)
  (CallFunction|SetupProgram 0 (Utilities|Map|MakeMap) (Utilities|Map|MakeMap)))

(fn StartProcess
  (params (Params :type Array%20of%20Strings) (IsPlayerOwned :type Boolean) (AtShell :type BP%20Shell%20Object%20Reference) (FastForward :type Boolean))
  (bind _output (Utilities|Array|Get(acopy) Params))
  (bind (_processtype _isfound) (Utilities|GetMappedProcess _output))
  (LocalVariables|SetTargetShell (select (Utilities|IsValid AtShell) AtShell (Variables|Default|GetShell)))
  (if _isfound
    (bind _process (CallFunction|StartProcessfromType Params _processtype (LocalVariables|GetTargetShell) IsPlayerOwned))
    (CallFunction|PlayStart)
    (return _process)
    (else
      (bind (_type _found) (CallFunction|GetTerminalCommandfromAlias (Utilities|Array|Get(acopy) Params)))
      (if _found
        (bind _process_2 (CallFunction|StartProcessfromType Params _type (LocalVariables|GetTargetShell) IsPlayerOwned))
        (CallFunction|PlayStart)
        (return _process_2)))))

(fn StartProcessfromType
  (params (Params :type Array%20of%20Strings) (Type :type BP%20Process%20Class%20Reference) (AtShell :type BP%20Shell%20Object%20Reference) (IsPlayerOwned :type Boolean))
  (Utilities|Array|RemoveIndex Params)
  (bind _returnvalue (Game|SpawnActorfromClass Type (Math|Transform|MakeTransform "0, 0, 0") "Undefined" "MultiplyWithRoot" 0 self false (Utilities|Map|MakeMap) Params 1.0 IsPlayerOwned false AtShell (Variables|Default|GetreadAccess) false 0))
  (return _returnvalue))

(fn CanAddProcess
  (params (AtShell :type BP%20Shell%20Object%20Reference) (Params :type Array%20of%20Strings))
  (bind _output (Utilities|Array|Get(acopy) Params))
  (bind (_processtype _isfound) (Utilities|GetMappedProcess _output))
  (bind (_load _threads) (Utilities|GetClassDefaults _processtype))
  (if _isfound
    (bind (_canadd _isthreads) (Default|CanAddProcess AtShell _load _threads))
    (return _canadd _isthreads)))

(fn CollectValidParameters
  (params (AtShell :type BP%20Shell%20Object%20Reference) (Input :type Array%20of%20Strings))
  (bind (_temporaryprocess _isfound) (CallFunction|StartTemporaryProcess Input))
  (LocalVariables|SetTemporaryProcess _temporaryprocess)
  (if _isfound
    (bind _validparameters (Default|CollectfromParam (LocalVariables|GetTemporaryProcess) (- (Utilities|Array|LastIndex Input) 1) AtShell Input))
    (Actor|DestroyActor (LocalVariables|GetTemporaryProcess))
    (return _validparameters)
    (else
      (return ""))))

(fn GetTerminalCommandfromAlias
  (params (Input :type String))
  (bind _outrownames (DataTable|GetDataTableRowNames (Variables|/Game/Blueprints/BP_Interpreter.BP_Interpreter_C|GetTerminalCommands (Variables|Default|GetInterpreter))))
  (for _array_element _outrownames
    (bind _returnvalue (Utilities|GetDataTableRow (Variables|/Game/Blueprints/BP_Interpreter.BP_Interpreter_C|GetTerminalCommands (Variables|Default|GetInterpreter)) _array_element)
      (:then
        (bind _output_get (LocalVariables|SetCommandType (Utilities|Struct|BreakStruct_Command _returnvalue)))
        (for _array_element_2 (.Aliases (Utilities|GetClassDefaults _output_get))
          (if (Utilities|Enum|Equal(Enum) _array_element_2 Input)
            (return (LocalVariables|GetCommandType) true)))))))

(fn GetPopupInfo
  (params (Parameters :type Array%20of%20Strings))
  (bind _info (CallFunction|GetDataInfo))
  (bind _text (CallFunction|GetProcessInfo Parameters))
  (return (Utilities|Text|FormatText "{data} 
<input>--------------------</> 
{process}" _info _text)))

(fn Duplicate
  (params (Input :type Array%20of%20Strings))
  (bind _output (Utilities|Array|Get(acopy) Input))
  (bind (_processtype _isfound) (Utilities|GetMappedProcess _output))
  (bind _output_get (LocalVariables|SetType _processtype))
  (if _isfound
    (bind _returnvalue (Game|SpawnActorfromClass "/Game/Blueprints/GameObjects/BP_Program.BP_Program_C" (Math|Transform|MakeTransform "0, 0, 0") "Undefined" "MultiplyWithRoot" 0 _output_get 0.5 10 (Utilities|Array|Get(acopy) (.Aliases (Utilities|GetClassDefaults _processtype))) 0 (Variables|Default|GetShell) true false 0))
    (LocalVariables|SetNewProgram _returnvalue)
    (CallFunction|SetupProgram (LocalVariables|GetNewProgram) 0 (Utilities|Map|MakeMap) (Utilities|Map|MakeMap))
    (return (LocalVariables|GetNewProgram))))

(fn SetSecondaryFocus
  (params (CameraFocus :type BP%20Camera%20Focus%20Object%20Reference) (Input :type Array%20of%20Strings))
  (if (== CameraFocus self)
    (for (_array_element _array_index) Input
      (LocalVariables|SetParam _array_element)
      (if (!= _array_index 0)
        (if (.IsFound (Utilities|GetMappedProcess (LocalVariables|GetParam)))
          (Default|DisplaySecondaryInfoPopup (Variables|Default|GetInterpreter) self (Utilities|Array|MakeArray (LocalVariables|GetParam)))
          (return true))))
    (else
      (bind _valid (|CallParentFunction CameraFocus 0))
      (return _valid))))

(fn StartTemporaryProcess
  (params (Input :type Array%20of%20Strings))
  (bind (_type _isfound) (CallFunction|GetProcessType Input))
  (if _isfound
    (bind _returnvalue (Game|SpawnActorfromClass _type (Math|Transform|MakeTransform "0, 0, 0") "Undefined" "MultiplyWithRoot" 0 self false (Utilities|Map|MakeMap) 0 0.0 false true (Variables|Default|GetShell) false false 0))
    (return _returnvalue true)))

(fn GetProcessType
  (params (Input :type Array%20of%20Strings))
  (bind _output (Utilities|Array|Get(acopy) Input))
  (bind (_processtype _isfound) (Utilities|GetMappedProcess _output))
  (if _isfound
    (return _processtype true)
    (else
      (bind (_type _found) (CallFunction|GetTerminalCommandfromAlias (Utilities|Array|Get(acopy) Input)))
      (if _found
        (return _type true)
        (else
          (return 0 false))))))

(fn GetProcessInfo
  (params (Input :type Array%20of%20Strings))
  (bind _array_element (Utilities|Array|ForEachLoopwithBreak Input :!label _label)
    (:LoopBody
      (bind (_temporaryprocess _isfound) (CallFunction|StartTemporaryProcess (Utilities|Array|MakeArray _array_element)))
      (if _isfound
        (LocalVariables|SetTempProc _temporaryprocess)
        (goto _label Break)))
    (:Completed
      (if (!= (LocalVariables|GetTempProc) 0)
        (bind _tempproc (LocalVariables|GetTempProc)
          (:then
            (bind _text (CallFunction|GetPopupInfo _tempproc Input))
            (LocalVariables|SetReturnText _text)
            (Actor|DestroyActor (LocalVariables|GetTempProc))
            (return (LocalVariables|GetReturnText)))
          (:else))
        (else
          (return "PROCESS NOT FOUND"))))))