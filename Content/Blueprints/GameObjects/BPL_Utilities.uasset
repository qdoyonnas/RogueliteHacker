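; Blueprint function library of shared helpers for a hacking game built on a network of Shells holding processes, links, programs and files.
; Lookups resolve shells, programs and data objects by name, alias, index or slash-delimited path.
; Graph queries follow navigation links: recursive connectivity checks, breadth-first pathfinding with optional read-access filtering, and two-way network scans for open ports.
; Small utilities cover sine oscillation, aiming, averaging, time formatting and curve-driven, level-scaled random stats.
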(fn Oscillate3DVector
  (params (Rate :type Float%20%28double-precision%29) (CycleOffset :type Float%20%28double-precision%29) (Distance :type Float%20%28double-precision%29))
  (return (Math|Vector|MakeVector 0.0 0.0 (* (Math|Trig|Sin(Radians) (+ (* (Class|KismetMathLibrary|ToUnixTimestampDouble (Math|DateTime|Now)) Rate) CycleOffset)) Distance))))

(fn Oscillate2DVector
  (params (Rate :type Float%20%28double-precision%29) (Cycle%20Offset :type Float%20%28double-precision%29) (Distance :type Float%20%28double-precision%29))
  (return (Math|Vector2D|MakeVector2D 0.0 (* (Math|Trig|Sin(Radians) (+ (* (Class|KismetMathLibrary|ToUnixTimestampDouble (Math|DateTime|Now)) Rate) Cycle%20Offset)) Distance))))

(fn FindAddress
  (params (AddressName :type String) (Shell :type BP%20Shell%20Object%20Reference))
  (for _array_element (Variables|/Game/Blueprints/GameObjects/BP_Shell.BP_Shell_C|GetDataObjects Shell)
    (bind _asfile_address (Utilities|Casting|CastToFile_Address _array_element))
    (if (Utilities|Enum|Equal(Enum) (Variables|/Game/Blueprints/GameObjects/BP_DataObject.BP_DataObject_C|GetFileName _asfile_address) AddressName)
      (return true (Variables|/Game/Blueprints/FileTypes/File_Address.File_Address_C|GetShellAddress _asfile_address) _asfile_address)))
  (return false 0 0))

(fn Pointat
  (params (Object :type Scene%20Component%20Object%20Reference) (Target :type Scene%20Component%20Object%20Reference))
  (bind _returnvalue (Transformation|GetWorldLocation Target))
  (bind _returnvalue_2 (Transformation|GetWorldLocation Object))
  (bind _returnvalue_3 (Math|Rotator|FindLookatRotation _returnvalue_2 _returnvalue))
  (bind (_roll _pitch _yaw) (Math|Rotator|BreakRotator _returnvalue_3))
  (Utilities|IsValid Target
    (:Is%20Valid
      (return (Math|Rotator|MakeRotator _roll (- _pitch 9e+01) _yaw)))
    (:Is%20Not%20Valid
      (return "0, 0, 0"))))

(fn CheckConnenctionExists
  (params (Shell :type BP%20Shell%20Object%20Reference) (Link :type String))
  (for _array_element (Variables|/Game/Blueprints/GameObjects/BP_Shell.BP_Shell_C|GetProcesses Shell)
    (bind _asbpi_navigation (Utilities|Casting|CastToBPI_Navigation _array_element))
    (bind _shell (Default|GetAddressShell _asbpi_navigation))
    (return (Utilities|Enum|Equal(Enum) (Variables|/Game/Blueprints/GameObjects/BP_Shell.BP_Shell_C|GetName _shell) Link))))

(fn MatchProcessAlias
  (params (Param :type String) (Process :type BP%20Process%20Object%20Reference))
  (bind _doesmatch (CallFunction|MatchProcessIndex Param Process))
  (if _doesmatch
    (return true)
    (else
      (Utilities|IsValid Process
        (:Is%20Valid
          (for _array_element (Variables|/Game/Blueprints/Processes/BP_Process.BP_Process_C|GetAliases Process)
            (if (Utilities|Enum|Equal(Enum) _array_element Param)
              (return true))))
        (:Is%20Not%20Valid
          _))
      (return false))))

(fn AverageRange
  (params (StartIndex :type Integer) (EndIndex :type Integer) (Array :type Array%20of%20Floats%20%28double-precision%29))
  (if (Utilities|Array|IsNotEmpty Array)
    (bind _output_get (LocalVariables|SetIndex StartIndex))
    (while (< _output_get EndIndex)
      (LocalVariables|SetValue (+ (Utilities|Array|Get(acopy) Array (LocalVariables|GetIndex)) (LocalVariables|GetValue)))
      (Math|Integer|IncrementInt (LocalVariables|GetIndex)))
    (bind _output_get_2 (LocalVariables|SetValue (/ (LocalVariables|GetValue) (- EndIndex StartIndex))))
    (return _output_get_2)))

(fn FindProgram
  (params (Shell :type BP%20Shell%20Object%20Reference) (Input :type String))
  (LocalVariables|SetAtShell Shell)
  (bind _output_get (LocalVariables|SetPath (Utilities|String|ParseIntoArray Input "/" false)))
  (LocalVariables|SetProgramName (Utilities|Array|Get(acopy) _output_get (Utilities|Array|LastIndex _output_get)))
  (Utilities|Array|RemoveIndex (LocalVariables|GetPath) (Utilities|Array|LastIndex (LocalVariables|GetPath)))
  (for _array_element (LocalVariables|GetPath)
    (bind (_isfound _linkprocess _linknav) (CallFunction|FindLinkonShell (LocalVariables|GetAtShell) _array_element))
    (if _isfound
      (bind _shell (Default|GetAddressShell _linknav))
      (LocalVariables|SetAtShell _shell)
      (else
        (return 0 false))))
  (bind (_program _isfound_2) (CallFunction|FindProgramonShell (LocalVariables|GetAtShell) (LocalVariables|GetProgramName)))
  (return _program _isfound_2))

(fn MatchProgramAlias
  (params (Param :type String) (Program :type BP%20Program%20Object%20Reference))
  (for _array_element (Variables|/Game/Blueprints/GameObjects/BP_Program.BP_Program_C|GetAliases Program)
    (if (Utilities|Enum|Equal(Enum) _array_element Param)
      (return true))))

(fn FindProgramonShell
  (params (Shell :type BP%20Shell%20Object%20Reference) (Input :type String))
  (for _array_element (Variables|/Game/Blueprints/GameObjects/BP_Shell.BP_Shell_C|GetDataObjects Shell)
    (bind _asbp_program (Utilities|Casting|CastToBP_Program _array_element))
    (bind _doesmatch (CallFunction|MatchProgramAlias Input _asbp_program))
    (if _doesmatch
      (return _asbp_program true)))
  (return 0 false))

(fn FindLinkonShell
  (params (Shell :type BP%20Shell%20Object%20Reference) (Name :type String))
  (for _array_element (Variables|/Game/Blueprints/GameObjects/BP_Shell.BP_Shell_C|GetProcesses Shell)
    (bind _output_get (LocalVariables|SetProcess _array_element))
    (bind _asbpi_navigation (Utilities|Casting|CastToBPI_Navigation _output_get))
    (bind _output_get_2 (LocalVariables|SetNav _asbpi_navigation))
    (bind _shell (Default|GetAddressShell _output_get_2))
    (Utilities|IsValid _shell
      (:Is%20Valid
        (bind _islink (Default|IsLink (LocalVariables|GetNav)))
        (if (and _islink (Utilities|Enum|Equal(Enum) (Utilities|String|ToLower (Variables|/Game/Blueprints/GameObjects/BP_Shell.BP_Shell_C|GetName _shell)) (Utilities|String|ToLower Name)))
          (return true (LocalVariables|GetProcess) (LocalVariables|GetNav))))))
  (return false 0 0))

(fn FloattoTime
  (params (Value :type Float%20%28double-precision%29))
  (LocalVariables|SetMinuteAmount (Math|Float|Floor (/ Value 6e+01)))
  (bind _output_get (LocalVariables|SetSecondsAmount (Math|Float|Floor (Math|Float|%(Float) Value 6e+01))))
  (return (Utilities|Text|FormatText "{min}:{sec}" (LocalVariables|GetMinuteAmount) (Utilities|Text|ToText(Integer) _output_get false true 2)) (LocalVariables|GetMinuteAmount) (LocalVariables|GetSecondsAmount)))

(fn AreShellsConnected
  (params (ShellA :type BP%20Shell%20Object%20Reference) (ShellB :type BP%20Shell%20Object%20Reference) (TraversedShells :type Array%20of%20BP%20Shell%20Object%20References))
  (if (and (Utilities|IsValid ShellA) (Utilities|IsValid ShellB))
    (bind _output_get (LocalVariables|SetLocalTraversed TraversedShells))
    (Utilities|Array|Add _output_get ShellA)
    (if (== ShellA ShellB)
      (Utilities|Array|Clear (LocalVariables|GetLocalTraversed))
      (return true)
      (else
        (for _array_element (Variables|/Game/Blueprints/GameObjects/BP_Shell.BP_Shell_C|GetProcesses ShellA)
          (bind _asbpi_navigation (Utilities|Casting|CastToBPI_Navigation _array_element))
          (bind _shell (Default|GetAddressShell _asbpi_navigation))
          (bind _output_get_2 (LocalVariables|SetLinkedShell _shell))
          (Utilities|IsValid _output_get_2
            (:Is%20Valid
              (if (not (Utilities|Array|ContainsItem (LocalVariables|GetLocalTraversed) _shell))
                (bind _areconnected (CallFunction|AreShellsConnected (LocalVariables|GetLinkedShell) ShellB (LocalVariables|GetLocalTraversed)))
                (if _areconnected
                  (Utilities|Array|Clear (LocalVariables|GetLocalTraversed))
                  (return true))))))
        (Utilities|Array|Clear (LocalVariables|GetLocalTraversed))
        (return false)))
    (else
      (return false))))

(fn FindDataObjectonShell
  (params (Shell :type BP%20Shell%20Object%20Reference) (FileName :type String))
  (for _array_element (Variables|/Game/Blueprints/GameObjects/BP_Shell.BP_Shell_C|GetDataObjects Shell)
    (if (Utilities|Enum|Equal(Enum) (Variables|/Game/Blueprints/GameObjects/BP_DataObject.BP_DataObject_C|GetFileName _array_element) FileName)
      (return true _array_element)))
  (return false 0))

(fn FindShellbyName
  (params (Name :type String) (RequireReadAccess :type Boolean) (AtShell :type BP%20Shell%20Object%20Reference))
  (if (Utilities|Enum|Equal(Enum) Name "~")
    (return AtShell false)
    (else
      (bind _asbp_game_manager (Utilities|Casting|CastToBP_GameManager (Game|GetGameMode)))
      (bind (_isfound _shell) (Default|FindShell (Variables|/Game/GameMode/BP_GameManager.BP_GameManager_C|GetNetworkBuilder _asbp_game_manager) Name))
      (bind _output_get (LocalVariables|SetFoundShell _shell))
      (Utilities|IsValid _output_get
        (:Is%20Valid
          (if (and (or (not RequireReadAccess) (Variables|/Game/Blueprints/GameObjects/BP_Shell.BP_Shell_C|GetReadAccess (LocalVariables|GetFoundShell))) _isfound)
            (return (LocalVariables|GetFoundShell) true)
            (else
              (return 0 false))))
        (:Is%20Not%20Valid
          (return 0 false))))))

(fn GetRandomProcessType
  (params (Types :type Array%20of%20BP%20Process%20Class%20References))
  (bind _returnvalue (Utilities|Array|LastIndex Types))
  (bind _returnvalue_2 (Math|Random|RandomIntegerinRange 0 _returnvalue))
  (bind _output (Utilities|Array|Get(acopy) Types _returnvalue_2))
  (return _output (Utilities|Array|Get(acopy) (.Aliases (Utilities|GetClassDefaults _output)))))

(fn GetShortestString
  (params (Strings :type Array%20of%20Strings))
  (LocalVariables|SetShort (Utilities|Array|Get(acopy) Strings))
  (for _array_element Strings
    (bind _output_get (LocalVariables|SetTemp _array_element))
    (if (and (or (< (Utilities|String|Len _output_get) (Utilities|String|Len (LocalVariables|GetShort))) (== (Utilities|String|Len (LocalVariables|GetShort)) 1)) (!= (Utilities|String|Len (LocalVariables|GetTemp)) 1))
      (LocalVariables|SetShort (LocalVariables|GetTemp))))
  (return (LocalVariables|GetShort)))

(fn FollowPath
  (params (AtShell :type BP%20Shell%20Object%20Reference) (Name :type String))
  (bind (_isfound _linkprocess _linknav) (CallFunction|FindLinkonShell AtShell Name))
  (if _isfound
    (bind _shell (Default|GetAddressShell _linknav))
    (Utilities|IsValid _shell
      (:Is%20Valid
        (return _shell true))
      (:Is%20Not%20Valid
        (return 0 false)))
    (else
      (return 0 false))))

(fn GetPathtoShell
  (params (StartShell :type BP%20Shell%20Object%20Reference) (EndShell :type BP%20Shell%20Object%20Reference) (RequireReadAccess :type Boolean))
  (if (!= StartShell EndShell)
    (Utilities|Array|Add (LocalVariables|GetShellQueue) StartShell)
    (Utilities|Array|Add (LocalVariables|GetPathQueue) "")
    (while (!= (Utilities|Array|Length (LocalVariables|GetShellQueue)) 0)
      (LocalVariables|SetTempShell (Utilities|Array|Get(acopy) (LocalVariables|GetShellQueue)))
      (LocalVariables|SetTempPath (Utilities|Array|Get(acopy) (LocalVariables|GetPathQueue)))
      (Utilities|Array|RemoveIndex (LocalVariables|GetShellQueue))
      (Utilities|Array|RemoveIndex (LocalVariables|GetPathQueue))
      (Utilities|Array|Add (LocalVariables|GetVisitedShells) (LocalVariables|GetTempShell))
      (bind (_foundpath _found _shellqueue _pathqueue) (CallFunction|ProcessShellforPath (LocalVariables|GetTempShell) (LocalVariables|GetTempPath) EndShell (LocalVariables|GetVisitedShells) RequireReadAccess))
      (if _found
        (return _foundpath)
        (else
          (Utilities|Array|AppendArray (LocalVariables|GetShellQueue) _shellqueue)
          (Utilities|Array|AppendArray (LocalVariables|GetPathQueue) _pathqueue))))
    (return (Variables|/Game/Blueprints/GameObjects/BP_Shell.BP_Shell_C|GetName EndShell))
    (else
      (return ""))))

(fn ProcessShellforPath
  (params (Shell :type BP%20Shell%20Object%20Reference) (Path :type String) (Target :type BP%20Shell%20Object%20Reference) (VisitedShells :type Array%20of%20BP%20Shell%20Object%20References) (RequireReadAccess :type Boolean))
  (bind _collectedpaths (LocalVariables|GetCollectedPaths))
  (bind _keys (Utilities|Map|Keys (Variables|/Game/Blueprints/GameObjects/BP_Shell.BP_Shell_C|GetLocalLinks Shell)))
  (for _array_element _keys
    (bind _output_get (LocalVariables|SetLinkName _array_element))
    (if (or (Variables|/Game/Blueprints/GameObjects/BP_ShellObject.BP_ShellObject_C|GetreadAccess (.Value (Utilities|Map|Find (Variables|/Game/Blueprints/GameObjects/BP_Shell.BP_Shell_C|GetLocalLinks Shell) _output_get))) (not RequireReadAccess))
      (bind _asbpi_navigation (Utilities|Casting|CastToBPI_Navigation (.Value (Utilities|Map|Find (Variables|/Game/Blueprints/GameObjects/BP_Shell.BP_Shell_C|GetLocalLinks Shell) _output_get))))
      (bind _shell (Default|GetAddressShell _asbpi_navigation))
      (bind _output_get_2 (LocalVariables|SetTempShell _shell))
      (if (not (Utilities|Array|ContainsItem VisitedShells _output_get_2))
        (Utilities|Array|Add (LocalVariables|GetCollectedShells) (LocalVariables|GetTempShell))
        (Utilities|Array|Add (LocalVariables|GetCollectedPaths) (Utilities|String|SelectString (LocalVariables|GetLinkName) (Utilities|String|ToString(Text) (Utilities|Text|FormatText "{p}/{n}" Path (LocalVariables|GetLinkName))) (Utilities|Array|IsEmpty Path)))
        (if (== (LocalVariables|GetTempShell) Target)
          (return (Utilities|Array|Get(acopy) _collectedpaths (Utilities|Array|LastIndex _collectedpaths)) true 0 0)))))
  (return "" false (LocalVariables|GetCollectedShells) (LocalVariables|GetCollectedPaths)))

(fn FindDataObjectfromPath
  (params (Input :type Array%20of%20Strings) (StartShell :type BP%20Shell%20Object%20Reference))
  (bind (_foundshell _isfound) (CallFunction|FindShellfromPath Input StartShell))
  (if _isfound
    (bind (_isfound_2 _dataobject) (CallFunction|FindDataObjectonShell _foundshell (Utilities|Array|Get(acopy) Input (Utilities|Array|LastIndex Input))))
    (return _isfound_2 _dataobject)))

(fn FindProgramfromPath
  (params (Input :type Array%20of%20Strings) (StartShell :type BP%20Shell%20Object%20Reference))
  (bind (_foundshell _isfound) (CallFunction|FindShellfromPath Input StartShell))
  (if _isfound
    (bind (_program _isfound_2) (CallFunction|FindProgramonShell _foundshell (Utilities|Array|Get(acopy) Input (Utilities|Array|LastIndex Input))))
    (return _program _isfound_2)))

(fn FindShellfromPath
  (params (Input :type Array%20of%20Strings) (StartShell :type BP%20Shell%20Object%20Reference))
  (switch int (Utilities|Array|Length Input)
    (:Default
      (bind (_shell _hasfound) (CallFunction|FindShellbyName (Utilities|Array|Get(acopy) Input (- (Utilities|Array|LastIndex Input) 1)) true StartShell))
      (return _shell _hasfound))
    (:0
      (return 0 false))
    (:1
      (return StartShell true))))

(fn RandomStat
  (params (StatStruct :type Struct%20Random%20Value%20Structure) (Level :type Float%20%28double-precision%29))
  (bind (_default _random) (Utilities|Struct|BreakStruct_RandomValue StatStruct))
  (bind (_default_2 _scaleswithlevel _scale _negativestat) (Utilities|Struct|BreakStruct_RandomValue StatStruct))
  (bind (_minimum _maximum) (Utilities|Struct|BreakStruct_RandomValue StatStruct))
  (bind _returnvalue (> _scaleswithlevel 0))
  (bind _returnvalue_2 (* _scale Level))
  (bind _returnvalue_3 (Math|Float|SelectFloat _returnvalue_2 1.0 _returnvalue))
  (if (> _random 0)
    (return (Math|Float|Min(Float) (Math|Float|Max(Float) (+ (Class|KismetMathLibrary|GetRuntimeFloatCurveValue (Utilities|Struct|BreakRigVMFunction_AnimRichCurve (Utilities|Struct|BreakStruct_RandomValue StatStruct)) (Math|Random|RandomFloat) 0.0) (Math|Float|SelectFloat (Math|Float|Min(Float) (/ _default_2 _returnvalue_3) _default_2) (Math|Float|Max(Float) _default_2 (* _default_2 _returnvalue_3)) (> _negativestat 0))) _minimum) _maximum))
    (else
      (return _default))))

(fn MatchProcessIndex
  (params (Param :type String) (Process :type BP%20Process%20Object%20Reference))
  (bind _asbpi_navigation (Utilities|Casting|CastToBPI_Navigation Process)
    (:then
      (bind _isindexed (Default|IsIndexed _asbpi_navigation))
      (if _isindexed
        _
        (else
          (return false))))
    (:CastFailed
      _))
  (return (Utilities|Enum|Equal(Enum) (Utilities|String|ToString(Integer) (Variables|/Game/Blueprints/Processes/BP_Process.BP_Process_C|GetProcessIndex Process)) Param)))

(fn GetAllShellsinNetwork
  (params (Shell :type BP%20Shell%20Object%20Reference))
  (Utilities|Array|Add (LocalVariables|GetTraversed) Shell)
  (Utilities|Array|Add (LocalVariables|GetFound) Shell)
  (while (> (Utilities|Array|Length (LocalVariables|GetFound)) 0)
    (bind _shells (CallFunction|GetAllShellsinNetworkHelper (Utilities|Array|Get(acopy) (LocalVariables|GetFound)) (LocalVariables|GetTraversed)))
    (Utilities|Array|AppendArray (LocalVariables|GetFound) _shells)
    (Utilities|Array|RemoveIndex (LocalVariables|GetFound)))
  (return (LocalVariables|GetTraversed)))

(fn GetAllShellsinNetworkHelper
  (params (Shell :type BP%20Shell%20Object%20Reference) (Traversed :type Array%20of%20BP%20Shell%20Object%20References))
  (bind _values (Utilities|Map|Values (Variables|/Game/Blueprints/GameObjects/BP_Shell.BP_Shell_C|GetLocalLinks Shell)))
  (for _array_element _values
    (bind _asbpi_navigation (Utilities|Casting|CastToBPI_Navigation _array_element))
    (bind _istwoway (Default|IsTwoWay _asbpi_navigation))
    (if _istwoway
      (bind _shell (Default|GetAddressShell _asbpi_navigation))
      (bind _output_get (LocalVariables|SetOnShell _shell))
      (if (not (Utilities|Array|ContainsItem Traversed _output_get))
        (Utilities|Array|Add (LocalVariables|GetFound) (LocalVariables|GetOnShell))
        (Utilities|Array|Add Traversed (LocalVariables|GetOnShell)))))
  (return (LocalVariables|GetFound)))

(fn GetOpenPortsonNetwork
  (params (Shell :type BP%20Shell%20Object%20Reference))
  (bind _shells (CallFunction|GetAllShellsinNetwork Shell))
  (for _array_element _shells
    (bind _output_get (LocalVariables|SetOnShell _array_element))
    (bind _availableports (Default|AvailablePorts _output_get))
    (bind _output_get_2 (LocalVariables|SetPortCount _availableports))
    (if (> _output_get_2 0)
      (Utilities|Map|Add (LocalVariables|GetFoundPorts) (LocalVariables|GetOnShell) (LocalVariables|GetPortCount))))
  (return (LocalVariables|GetFoundPorts)))