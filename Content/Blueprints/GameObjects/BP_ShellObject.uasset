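; BP_ShellObject is an actor that attaches to a Shell, with visibility requiring both its own and the Shell's ReadAccess.
; Setup randomizes orbit and oscillation, then plays or skips the install animation; deletion optionally animates before destroying it, with dispatchers announcing lifecycle changes.
; Nested components layer motion independently: Anchor orbits, Bounce bobs from a random timeline start, Offset and Point animate install, delete and pulse, and Bump scales to GameManager music data.
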(event Custom|PlayInstall
  (bind (_direction _height _scale) (Timeline|InstallTimeline PlayFromStart)
    (:Update
      (Transformation|SetRelativeLocation (Variables|Default|GetOffset) (Math|Vector|MakeVector 0.0 0.0 _height) false false)
      (Transformation|SetRelativeScale3D (Variables|Default|GetPoint) _scale))
    (:Finished
      (CallFunction|DoneInstalling))))

(event Custom|PlayDelete
  (bind (_direction _height _scale) (Timeline|DeleteTimeline PlayFromStart)
    (:Update
      (Transformation|SetRelativeLocation (Variables|Default|GetOffset) (Math|Vector|MakeVector 0.0 0.0 _height) false false)
      (Transformation|SetRelativeScale3D (Variables|Default|GetPoint) _scale))
    (:Finished
      (CallFunction|DoneDeleting))))

(event Custom|PlayPulse
  (bind _scale (Timeline|PulseTimeline PlayFromStart)
    (:Update
      (Transformation|SetRelativeScale3D (Variables|Default|GetPoint) _scale))))

(event EventBeginPlay
  (CallFunction|Setup)
  (bind _height (Timeline|OscillateTimeline SetNewTime)
    (:Update
      (Transformation|SetRelativeLocation (Variables|Default|GetBounce) (Math|Vector|MakeVector 0.0 0.0 (* _height (Variables|Default|GetOscillationDistance))) false false)
      (Components|Timeline|SetPlayRate (Variables|Default|GetOscillateTimeline) (Variables|Default|GetOscillationRate)))))

(fn ConstructionScript)

(fn Oscillate
  (if (Variables|Default|GetDoOscillation)
    (bind _returnvalue (CallFunction|Oscillate3DVector (Variables|Default|GetOscillationRate) (Variables|Default|GetOscillationOffset) (Variables|Default|GetOscillationDistance)))
    (Transformation|SetRelativeLocation (Variables|Default|GetBounce) _returnvalue false false)))

(fn SetupOscillation
  (Variables|Default|SetOscillationOffset (Math|Random|RandomFloatinRange -1e+01 1e+01)))

(fn Orbit
  (if (Variables|Default|GetDoOrbit)
    (Transformation|AddLocalRotation (Variables|Default|GetAnchor) (Variables|Default|GetOrbitRotator) false false)))

(fn SetupOrbit
  (Transformation|SetRelativeRotation (Variables|Default|GetAnchor) (Math|Random|RandomRotator true) false false)
  (CallFunction|SetupRandomOrbit))

(fn Setup
  (CallFunction|SetVisible (Variables|Default|GetreadAccess))
  (Transformation|AttachActorToActor (Variables|Default|GetShell) "None" "SnapToTarget" "KeepRelative" "KeepRelative" true)
  (CallFunction|SetupOscillation)
  (CallFunction|SetupOrbit)
  (if (Variables|Default|GetSkipInstall)
    (CallFunction|AssigntoShell)
    (else
      (CallFunction|Install))))

(fn Install
  (CallFunction|PlayInstall)
  (Default|CallOnInstall))

(fn Delete
  (params (SkipAnimation :type Boolean))
  (Variables|Default|SetIsDeleting true)
  (Variables|Default|SetDoOrbit false)
  (Variables|Default|SetDoOscillation false)
  (Default|CallOnDelete self SkipAnimation)
  (if SkipAnimation
    (CallFunction|DoneDeleting)
    (else
      (CallFunction|PlayDelete))))

(fn AssigntoShell
  (Transformation|AttachActorToActor (Variables|Default|GetShell) "None" "SnapToTarget" "KeepRelative" "KeepRelative" true))

(fn DoneDeleting
  (EventDispatchers|UnbindallEventsfromOnDelete)
  (EventDispatchers|UnbindallEventsfromOnDoneInstalling)
  (EventDispatchers|UnbindallEventsfromOnInstall)
  (Actor|DestroyActor))

(fn DoneInstalling
  (if (not (Variables|Default|GetIsDeleting))
    (CallFunction|AssigntoShell)
    (Default|CallOnDoneInstalling)))

(fn SetVisible
  (params (NewState :type Boolean))
  (Variables|Default|SetreadAccess NewState)
  (Variables|Default|GetShell
    (:then
      (Rendering|SetActorHiddenInGame (not (and (Variables|Default|GetreadAccess) (Variables|/Game/Blueprints/GameObjects/BP_Shell.BP_Shell_C|GetReadAccess (Variables|Default|GetShell))))))
    (:else)))

(fn BumptoMusic
  (params (StartIndex :type Integer) (EndIndex :type Integer))
  (bind _asbp_game_manager (Utilities|Casting|CastToBP_GameManager (Game|GetGameMode)))
  (bind _outvalue (CallFunction|AverageRange StartIndex EndIndex (Variables|/Game/GameMode/BP_GameManager.BP_GameManager_C|GetMusicConstants _asbp_game_manager)))
  (Transformation|SetRelativeScale3D (Variables|Default|GetBump) (Math|Vector|MakeVector (Math|Float|Clamp(Float) (+ (/ (- _outvalue 0.5) 2.0) 0.8) 0.8 1.1) (Math|Float|Clamp(Float) (+ (/ (- _outvalue 0.5) 2.0) 0.8) 0.8 1.1) (Math|Float|Clamp(Float) (+ (/ (- _outvalue 0.5) 2.0) 0.8) 0.8 1.1))))

(fn SetupRandomOrbit
  (bind _returnvalue (Math|Random|RandomFloat))
  (bind _returnvalue_2 (Math|Random|RandomFloat))
  (bind _returnvalue_3 (* _returnvalue 2.0))
  (bind _returnvalue_4 (* _returnvalue_2 2.0))
  (bind _returnvalue_5 (- _returnvalue_3 1.0))
  (bind _returnvalue_6 (- _returnvalue_4 1.0))
  (bind _returnvalue_7 (Math|Vector|MakeVector _returnvalue_6 _returnvalue_5 0.0))
  (bind _returnvalue_8 (Math|Vector|Normalize _returnvalue_7))
  (bind (_x _y _z) (Math|Vector|BreakVector _returnvalue_8))
  (Variables|Default|SetOrbitRotator (* (Math|Rotator|MakeRotator _x _y _z) (Variables|Default|GetOrbitSpeed))))

(fn Duplicate
  (bind _returnvalue (Game|SpawnActorfromClass (Utilities|GetClass self) (Math|Transform|MakeTransform "0, 0, 0") "Undefined" "MultiplyWithRoot" 0 (Variables|Default|GetShell) (Variables|Default|GetreadAccess) false 0))
  (return _returnvalue))