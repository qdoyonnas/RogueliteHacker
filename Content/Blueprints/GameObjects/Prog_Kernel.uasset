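; Prog_Kernel is the kernel program, a program variant that runs through one dedicated Proc_KernelProcess.
; Setup spawns that process at its own transform if none is valid, passing along its stats, level, ownership, shell and access state.
; Packets and deletion are forwarded to the process.
; Orbit is disabled, oscillation and size calculation are stubbed out, and GetInfo sets visibility from read access and returns a KERNEL label.
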(fn ConstructionScript
  (|CallParentFunction))

(fn StartUniqueProcess
  (bind _skipinstall (Variables|Default|GetSkipInstall))
  (Variables|Default|GetKernelProcess
    (:then)
    (:else
      (bind _returnvalue (Game|SpawnActorfromClass (Variables|Default|GetProcessType) (Transformation|GetActorTransform self) "Undefined" "MultiplyWithRoot" 0 self _skipinstall (Variables|Default|GetProcessStats) 0 (Variables|Default|GetLevel) (Variables|Default|GetPlayerOwned) false (Variables|Default|GetShell) (Variables|Default|GetreadAccess) _skipinstall 0))
      (bind _asproc_kernel_process (Utilities|Casting|CastToProc_KernelProcess _returnvalue))
      (bind _output_get (Variables|Default|SetKernelProcess _asproc_kernel_process))
      (Default|CallOnStartProcess _output_get))))

(fn CalculateSize)

(fn SetupOrbit
  (Variables|Default|SetDoOrbit false))

(fn Orbit
  (params (Alpha :type Float%20%28single-precision%29)))

(fn Oscillate
  (params (Height :type Float%20%28double-precision%29)))

(fn SendPacket
  (params (Path :type Array%20of%20Strings) (Values :type Map%20of%20Strings%20to%20Strings))
  (Default|SendPacket (Variables|Default|GetKernelProcess) Path Values))

(fn Delete
  (params (SkipAnimation :type Boolean))
  (CallFunction|Delete (Variables|Default|GetKernelProcess) SkipAnimation)
  (|CallParentFunction SkipAnimation))

(fn GetInfo
  (params (withReadAccess :type Boolean))
  (CallFunction|SetVisible (or withReadAccess (Variables|Default|GetreadAccess)))
  (return (Utilities|Text|FormatText "{name} <input>.</> <process>KERNEL</>" (CallFunction|GetDisplayName))))

(fn SetupProgram
  (params (Tags :type Array%20of%20Strings) (Properties :type Map%20of%20Strings%20to%20Strings) (InStats :type Map%20of%20Strings%20to%20Reals))
  (CallFunction|StartUniqueProcess)
  (|CallParentFunction Tags Properties InStats)
  (return))