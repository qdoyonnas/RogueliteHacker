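; Network root shell of a hacking game, which drives the network's alert and counterattack behavior.
; A looping timer generates alert until level 5, when it is replaced by a siege-rate timer.
; Shells are ranked by accumulated alert; another timer sends attack shells with Seeker processes at the top one once thresholds are met.
; It can also spawn wipe shells running five wipe programs, with a delete-event binding for restarts.
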(event EventBeginPlay
  (|CallParentFunction)
  (bind _output_get (Variables|Default|SetAlert%20HUD (Variables|/Game/UI/WBP_HUD.WBP_HUD_C|GetAlertHUD (Variables|/Game/GameMode/BP_GameManager.BP_GameManager_C|GetHUD (Variables|Default|GetGameManager)))))
  (EventDispatchers|BindEventtoOnAlertLevelIncrease _output_get (EventDispatchers|CreateEvent :!event AlertLevelIncreased))
  (EventDispatchers|BindEventtoOnAlertIncrease (Variables|Default|GetAlert%20HUD) (EventDispatchers|CreateEvent :!event AlertIncrease))
  (bind _returnvalue (Utilities|Time|SetTimerbyEvent (EventDispatchers|CreateEvent :!event AlertTick) (Variables|Alert|GetAlertTickLength) true))
  (Variables|Alert|SetAlertTimer _returnvalue)
  (bind _returnvalue_2 (Utilities|Time|SetTimerbyEvent (EventDispatchers|CreateEvent :!event SendAttackShells) (Variables|Alert|GetAttackTime) true))
  (Variables|Alert|SetAttackTimer _returnvalue_2))

(fn ConstructionScript
  (|CallParentFunction))

(fn ShutdownShell
  (bind _asbp_game_manager (Utilities|Casting|CastToBP_GameManager (Game|GetGameMode)))
  (Variables|/Game/GameMode/NetworkBuilder/BP_NetworkBuilder.BP_NetworkBuilder_C|SetNetworkRoot (Variables|/Game/GameMode/BP_GameManager.BP_GameManager_C|GetNetworkBuilder _asbp_game_manager) 0)
  (|CallParentFunction))

(fn AlertTick
  (Default|GenerateAlert (Variables|Default|GetGameManager) (Variables|Alert|GetAlertTickAmount)))

(fn AlertLevelIncreased
  (params (AlertLevel :type Integer))
  (if (== AlertLevel 5)
    (Utilities|Time|ClearandInvalidateTimerbyHandle (Variables|Alert|GetAlertTimer))
    (bind _returnvalue (Utilities|Time|SetTimerbyEvent (EventDispatchers|CreateEvent :!event StartWipeShell) (Variables|Wipe|GetSiegeIncreaseRate) true))
    (Variables|Alert|SetAlertTimer _returnvalue)))

(fn StartWipeShell
  (bind _wipeshelllevel (Variables|Wipe|GetWipeShellLevel))
  (bind _spawnedshell (Default|SpawnShellwithDataObjects (Variables|/Game/GameMode/BP_GameManager.BP_GameManager_C|GetNetworkBuilder (Variables|Default|GetGameManager)) (Utilities|Struct|MakeStruct_ShellData "wipe_" (Utilities|Struct|MakeStruct_RandomValue 2e+02 0) (Utilities|Struct|MakeStruct_RandomValue 2e+02 0) (Utilities|Struct|MakeStruct_RandomValue 1e+01 0) (Utilities|Array|MakeArray (Utilities|Struct|MakeStruct_DataObjectData "barrier" "/Game/Blueprints/Processes/SecurityProcesses/Proc_Barrier.Proc_Barrier_C" 10 0 true "" "" "()" false _wipeshelllevel) (Utilities|Struct|MakeStruct_DataObjectData "wipe" "/Game/Blueprints/Processes/SystemProcesses/Proc_Wipe.Proc_Wipe_C" 10 0 false "" "" "()" false _wipeshelllevel) (Utilities|Struct|MakeStruct_DataObjectData "_accessshell" 0 4 0 false "" "AccessShell") (Utilities|Struct|MakeStruct_DataObjectData "message" "/Game/Blueprints/Processes/BasicProcesses/Proc_Message.Proc_Message_C" 10)) 0 false true false) (Variables|Wipe|GetWipeShellLevel) false))
  (bind (_program _isfound) (CallFunction|FindProgramonShell _spawnedshell "message"))
  (LocalVariables|SetMessage _program)
  (if _isfound
    (for _index (range 0 4)
      (Wipe|StartWipeProgram (LocalVariables|GetMessage)))))

(fn RestartWipe
  (params (ShellObject :type BP%20Shell%20Object%20Object%20Reference) (SkipDelete :type Boolean))
  (Utilities|IsValid ShellObject
    (:Is%20Valid
      (bind _asbp_process (Utilities|Casting|CastToBP_Process ShellObject))
      (Utilities|IsValid (Variables|/Game/Blueprints/Processes/BP_Process.BP_Process_C|GetProgram _asbp_process)
        (:Is%20Valid
          (Wipe|StartWipeProgram (Variables|/Game/Blueprints/Processes/BP_Process.BP_Process_C|GetProgram _asbp_process)))))))

(fn StartWipeProgram
  (params (MessageProgram :type BP%20Program%20Object%20Reference))
  (bind _process (Default|StartProcess MessageProgram (Utilities|Array|MakeArray "message" "_accessshell" "wipe") false 0 false))
  (EventDispatchers|BindEventtoOnDelete _process (EventDispatchers|CreateEvent :!event RestartWipe)))

(fn AlertIncrease
  (params (Value :type Float%20%28double-precision%29) (Shell :type BP%20Shell%20Object%20Reference))
  (Utilities|IsValid Shell
    (:Is%20Valid
      (Utilities|Array|RemoveItem (Variables|Alert|GetShellAlertOrder) Shell)
      (if (> (Utilities|Array|Length (Variables|Alert|GetShellAlertOrder)) 0)
        (for _index (range 0 (Utilities|Array|LastIndex (Variables|Alert|GetShellAlertOrder)))
          (bind _output_get (LocalVariables|SetIndex _index))
          (if (<= (Variables|/Game/Blueprints/GameObjects/BP_Shell.BP_Shell_C|GetAccumulatedAlert (Utilities|Array|Get(acopy) (Variables|Alert|GetShellAlertOrder) _output_get)) (Variables|/Game/Blueprints/GameObjects/BP_Shell.BP_Shell_C|GetAccumulatedAlert Shell))
            (Utilities|Array|Insert (Variables|Alert|GetShellAlertOrder) Shell (LocalVariables|GetIndex))
            (return)))
        (Utilities|Array|Add (Variables|Alert|GetShellAlertOrder) Shell)
        (else
          (Utilities|Array|Add (Variables|Alert|GetShellAlertOrder) Shell))))))

(fn StartAttackShell
  (params (TargetShell :type BP%20Shell%20Object%20Reference) (Level :type Float%20%28double-precision%29))
  (bind _spawnedshell (Default|SpawnShellwithDataObjects (Variables|/Game/GameMode/BP_GameManager.BP_GameManager_C|GetNetworkBuilder (Variables|Default|GetGameManager)) (Utilities|Struct|MakeStruct_ShellData "attack_" (Utilities|Struct|MakeStruct_RandomValue 2e+02 0) (Utilities|Struct|MakeStruct_RandomValue 2e+02 0) (Utilities|Struct|MakeStruct_RandomValue 12.0 0) (Utilities|Array|MakeArray (Utilities|Struct|MakeStruct_DataObjectData "shield" "/Game/Blueprints/Processes/SecurityProcesses/Proc_Shield.Proc_Shield_C" 10 0 true "" "" "()" false Level) (Utilities|Struct|MakeStruct_DataObjectData "kill" "/Game/Blueprints/Processes/BasicProcesses/Proc_Kill.Proc_Kill_C" 10 0 false "" "" "()" false Level) (Utilities|Struct|MakeStruct_DataObjectData "delete" "/Game/Blueprints/Processes/BasicProcesses/Proc_Delete.Proc_Delete_C" 10 0 false "" "" "()" false Level) (Utilities|Struct|MakeStruct_DataObjectData "wall" "/Game/Blueprints/Processes/SecurityProcesses/Proc_Wall.Proc_Wall_C" 10 0 false "" "" "()" false Level) (Utilities|Struct|MakeStruct_DataObjectData "link" "/Game/Blueprints/Processes/BasicProcesses/Proc_Link.Proc_Link_C" 10) (Utilities|Struct|MakeStruct_DataObjectData "message" "/Game/Blueprints/Processes/BasicProcesses/Proc_Message.Proc_Message_C" 10) (Utilities|Struct|MakeStruct_DataObjectData (Utilities|GetAddressFileName TargetShell) 0 4 0 false "" (Variables|/Game/Blueprints/GameObjects/BP_Shell.BP_Shell_C|GetName TargetShell))) 0 false true false) Level false))
  (Attack|StartAttackProgram _spawnedshell Level)
  (bind _asbp_game_manager (Utilities|Casting|CastToBP_GameManager (Game|GetGameMode)))
  (Default|Print (Variables|/Game/Blueprints/BP_Interpreter.BP_Interpreter_C|GetTerminal (Variables|/Game/GameMode/BP_GameManager.BP_GameManager_C|GetInterpreter _asbp_game_manager)) (Utilities|Text|FormatText "Attack shell sent to <shell>{s}</>!" (Variables|/Game/Blueprints/GameObjects/BP_Shell.BP_Shell_C|GetName TargetShell))))

(fn StartAttackProgram
  (params (Shell :type BP%20Shell%20Object%20Reference) (Level :type Float%20%28double-precision%29))
  (bind _returnvalue (Game|SpawnActorfromClass "/Game/Blueprints/Processes/RootProcesses/Proc_Seeker.Proc_Seeker_C" (Transformation|GetActorTransform Shell) "Undefined" "MultiplyWithRoot" 0 0 false 0 0 Level false false Shell false true 0))
  (Utilities|Array|Add (Variables|Alert|GetAttackProcesses) _returnvalue))

(fn SendAttackShells
  (bind _alert (Default|GetCurrentAlertLevel (Variables|Default|GetAlert%20HUD)))
  (if (and (>= _alert (Variables|Alert|GetAttackAlertThreshold)) (> (Utilities|Array|Length (Variables|Alert|GetShellAlertOrder)) 0))
    (bind _output_get (LocalVariables|SetShellTarget (Utilities|Array|Get(acopy) (Variables|Alert|GetShellAlertOrder))))
    (if (>= (Variables|/Game/Blueprints/GameObjects/BP_Shell.BP_Shell_C|GetAccumulatedAlert _output_get) (Variables|Alert|GetAttackAlertShellThreshold))
      (Variables|/Game/Blueprints/GameObjects/BP_Shell.BP_Shell_C|SetAccumulatedAlert (LocalVariables|GetShellTarget) 0.0)
      (Utilities|Array|RemoveIndex (Variables|Alert|GetShellAlertOrder))
      (Attack|StartAttackShell (LocalVariables|GetShellTarget) 1.0))))