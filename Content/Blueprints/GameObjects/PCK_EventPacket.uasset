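; PCK_EventPacket is a packet actor that carries a network event along a path of shells.
; HandleNavigation checks the path index and keeps moving to the next shell until the path ends.
; At the end it changes its travel state, fires the arrive-at-shell call, and, if its network event is valid, prints a message and notifies that event of the arrival.
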(fn ConstructionScript
  (|CallParentFunction))

(fn HandleNavigation
  (bind _shell (Variables|Default|GetShell))
  (if (== (Utilities|Array|Length (Variables|Default|GetPath)) (Variables|Default|GetPathIndex))
    (Variables|Default|SetTravelState "NewEnumerator2")
    (Default|CallOnArriveatShell _shell)
    (bind _networkevent (Variables|Default|GetNetworkEvent)
      (:then
        (Development|PrintText (Utilities|Text|FormatText "Event packet arrived at {shell}" (Variables|/Game/Blueprints/GameObjects/BP_Shell.BP_Shell_C|GetNickname _shell)))
        (Default|PacketArrived _networkevent _shell self))
      (:else))
    (else
      (CallFunction|PathtoNextShell))))