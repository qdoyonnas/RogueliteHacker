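; Access kernel program that also dispatches terminal commands, each run as its own spawned process actor.
; It matches the first parameter against class-default aliases of processes in the TerminalCommands data table.
; A match bypasses the parent's add check and spawns that process as player-owned with read access; otherwise parent logic runs.
; Valid-parameter collection for a matched command spawns a temporary process, queries it, then destroys it.
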(fn ConstructionScript
  (|CallParentFunction))

(fn CanAddProcess
  (params (AtShell :type BP%20Shell%20Object%20Reference) (Params :type Array%20of%20Strings))
  (if (.IsFound (CallFunction|GetTerminalCommand Params))
    (return true "")
    (else
      (bind (_canadd _cause) (|CallParentFunction 0 Params))
      (return _canadd _cause))))

(fn StartProcess
  (params (Params :type Array%20of%20Strings) (IsPlayerOwned :type Boolean) (AtShell :type BP%20Shell%20Object%20Reference) (FastForward :type Boolean))
  (bind (_isfound _process) (CallFunction|GetTerminalCommand Params))
  (if _isfound
    (CallFunction|StartTerminalProcess Params _process)
    (return 0)
    (else
      (bind _process_2 (|CallParentFunction Params IsPlayerOwned AtShell FastForward))
      (return _process_2))))

(fn StartTerminalProcess
  (params (Params :type Array%20of%20Strings) (Process :type BP%20Process%20Class%20Reference))
  (Game|SpawnActorfromClass Process (Transformation|GetActorTransform) "Undefined" "MultiplyWithRoot" 0 self false 0 Params 0.0 true false (Variables|Default|GetShell) true false 0)
  (Default|CallOnTerminalCommandStart (LocalVariables|GetCommandAlias)))

(fn CollectValidParameters
  (params (AtShell :type BP%20Shell%20Object%20Reference) (Input :type Array%20of%20Strings))
  (bind (_isfound _process) (CallFunction|GetTerminalCommand Input))
  (if _isfound
    (bind _validparameters (CallFunction|CollectTerminalValidParameters _process Input AtShell))
    (return _validparameters)
    (else
      (bind _validparameters_2 (|CallParentFunction AtShell Input))
      (return _validparameters_2))))

(fn GetTerminalCommand
  (params (Params :type Array%20of%20Strings))
  (bind _outrownames (DataTable|GetDataTableRowNames (Variables|Default|GetTerminalCommands)))
  (for _array_element _outrownames
    (bind _returnvalue (Utilities|GetDataTableRow (Variables|Default|GetTerminalCommands) _array_element)
      (:then
        (bind _output_get (LocalVariables|SetCommand (Utilities|Struct|BreakStruct_Command _returnvalue)))
        (for _array_element_2 (.Aliases (Utilities|GetClassDefaults _output_get))
          (if (Utilities|Enum|Equal(Enum) _array_element_2 (Utilities|Array|Get(acopy) Params))
            (return true (LocalVariables|GetCommand)))))))
  (return false 0))

(fn CollectTerminalValidParameters
  (params (Process :type BP%20Process%20Class%20Reference) (Input :type Array%20of%20Strings) (AtShell :type BP%20Shell%20Object%20Reference))
  (bind _temporary_process (CallFunction|StartTerminalTemporaryProcess Process))
  (bind _output_get (LocalVariables|SetTempProcess _temporary_process))
  (bind _validparameters (Default|CollectfromParam _output_get (- (Utilities|Array|LastIndex Input) 1) AtShell Input))
  (Actor|DestroyActor (LocalVariables|GetTempProcess))
  (return _validparameters))

(fn StartTerminalTemporaryProcess
  (params (Process :type BP%20Process%20Class%20Reference))
  (bind _returnvalue (Game|SpawnActorfromClass Process (Math|Transform|MakeTransform "0, 0, 0") "Undefined" "MultiplyWithRoot" 0 self false (Variables|Default|GetProcessStats) 0 (Variables|Default|GetLevel) false true (Variables|Default|GetShell) false false 0))
  (return _returnvalue))