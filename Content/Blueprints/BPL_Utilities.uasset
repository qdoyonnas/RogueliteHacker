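; Blueprint function library of shared math helpers and lookup queries for the game's shell objects, which hold files, programs and processes.
; Lookups scan a shell's DataObjects or Processes by cast, matching address file names, navigation link names, or program and process aliases.
; Math helpers provide sine bobbing driven by wall-clock Unix time, look-at rotation pitched back 90 degrees, and an end-exclusive array range average.
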(fn Oscillate3DVector
  (params (Rate :type Float%20%28double-precision%29) (CycleOffset :type Float%20%28double-precision%29) (Distance :type Float%20%28double-precision%29))
  (return (Math|Vector|MakeVector 0.0 0.0 (* (Math|Trig|Sin(Radians) (+ (* (Class|KismetMathLibrary|ToUnixTimestampDouble (Math|DateTime|Now)) Rate) CycleOffset)) Distance))))

(fn Oscillate2DVector
  (params (Rate :type Float%20%28double-precision%29) (Cycle%20Offset :type Float%20%28double-precision%29) (Distance :type Float%20%28double-precision%29))
  (return (Math|Vector2D|MakeVector2D 0.0 (* (Math|Trig|Sin(Radians) (+ (* (Class|KismetMathLibrary|ToUnixTimestampDouble (Math|DateTime|Now)) Rate) Cycle%20Offset)) Distance))))

(fn FindAddress
  (params (AddressName :type String) (Shell :type BP%20Shell%20Object%20Reference) (__WorldContext :type Object%20Object%20Reference))
  (for _array_element (Variables|/Game/Blueprints/BP_Shell.BP_Shell_C|GetDataObjects Shell)
    (bind _asfile_address (Utilities|Casting|CastToFile_Address _array_element))
    (if (Utilities|Enum|Equal(Enum) (Variables|/Game/Blueprints/BP_DataObject.BP_DataObject_C|GetFileName _asfile_address) AddressName)
      (return true (Variables|/Game/Blueprints/FileTypes/File_Address.File_Address_C|GetShellAddress _asfile_address) _asfile_address)))
  (return false 0 0))

(fn Pointat
  (params (Object :type Scene%20Component%20Object%20Reference) (Target :type Scene%20Component%20Object%20Reference) (__WorldContext :type Object%20Object%20Reference))
  (bind _returnvalue (Transformation|GetWorldLocation Target))
  (bind _returnvalue_2 (Transformation|GetWorldLocation Object))
  (bind _returnvalue_3 (Math|Rotator|FindLookatRotation _returnvalue_2 _returnvalue))
  (bind (_roll _pitch _yaw) (Math|Rotator|BreakRotator _returnvalue_3))
  (return (Math|Rotator|MakeRotator _roll (- _pitch 9e+01) _yaw)))

(fn CheckLinkExists
  (params (Shell :type BP%20Shell%20Object%20Reference) (Link :type String) (__WorldContext :type Object%20Object%20Reference))
  (for _array_element (Variables|/Game/Blueprints/BP_Shell.BP_Shell_C|GetProcesses Shell)
    (bind _asbp_navigation_process (Utilities|Casting|CastToBP_NavigationProcess _array_element))
    (return (Utilities|Enum|Equal(Enum) (Variables|/Game/Blueprints/BP_Shell.BP_Shell_C|GetName (Variables|/Game/Blueprints/Processes/BP_NavigationProcess.BP_NavigationProcess_C|GetAddressShell _asbp_navigation_process)) Link))))

(fn MatchProcessAlias
  (params (Param :type String) (Process :type BP%20Process%20Object%20Reference))
  (for _array_element (Variables|/Game/Blueprints/Processes/BP_Process.BP_Process_C|GetAliases Process)
    (if (Utilities|Enum|Equal(Enum) _array_element Param)
      (return true))))

(fn AverageRange
  (params (StartIndex :type Integer) (EndIndex :type Integer) (Array :type Array%20of%20Floats%20%28double-precision%29))
  (if (Utilities|Array|IsNotEmpty Array)
    (bind _output_get (LocalVariables|SetIndex StartIndex))
    (while (< _output_get EndIndex)
      (LocalVariables|SetValue (+ (Utilities|Array|Get(acopy) Array (LocalVariables|GetIndex)) (LocalVariables|GetValue)))
      (Math|Integer|IncrementInt (LocalVariables|GetIndex)))
    (bind _output_get_2 (LocalVariables|SetValue (/ (LocalVariables|GetValue) (- EndIndex StartIndex))))
    (return _output_get_2)))

(fn FindProgramonShell
  (params (Shell :type BP%20Shell%20Object%20Reference) (Input :type String))
  (for _array_element (Variables|/Game/Blueprints/BP_Shell.BP_Shell_C|GetDataObjects Shell)
    (bind _asbp_program (Utilities|Casting|CastToBP_Program _array_element))
    (bind _doesmatch (CallFunction|MatchProgramAlias Input _asbp_program))
    (if _doesmatch
      (return _asbp_program true)))
  (return 0 false))

(fn MatchProgramAlias
  (params (Param :type String) (Program :type BP%20Program%20Object%20Reference))
  (for _array_element (Variables|/Game/Blueprints/BP_Program.BP_Program_C|GetAliases Program)
    (if (Utilities|Enum|Equal(Enum) _array_element Param)
      (return true))))