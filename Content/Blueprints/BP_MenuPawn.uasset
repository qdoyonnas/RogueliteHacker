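; BP_MenuPawn is the pawn for a menu, turning an Anchor component while it waits for the player's choice.
; Tick yaws Anchor at a constant rate scaled by delta time.
; Input actions open the LVL_Iterations level for instructions or LVL_Dive for the dive, and the exit action prints a message and quits the game.
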(event Input|EnhancedActionEvents|EnhancedInputActionIA_Dive
  (params (ActionValue :type Boolean) (ElapsedSeconds :type Float%20%28double-precision%29) (TriggeredSeconds :type Float%20%28double-precision%29) (InputAction :type Input%20Action%20Object%20Reference :default "/Game/GameMode/Inputs/IA_Dive.IA_Dive"))
  (Game|OpenLevel(byName) "LVL_Dive"))

(event Input|EnhancedActionEvents|EnhancedInputActionIA_Exit
  (params (ActionValue :type Boolean) (ElapsedSeconds :type Float%20%28double-precision%29) (TriggeredSeconds :type Float%20%28double-precision%29) (InputAction :type Input%20Action%20Object%20Reference :default "/Game/GameMode/Inputs/IA_Exit.IA_Exit"))
  (Development|PrintString "EXIT")
  (Game|QuitGame 0 "Quit" false))

(event Input|EnhancedActionEvents|EnhancedInputActionIA_Instructions
  (params (ActionValue :type Boolean) (ElapsedSeconds :type Float%20%28double-precision%29) (TriggeredSeconds :type Float%20%28double-precision%29) (InputAction :type Input%20Action%20Object%20Reference :default "/Game/GameMode/Inputs/IA_Instructions.IA_Instructions"))
  (Game|OpenLevel(byName) "LVL_Iterations"))

(event EventTick
  (params (DeltaSeconds :type Float%20%28single-precision%29))
  (Transformation|AddWorldRotation (Variables|Default|GetAnchor) (* (Math|Rotator|MakeRotator 0.0 0.0 1e+01) DeltaSeconds) false false))

(fn ConstructionScript)