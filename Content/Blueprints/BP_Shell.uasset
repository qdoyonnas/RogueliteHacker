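; BP_Shell is a named network node holding data objects, processes and address files, with data, memory and thread limits.
; It reports its contents as text, relays packet events, and hides itself without read access.
; Tick scales it to music and lerps pull-in and push-out moves.
; When unanchored without address files or navigation processes, it leaves the NetworkBuilder registry, shrinks away, then deletes its contents and itself.
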(event Custom|PlayPulse
  (bind _scale (Timeline|PulseTimeline PlayFromStart)
    (:Update
      (Transformation|SetRelativeScale3D (Variables|Default|GetBounce) _scale))))

(event EventTick
  (params (DeltaSeconds :type Float%20%28single-precision%29))
  (CallFunction|DoTick DeltaSeconds))

(event EventBeginPlay
  (CallFunction|CollectChildren)
  (Variables|Default|SetPullCurrentTime (Variables|Default|GetPullTime))
  (CallFunction|SetVisible (Variables|Default|GetReadAccess))
  (bind _height (Timeline|OscillateTimeline SetNewTime)
    (:Update
      (Transformation|SetRelativeLocation (Variables|Default|GetBounce) (Math|Vector|MakeVector 0.0 0.0 (* _height (Variables|Default|GetOscillationRange))) false false)
      (Components|Timeline|SetPlayRate (Variables|Default|GetOscillateTimeline) (Variables|Default|GetOscillationRate)))))

(fn ConstructionScript)

(fn AddDataObject
  (params (DataObject :type BP%20Data%20Object%20Object%20Reference))
  (Utilities|Array|Add (Variables|Default|GetDataObjects) DataObject)
  (Variables|/Game/Blueprints/BP_ShellObject.BP_ShellObject_C|SetShell DataObject self))

(fn AddProcess
  (params (Process :type BP%20Process%20Object%20Reference) (InThreads :type Integer))
  (Utilities|Array|Add (Variables|Default|GetProcesses) Process)
  (Variables|/Game/Blueprints/BP_ShellObject.BP_ShellObject_C|SetShell Process self))

(fn CollectChildren
  (for _array_element (Actor|GetAttachedActors true false)
    (bind _asbp_data_object (Utilities|Casting|CastToBP_DataObject _array_element))
    (CallFunction|AddDataObject _asbp_data_object)))

(fn RemoveDataObject
  (params (DataObject :type BP%20Data%20Object%20Object%20Reference))
  (Utilities|Array|RemoveItem (Variables|Default|GetDataObjects) DataObject)
  (Variables|/Game/Blueprints/BP_ShellObject.BP_ShellObject_C|SetShell DataObject 0))

(fn RemoveProcess
  (params (Process :type BP%20Process%20Object%20Reference) (InThreads :type Integer))
  (Utilities|Array|RemoveItem (Variables|Default|GetProcesses) Process)
  (Variables|/Game/Blueprints/BP_ShellObject.BP_ShellObject_C|SetShell Process 0))

(fn CanAddDataObject
  (params (Size :type Integer))
  (bind _data (CallFunction|GetUsedData))
  (return (>= (Variables|Default|GetData) (+ _data Size))))

(fn ShutdownShell
  (Variables|Default|SetHasShutdown true)
  (bind _asbp_game_manager (Utilities|Casting|CastToBP_GameManager (Game|GetGameMode)))
  (Utilities|Map|Remove (Variables|/Game/GameMode/NetworkBuilder/BP_NetworkBuilder.BP_NetworkBuilder_C|GetNetworkShells (Variables|/Game/GameMode/BP_GameManager.BP_GameManager_C|GetNetworkBuilder _asbp_game_manager)) (Utilities|String|ToLower (Variables|Default|GetName)))
  (Default|CallOnShutdownStarted)
  (Utilities|FlowControl|Sequence
    (:then_0
      (EventDispatchers|UnbindallEventsfromOnShutdownStarted))
    (:then_1
      (bind _output_get (LocalVariables|SetDataObjectsCopy (Variables|Default|GetDataObjects)))
      (for _array_element _output_get
        (Default|Delete _array_element true)))
    (:then_2
      (bind _output_get_2 (LocalVariables|SetProcessesCopy (Variables|Default|GetProcesses)))
      (for _array_element_2 _output_get_2
        (Default|Delete _array_element_2 true)))
    (:then_3
      (bind _output_get_3 (LocalVariables|SetFileCopy (Variables|Default|GetAddressFiles)))
      (for _array_element_3 _output_get_3
        (Default|Delete _array_element_3 true)))
    (:then_4
      (Actor|DestroyActor))))

(fn CanAddProcess
  (params (Process :type BP%20Process%20Object%20Reference))
  (bind _memory (CallFunction|GetUsedMemory))
  (bind _threads (CallFunction|GetUsedThreads))
  (return (and (>= (Variables|Default|GetThreads) (+ (Variables|/Game/Blueprints/Processes/BP_Process.BP_Process_C|GetThreads Process) _threads)) (>= (Variables|Default|GetMemory) (+ _memory (Variables|/Game/Blueprints/Processes/BP_Process.BP_Process_C|GetLoad Process)))) (>= (Variables|Default|GetMemory) (+ _memory (Variables|/Game/Blueprints/Processes/BP_Process.BP_Process_C|GetLoad Process)))))

(fn Oscillate
  (bind _returnvalue (CallFunction|Oscillate3DVector 2.0 (Variables|Default|GetOscillationOffset) 3.0))
  (Transformation|SetRelativeLocation (Variables|Default|GetBounce) _returnvalue false false))

(fn StartPull
  (params (ToShell :type BP%20Shell%20Object%20Reference) (Forced :type Boolean) (GiveReadAccess :type Boolean))
  (if (or (not (Variables|Default|GetReadAccess)) Forced)
    (Variables|Default|SetPullEndTransform (Math|Transform|MakeTransform (+ (Transformation|GetActorLocation ToShell) (* (Math|Random|RandomUnitVector) (Variables|Default|GetPullRange)))))
    (Variables|Default|SetPullStartTransform (Math|Transform|MakeTransform (Transformation|GetActorLocation) "0, 0, 0" "0.000000,0.000000,0.000000"))
    (Variables|Default|SetPullCurrentTime 0.0)
    (CallFunction|SetVisible GiveReadAccess)))

(fn DoSlide
  (params (DeltaTime :type Float%20%28double-precision%29))
  (if (>= (Variables|Default|GetPullCurrentTime) (Variables|Default|GetPullTime))
    (if (and (not (Variables|Default|GetHasShutdown)) (Variables|Default|GetBeingShutdown))
      (CallFunction|ShutdownShell))
    (else
      (bind _output_get (Variables|Default|SetPullCurrentTime (+ DeltaTime (Variables|Default|GetPullCurrentTime))))
      (Transformation|SetActorTransform (Math|Transform|Lerp(Transform) (Variables|Default|GetPullStartTransform) (Variables|Default|GetPullEndTransform) (/ _output_get (Variables|Default|GetPullTime)))))))

(fn GetUsedMemory
  (for _array_element (Variables|Default|GetProcesses)
    (LocalVariables|SetMemoryCount (+ (Variables|/Game/Blueprints/Processes/BP_Process.BP_Process_C|GetLoad _array_element) (LocalVariables|GetMemoryCount))))
  (return (LocalVariables|GetMemoryCount)))

(fn GetUsedData
  (for _array_element (Variables|Default|GetDataObjects)
    (LocalVariables|SetDataCount (+ (Variables|/Game/Blueprints/BP_DataObject.BP_DataObject_C|GetSize _array_element) (LocalVariables|GetDataCount))))
  (return (LocalVariables|GetDataCount)))

(fn GetUsedThreads
  (for _array_element (Variables|Default|GetProcesses)
    (LocalVariables|SetThreadsCount (+ (Variables|/Game/Blueprints/Processes/BP_Process.BP_Process_C|GetThreads _array_element) (LocalVariables|GetThreadsCount))))
  (return (LocalVariables|GetThreadsCount)))

(fn GetInfo
  (params (IgnoreProcess :type BP%20Process%20Object%20Reference) (HasReadAccess :type Boolean))
  (CallFunction|SetVisible (or HasReadAccess (Variables|Default|GetReadAccess)))
  (bind _output (CallFunction|CollectDataInfo HasReadAccess))
  (bind _output_2 (CallFunction|CollectMemoryInfo IgnoreProcess HasReadAccess))
  (return (Utilities|Text|FormatText "{list} 
 
{ps} 
" _output _output_2)))

(fn CollectDataObjectInfo
  (params (HasReadAccess :type Boolean))
  (for _array_element (Variables|Default|GetDataObjects)
    (bind _output (Default|GetInfo _array_element HasReadAccess))
    (if (not (Utilities|Text|TextIsEmpty _output))
      (LocalVariables|SetListOutput (Utilities|Text|FormatText "{input} 
{output}" (LocalVariables|GetListOutput) _output))))
  (return (LocalVariables|GetListOutput)))

(fn CollectProcessInfo
  (params (IgnoreProcess :type BP%20Process%20Object%20Reference) (HasReadAccess :type Boolean))
  (for _array_element (Variables|Default|GetProcesses)
    (if (!= _array_element IgnoreProcess)
      (bind _output (Default|GetInfo _array_element HasReadAccess))
      (if (not (Utilities|Text|TextIsEmpty _output))
        (LocalVariables|SetOutputText (Utilities|Text|FormatText "{input} 
{output}" (LocalVariables|GetOutputText) _output)))))
  (return (LocalVariables|GetOutputText)))

(fn CollectMemoryInfo
  (params (IgnoreProcess :type BP%20Process%20Object%20Reference) (HasReadAccess :type Boolean))
  (bind _output (CallFunction|CollectProcessInfo IgnoreProcess HasReadAccess))
  (bind _threads (CallFunction|GetUsedThreads))
  (bind _memory (CallFunction|GetUsedMemory))
  (return (Utilities|Text|FormatText "Active Processes: 
Threads: {threads}/{maxthreads} 
-------{used}/{max}-------{ps}" _threads (Variables|Default|GetThreads) _memory (Variables|Default|GetData) _output)))

(fn CollectDataInfo
  (params (HasReadAccess :type Boolean))
  (bind _returnvalue (CallFunction|CollectDataObjectInfo HasReadAccess))
  (bind _data (CallFunction|GetUsedData))
  (return (Utilities|Text|FormatText "{name}: 
-------{used}/{max}-------{ls}" (Variables|Default|GetName) _data (Variables|Default|GetData) _returnvalue)))

(fn PacketApproaching
  (params (Packet :type BP%20Packet%20Object%20Reference) (FromShell :type BP%20Shell%20Object%20Reference))
  (Default|CallOnPacketApproach Packet FromShell))

(fn BumptoMusic
  (bind _asbp_game_manager (Utilities|Casting|CastToBP_GameManager (Game|GetGameMode)))
  (bind _outvalue (CallFunction|AverageRange 0 5 (Variables|/Game/GameMode/BP_GameManager.BP_GameManager_C|GetMusicConstants _asbp_game_manager)))
  (Transformation|SetRelativeScale3D (Variables|Default|GetBump) (Math|Vector|MakeVector (Math|Float|Clamp(Float) (+ (/ (- _outvalue 0.5) 2.0) 0.8) 0.8 1.1) (Math|Float|Clamp(Float) (+ (/ (- _outvalue 0.5) 2.0) 0.8) 0.8 1.1) (Math|Float|Clamp(Float) (+ (/ (- _outvalue 0.5) 2.0) 0.8) 0.8 1.1))))

(fn DoTick
  (params (DeltaTime :type Float%20%28double-precision%29))
  (CallFunction|BumptoMusic)
  (CallFunction|CheckIsolation)
  (CallFunction|DoSlide DeltaTime))

(fn PacketIntercepted
  (params (Packet :type BP%20Packet%20Object%20Reference) (Process :type BP%20Process%20Object%20Reference))
  (Default|CallOnPacketIntercepted Packet Process))

(fn CheckIsolation
  (if (not (Variables|Default|GetBeingShutdown))
    (bind _isisolated (CallFunction|GetIsIsolated))
    (if _isisolated
      (CallFunction|StartPush))))

(fn StartPush
  (Default|CallOnPushStarted)
  (Utilities|FlowControl|Sequence
    (:then_0
      (EventDispatchers|UnbindallEventsfromOnPushStarted)
      (EventDispatchers|UnbindallEventsfromOnPacketApproach)
      (EventDispatchers|UnbindallEventsfromOnPacketIntercepted))
    (:then_1
      (Variables|Default|SetBeingShutdown true)
      (Variables|Default|SetPullCurrentTime 0.0)
      (Variables|Default|SetPullTime 4.0))
    (:then_2
      (Variables|Default|SetPullStartTransform (Math|Transform|MakeTransform (Transformation|GetActorLocation)))
      (bind _asbp_game_manager (Utilities|Casting|CastToBP_GameManager (Game|GetGameMode)))
      (bind _shelltransform (Default|FindNewShellPosition (Variables|/Game/GameMode/BP_GameManager.BP_GameManager_C|GetNetworkBuilder _asbp_game_manager)))
      (Variables|Default|SetPullEndTransform (Math|Transform|MakeTransform (.Location (Math|Transform|BreakTransform _shelltransform)) (.Rotation (Math|Transform|BreakTransform _shelltransform)) "0.000000,0.000000,0.000000"))
      (Utilities|Map|Remove (Variables|/Game/GameMode/NetworkBuilder/BP_NetworkBuilder.BP_NetworkBuilder_C|GetNetworkShells (Variables|/Game/GameMode/BP_GameManager.BP_GameManager_C|GetNetworkBuilder _asbp_game_manager)) (Utilities|String|ToLower (Variables|Default|GetName))))
    (:then_3
      (bind _asbp_interpreter (Utilities|Casting|CastToBP_Interpreter (Game|Player|GetPlayerPawn 0)))
      (if (== (Variables|/Game/Blueprints/BP_Interpreter.BP_Interpreter_C|GetFocusShell _asbp_interpreter) self)
        (Default|StartZoom _asbp_interpreter (Variables|/Game/Blueprints/BP_ShellObject.BP_ShellObject_C|GetShell (Variables|/Game/Blueprints/BP_Interpreter.BP_Interpreter_C|GetRootProgram _asbp_interpreter)) false)))))

(fn GetIsIsolated
  (for _array_element (Variables|Default|GetProcesses)
    (Utilities|Casting|CastToBP_NavigationProcess _array_element
      (:then
        _)
      (:CastFailed
        (Utilities|Casting|CastToBP_NavigationSubprocess _array_element)))
    (return false))
  (return (and (== (Utilities|Array|Length (Variables|Default|GetAddressFiles)) 0) (not (Variables|Default|GetAnchored)))))

(fn SetName
  (params (NewName :type String))
  (bind _asbp_game_manager (Utilities|Casting|CastToBP_GameManager (Game|GetGameMode)))
  (bind _output_get (LocalVariables|SetNetworkBuilder (Variables|/Game/GameMode/BP_GameManager.BP_GameManager_C|GetNetworkBuilder _asbp_game_manager)))
  (if (not (.ReturnValue (Utilities|Map|Find (Variables|/Game/GameMode/NetworkBuilder/BP_NetworkBuilder.BP_NetworkBuilder_C|GetNetworkShells _output_get) (Utilities|String|ToLower NewName))))
    (Utilities|Map|Remove (Variables|/Game/GameMode/NetworkBuilder/BP_NetworkBuilder.BP_NetworkBuilder_C|GetNetworkShells (LocalVariables|GetNetworkBuilder)) (Utilities|String|ToLower (Variables|Default|GetName)))
    (bind _output_get_2 (Variables|Default|SetName NewName))
    (Utilities|Map|Add (Variables|/Game/GameMode/NetworkBuilder/BP_NetworkBuilder.BP_NetworkBuilder_C|GetNetworkShells (LocalVariables|GetNetworkBuilder)) (Utilities|String|ToLower _output_get_2) self)
    (for _array_element (Variables|Default|GetAddressFiles)
      (bind _filename (CallFunction|GetAddressFileName self))
      (Variables|/Game/Blueprints/BP_DataObject.BP_DataObject_C|SetFileName _array_element _filename))))

(fn SetVisible
  (params (NewState :type Boolean))
  (bind _output_get (Variables|Default|SetReadAccess NewState))
  (Rendering|SetActorHiddenInGame (not _output_get)))